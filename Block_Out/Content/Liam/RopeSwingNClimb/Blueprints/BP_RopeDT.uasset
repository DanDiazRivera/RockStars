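; BP_RopeDT is a work-in-progress skeletal-mesh rope for the third-person character to grab.
; Construction adds a box component at every bone, and the TickTrigger overlap toggles the character's tick.
; Hold snaps the character's capsule to the bone returned by FindNearestRopeBone and stops movement.
; That nearest-to-right-hand search is disconnected, as are the physics simulation and flying-mode logic.
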(event OnComponentBeginOverlap(TickTrigger)
  (params (OverlappedComponent :type Primitive%20Component%20Object%20Reference) (OtherActor :type Actor%20Object%20Reference) (OtherComp :type Primitive%20Component%20Object%20Reference) (OtherBodyIndex :type Integer) (bFromSweep :type Boolean) (SweepResult :type Hit%20Result%20Structure%20%28by%20ref%29))
  (bind _asbp_third_person_character (Utilities|Casting|CastToBP_ThirdPersonCharacter OtherActor))
  (Actor|Tick|SetActorTickEnabled _asbp_third_person_character true))

(event OnComponentEndOverlap(TickTrigger)
  (params (OverlappedComponent :type Primitive%20Component%20Object%20Reference) (OtherActor :type Actor%20Object%20Reference) (OtherComp :type Primitive%20Component%20Object%20Reference) (OtherBodyIndex :type Integer))
  (bind _asbp_third_person_character (Utilities|Casting|CastToBP_ThirdPersonCharacter OtherActor))
  (Actor|Tick|SetActorTickEnabled _asbp_third_person_character))

(event EventHold
  (params (Character :type Character%20Object%20Reference))
  ;[1 1 1] TO DO: Revisit 11:55
  (bind _asbp_third_person_character (Utilities|Casting|CastToBP_ThirdPersonCharacter Character))
  (Variables|Default|SetPlayer _asbp_third_person_character)
  (Utilities|FlowControl|Sequence
    (:then_0
      ;[1 1 1] Get Rope Bone
      (bind _bestindex (CallFunction|FindNearestRopeBone))
      (Variables|Default|SetActiveBone (Class|SkinnedMeshComponent|GetBoneName (Variables|Default|GetSkeletalMesh) _bestindex)))
    (:then_1
      ;[1 1 1] https://www.youtube.com/watch?v=ak0gOuC5u98 - Left off @ 26:23
      (Transformation|SetWorldLocation (Variables|/Script/Engine.Character|GetCapsuleComponent (Variables|Default|GetPlayer)) (Transformation|GetSocketLocation (Variables|Default|GetSkeletalMesh) (Variables|Default|GetActiveBone)) false false)
      (Components|Movement|StopMovementImmediately (Variables|/Script/Engine.Character|GetCharacterMovement (Variables|Default|GetPlayer))))))

(event EventBeginPlay
  (Actor|Tick|SetActorTickEnabled false))

(event EventTick
  (params (DeltaSeconds :type Float%20%28single-precision%29))
  ;[0.05448 0.05781 0] OLD FUNCTION
  ;;[0.125 0.125 0.125] Display the locations of the bones.
)

(fn ConstructionScript
  (bind _skeletalmesh (Variables|Default|GetSkeletalMesh))
  (for _index (range 0 (- (Class|SkinnedMeshComponent|GetNumBones (Variables|Default|GetSkeletalMesh)) 1))
    (bind _returnvalue (AddComponent|AddBoxComponent false (Math|Transform|MakeTransform (- (Transformation|GetSocketLocation _skeletalmesh (Class|SkinnedMeshComponent|GetBoneName _skeletalmesh _index)) (Transformation|GetWorldLocation _skeletalmesh)) "0, 0, 0" "2.000000,2.000000,2.000000")))
    (Utilities|Array|Add (Variables|Default|GetBoneBox) _returnvalue)))

(fn FindNearestRopeBone)