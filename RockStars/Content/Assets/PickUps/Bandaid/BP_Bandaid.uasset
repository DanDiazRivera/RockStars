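; BP_Bandaid is a health pickup that changes the player's health when touched and is registered to respawn after death.
; A looping timer bobs its static mesh vertically on a sine wave around the starting relative location.
; On overlap with the tagged player, it calls ChangeHealth on BP_ThirdPersonCharacter, adds its class and initial transform to the game mode's RespawnableActors array, then destroys itself.
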(event OnComponentBeginOverlap(BandAidStaticMesh)
  (params (OverlappedComponent :type Primitive%20Component%20Object%20Reference) (OtherActor :type Actor%20Object%20Reference) (OtherComp :type Primitive%20Component%20Object%20Reference) (OtherBodyIndex :type Integer) (bFromSweep :type Boolean) (SweepResult :type Hit%20Result%20Structure%20%28by%20ref%29))
  ;[0.03955 0.6584 0] Changes Player's Health
  (if (Actor|ActorHasTag OtherActor "Player")
    (bind _asbp_third_person_character (Utilities|Casting|CastToBP_ThirdPersonCharacter OtherActor))
    (Default|ChangeHealth _asbp_third_person_character (Variables|Default|GetChangeValue))
    ;[0.000304 0.09306 0.5457] Calls Add to Respawnable and Destroys Bandaid
    (CallFunction|AddtoRespawnable)
    (Actor|DestroyActor)))

(event Custom|BandAidBobbing
  (bind _relativelocation (Variables|Default|GetRelativeLocation))
  ;[0.956 0.5647 0.01681] Bobbing Effect
  (Transformation|SetRelativeLocation (Variables|Default|GetBandAidStaticMesh) (Math|Vector|MakeVector (.x _relativelocation) (.y _relativelocation) (+ (.z _relativelocation) (* (Math|Trig|Sin(Degrees) (* (Actor|GetGameTimeSinceCreation) (Variables|Default|GetBobbingSpeed))) (Variables|Default|GetBobbingDistance)))) false false))

(event Custom|AddToRespawnable
  ;[0 0.09759 0.5841] Adds to Respawnable Struct Array so that Bandaid respawns on death
  (bind _asbp_third_person_game_mode (Utilities|Casting|CastToBP_ThirdPersonGameMode (Game|GetGameMode)))
  (Utilities|Array|Add (Variables|/Game/LevelStuff/ThirdPerson/Blueprints/Movement/BP_ThirdPersonGameMode.BP_ThirdPersonGameMode_C|GetRespawnableActors _asbp_third_person_game_mode) (Utilities|Struct|MakeStruct_RespawnableActors "BP_Bandaid_C" self (Variables|Default|GetInitialTransform))))

(event EventBeginPlay
  ;[0.9911 0.1714 0] Sets Initial Transform
  (Variables|Default|SetInitialTransform (Transformation|GetActorTransform))
  ;[0.9734 0.5776 0.01681] Sets Timer and Relative Location for Bobbing Effect
  (Utilities|Time|SetTimerbyFunctionName 0 "BandAidBobbing" 0.01 true)
  (Variables|Default|SetRelativeLocation (Variables|/Script/Engine.SceneComponent|GetRelativeLocation (Variables|Default|GetBandAidStaticMesh))))

(fn ConstructionScript)