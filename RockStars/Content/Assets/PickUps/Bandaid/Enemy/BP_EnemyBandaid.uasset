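; BP_EnemyBandaid is an enemy-dropped health pickup that bobs in place, heals the player on overlap unless at full health, and despawns after a delay.
; On spawn it registers in the game mode's EnemyDroppedBandaids array, destroying the oldest entry to cap active drops at two.
; A looping timer drives the sine-wave bob.
; Pickup and timeout both remove it from the array before destroying it, keeping the count accurate.
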(event OnComponentBeginOverlap(BandAidStaticMesh)
  (params (OverlappedComponent :type Primitive%20Component%20Object%20Reference) (OtherActor :type Actor%20Object%20Reference) (OtherComp :type Primitive%20Component%20Object%20Reference) (OtherBodyIndex :type Integer) (bFromSweep :type Boolean) (SweepResult :type Hit%20Result%20Structure%20%28by%20ref%29))
  ;[0.03955 0.6584 0] Changes Player's Health
  (if (Actor|ActorHasTag OtherActor "Player")
    (bind _asbp_third_person_character (Utilities|Casting|CastToBP_ThirdPersonCharacter OtherActor))
    ;;[0.03955 0.6584 0] Make sure player is not at max health. If they are, do nothing (bandaid isn't picked up).
    (if (!= (Variables|/Game/LevelStuff/ThirdPerson/Blueprints/Movement/BP_ThirdPersonCharacter.BP_ThirdPersonCharacter_C|GetHealthOfCharacter _asbp_third_person_character) 1e+02)
      (Default|ChangeHealth _asbp_third_person_character (Variables|Default|GetChangeValue))
      (Audio|PlaySound2D "/Game/Assets/PickUps/Bandaid/Health_Collectible.Health_Collectible" 1.0 1.0 0.0 0 0)
      (CallFunction|RemovefromArrayandDestroy self))))

(event Custom|BandAidBobbing
  (bind _relativelocation (Variables|Default|GetRelativeLocation))
  ;[0.956 0.5647 0.01681] Bobbing Effect
  (Transformation|SetRelativeLocation (Variables|Default|GetBandAidStaticMesh) (Math|Vector|MakeVector (.x _relativelocation) (.y _relativelocation) (+ (.z _relativelocation) (* (Math|Trig|Sin(Degrees) (* (Actor|GetGameTimeSinceCreation) (Variables|Default|GetBobbingSpeed))) (Variables|Default|GetBobbingDistance)))) false false))

(event Custom|RemoveFromArrayAndDestroy
  (params (Bandaid :type BP%20Enemy%20Bandaid%20Object%20Reference%20%28by%20ref%29))
  ;[0.9734 0.5776 0.01681] Take in a bandaid, remove it from the array of dropped bandaids, then destroy it. This ensures the bandaid is removed from the array before trying to add a new one to it. If not removed, the number of active bandaids (length of the array) will be off, and there will be an error when trying to destroy it since it was already destroyed.
  (Utilities|Array|RemoveItem (Variables|/Game/LevelStuff/ThirdPerson/Blueprints/Movement/BP_ThirdPersonGameMode.BP_ThirdPersonGameMode_C|GetEnemyDroppedBandaids (Variables|Default|GetGameModeRef)) Bandaid)
  (Actor|DestroyActor))

(event EventBeginPlay
  ;[0.007609 0.07292 0.01102] When this bandaid first spawns, get a ref to the gamemode and then access its bandaid array to check how may bandaids are currently in the level. If there are currently 2 (or more on the off chance) destroy the first bandaid in the array, remove it from the array, and then add the new bandaid to the array. This ensures there are only ever two bandaids dropped from enemies in the level. If a new one is dropped, then the oldest bandaid gets destroyed.
  (bind _asbp_third_person_game_mode (Utilities|Casting|CastToBP_ThirdPersonGameMode (Game|GetGameMode)))
  (bind _output_get (Variables|Default|SetGameModeRef _asbp_third_person_game_mode))
  (if (>= (Utilities|Array|Length (Variables|/Game/LevelStuff/ThirdPerson/Blueprints/Movement/BP_ThirdPersonGameMode.BP_ThirdPersonGameMode_C|GetEnemyDroppedBandaids _output_get)) 2)
    (Actor|DestroyActor (Utilities|Array|Get(acopy) (Variables|/Game/LevelStuff/ThirdPerson/Blueprints/Movement/BP_ThirdPersonGameMode.BP_ThirdPersonGameMode_C|GetEnemyDroppedBandaids _output_get)))
    (Utilities|Array|RemoveIndex (Variables|/Game/LevelStuff/ThirdPerson/Blueprints/Movement/BP_ThirdPersonGameMode.BP_ThirdPersonGameMode_C|GetEnemyDroppedBandaids _output_get)))
  (Utilities|Array|Add (Variables|/Game/LevelStuff/ThirdPerson/Blueprints/Movement/BP_ThirdPersonGameMode.BP_ThirdPersonGameMode_C|GetEnemyDroppedBandaids _output_get) self)
  ;[0.9911 0.1714 0] Sets Initial Transform
  (Variables|Default|SetInitialTransform (Transformation|GetActorTransform))
  ;[0.9734 0.5776 0.01681] Sets Timer and Relative Location for Bobbing Effect
  (Utilities|Time|SetTimerbyFunctionName 0 "BandAidBobbing" 0.01 true)
  (Variables|Default|SetRelativeLocation (Variables|/Script/Engine.SceneComponent|GetRelativeLocation (Variables|Default|GetBandAidStaticMesh)))
  ;[0.9734 0.5776 0.01681] Once the bandaid spawns, wait for the despawn time before destroying the bandaid.
  (Utilities|FlowControl|Delay (Variables|Default|GetDespawnTime))
  (CallFunction|RemovefromArrayandDestroy self))

(fn ConstructionScript)