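; A floating bubble pickup that restores the player's double jump on overlap, only if it is spent.
; After collection it hides and stops being collectible for a set delay, then reappears.
; Looping timers drive a sine-wave bob and poll the player's weapon index, with DoOnce-gated timelines shrinking the bubble when the keytar is away and restoring it when out.
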(event OnComponentBeginOverlap(Bubble)
  (params (OverlappedComponent :type Primitive%20Component%20Object%20Reference) (OtherActor :type Actor%20Object%20Reference) (OtherComp :type Primitive%20Component%20Object%20Reference) (OtherBodyIndex :type Integer) (bFromSweep :type Boolean) (SweepResult :type Hit%20Result%20Structure%20%28by%20ref%29))
  (bind _playercharacter (CallFunction|GetValidPlayer))
  (bind _bubble (Variables|Default|GetBubble))
  ;[1 1 1] Let player jump again
  (if (Variables|Default|GetCanBeCollected)
    (if (Actor|ActorHasTag OtherActor "Player")
      (if (not (Variables|/Game/LevelStuff/ThirdPerson/Blueprints/Movement/BP_ThirdPersonCharacter.BP_ThirdPersonCharacter_C|GetCanDoubleJump _playercharacter)) ; Only if double jump is false should it be set to true, \nand the collectible then turned off for a brief period of time.
        (Variables|/Game/LevelStuff/ThirdPerson/Blueprints/Movement/BP_ThirdPersonCharacter.BP_ThirdPersonCharacter_C|SetCanDoubleJump _playercharacter true)
        (Variables|Default|SetCanBeCollected false)
        (Rendering|SetVisibility _bubble false false)
        (Utilities|FlowControl|Delay (Variables|Default|GetNotCollectibleTime))
        (Variables|Default|SetCanBeCollected true)
        (Rendering|SetVisibility _bubble true false)))))

(event Custom|JumpRefreshBobbing
  (bind _relativelocation (Variables|Default|GetRelativeLocation))
  ;[1 1 1] Bobbing Effect
  (Transformation|SetRelativeLocation (Variables|Default|GetBubble) (Math|Vector|MakeVector (.x _relativelocation) (.y _relativelocation) (+ (.z _relativelocation) (* (Math|Trig|Sin(Degrees) (* (Actor|GetGameTimeSinceCreation) (Variables|Default|GetBobbingSpeed))) (Variables|Default|GetBobbingDistance)))) false false))

(event Custom|OpacityAdjustment
  (if (!= (Variables|/Game/LevelStuff/ThirdPerson/Blueprints/Movement/BP_ThirdPersonCharacter.BP_ThirdPersonCharacter_C|GetCurrentWeaponIndex (CallFunction|GetValidPlayer)) 1)
    (Utilities|FlowControl|DoOnce false :!label _label
      (:Completed
        ;[0 0.05758 0.2083] If the keytar is not out, shrink its size.
        (bind _scale (Timeline|ScaleDown PlayFromStart)
          (:Update
            (Transformation|SetWorldScale3D (Variables|Default|GetBubble) (Math|Vector|MakeVector _scale _scale _scale)))
          (:Finished
            (goto _label_2 Reset)))))
    (else
      (Utilities|FlowControl|DoOnce false :!label _label_2
        (:Completed
          ;[0 0.05758 0.2083] If the keytar is out, make it scale up to normal size
          (bind _scale_2 (Timeline|ScaleUp PlayFromStart)
            (:Update
              (Transformation|SetWorldScale3D (Variables|Default|GetBubble) (Math|Vector|MakeVector _scale_2 _scale_2 _scale_2)))
            (:Finished
              (goto _label Reset))))))))

(event EventBeginPlay
  ;[1 1 1] Sets Timer and Relative Location for Bobbing Effect
  (Utilities|Time|SetTimerbyFunctionName 0 "JumpRefreshBobbing" 0.01 true)
  (Variables|Default|SetRelativeLocation (Variables|/Script/Engine.SceneComponent|GetRelativeLocation (Variables|Default|GetBubble)))
  (bind _asbp_third_person_character (Utilities|Casting|CastToBP_ThirdPersonCharacter (Game|GetPlayerCharacter 0)))
  (Variables|Default|SetPlayerCharacter _asbp_third_person_character)
  (Utilities|Time|SetTimerbyEvent (delegate Custom|OpacityAdjustment) 0.5 true))

(fn ConstructionScript)

(fn GetValidPlayer
  (bind _playercharacter (Variables|Default|GetPlayerCharacter)
    (:then
      (return _playercharacter))
    (:else
      (bind _asbp_third_person_character (Utilities|Casting|CastToBP_ThirdPersonCharacter (Game|GetPlayerCharacter 0)))
      (bind _output_get (Variables|Default|SetPlayerCharacter _asbp_third_person_character))
      (return _output_get))))