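; BP_SpawnVFX is a one-shot sprite effect actor that plays a chosen Paper2D flipbook and destroys itself when playback finishes.
; The construction script assigns the flipbook, applies a configurable relative transform and turns off looping.
; When ConstantlyFacePlayer is enabled, Tick billboards the flipbook toward player 0's camera, combining the look-at rotation with the configured transform's rotation as an offset.
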(event OnFinishedPlaying(PaperFlipbook)
  ;[0 0 0] Destroy this when it is done playing.
  (Actor|DestroyActor))

(event EventTick
  (params (DeltaSeconds :type Float%20%28single-precision%29))
  (if (Variables|Default|GetConstantlyFacePlayer)
    (CallFunction|FacePlayer)))

(fn ConstructionScript
  (bind _paperflipbook (Variables|Default|GetPaperFlipbook))
  ;[0 0 0] Set the flipbbok to play and turn off looping.
  (Sprite|SetFlipbook _paperflipbook (Variables|Default|GetFlipbookToPlay))
  (Transformation|SetRelativeTransform _paperflipbook (Variables|Default|GetTransform) false false)
  (Components|Timeline|SetLooping _paperflipbook false))

(fn FacePlayer
  (Transformation|SetWorldRotation (Variables|Default|GetPaperFlipbook) (Math|Rotator|CombineRotators (Math|Rotator|FindLookatRotation (Transformation|GetWorldLocation (Variables|Default|GetPaperFlipbook)) (Transformation|GetWorldLocation (Variables|/Script/Engine.PlayerCameraManager|GetTransformComponent (Game|GetPlayerCameraManager 0)))) (.rotation (Variables|Default|GetTransform))) false false))