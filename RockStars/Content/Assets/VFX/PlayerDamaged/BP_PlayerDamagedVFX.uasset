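; One-shot flipbook effect actor for player damage, which always faces the camera and removes itself when done.
; The construction script turns off looping on the Paper2D flipbook, and its finished-playing event destroys the actor.
; Every tick, FacePlayer billboards the flipbook toward the first player's camera manager using a look-at rotation combined with a fixed rotation offset.
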(event OnFinishedPlaying(PaperFlipbook)
  ;[0 0 0] Destroy this when it is done playing.
  (Actor|DestroyActor))

(event EventTick
  (params (DeltaSeconds :type Float%20%28single-precision%29))
  (CallFunction|FacePlayer))

(fn ConstructionScript
  ;[0 0 0] When created, turn off looping.
  (Components|Timeline|SetLooping (Variables|Default|GetPaperFlipbook) false))

(fn FacePlayer
  (Transformation|SetWorldRotation (Variables|Default|GetPaperFlipbook) (Math|Rotator|CombineRotators (Math|Rotator|FindLookatRotation (Transformation|GetWorldLocation (Variables|Default|GetPaperFlipbook)) (Transformation|GetWorldLocation (Variables|/Script/Engine.PlayerCameraManager|GetTransformComponent (Game|GetPlayerCameraManager 0)))) "0.000000,90.000000,0.000000") false false))