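; Combat arena gate that stays hidden until the player enters or spawns inside, then fades in with blocking collision until enemies drop to a despawn threshold.
; Detector overlaps update a bobbing, player-facing enemy counter and set custom depth stencil to outline enemies within.
; Activation registers the gate (as BP_EnemyGate) and its initial enemies in the GameMode's respawn array.
; Reaching the threshold fades the gate out and destroys it.
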(event OnComponentBeginOverlap(PlayerDetector)
  (params (OverlappedComponent :type Primitive%20Component%20Object%20Reference) (OtherActor :type Actor%20Object%20Reference) (OtherComp :type Primitive%20Component%20Object%20Reference) (OtherBodyIndex :type Integer) (bFromSweep :type Boolean) (SweepResult :type Hit%20Result%20Structure%20%28by%20ref%29))
  (bind _gatevisual (Variables|Default|GetGateVisual))
  ;[1 0.5284 0.868] When the player enters the gate, it turns on and displays the amount of enemies inside!
  (if (Utilities|Array|IsNotEmpty (Variables|Default|GetInitialOverlappingActors))
    (if (Variables|Default|GetGateTriggeredByPlayer)
      ;;[1 0.6902 0] See bottom right!
      (CallFunction|EnemyMatOverlay))
    (if (Actor|ActorHasTag OtherActor "Player")
      (Variables|Default|SetGateTriggeredByPlayer true)
      (Utilities|FlowControl|Sequence
        (:then_0
          (Utilities|FlowControl|DoOnce false
            (:Completed
              (CallFunction|AddtoRespawnble)
              (CallFunction|AddEnemiestoRespawnable))))
        (:then_1
          (Rendering|SetActorHiddenInGame false)
          (Development|PrintString "ENTERING ENEMY GATE! ENEMIES INSIDE: " true true "(R=1.000000,G=0.176471,B=0.396078,A=1.000000)")
          ;;[1 0.6902 0] See bottom right!
          (CallFunction|EnemyMatOverlay)
          (Collision|SetCollisionResponsetoChannel _gatevisual "ECC_Pawn" "ECR_Block")
          (Collision|SetCollisionResponsetoChannel _gatevisual "ECC_WorldStatic" "ECR_Block")
          (Collision|SetCollisionResponsetoChannel _gatevisual "ECC_GameTraceChannel1" "ECR_Block")
          (CallFunction|CounterBobbing true)
          (CallFunction|MaterialFade true))))))

(event Custom|EnemyCleared
  (params (Remaining :type Integer))
  ;[0.5469 1 0.5704] When the amount of enemies inside the gate equals the despawn threshold, the gate is destroyed!
  (if (== Remaining (Variables|Default|GetDespawnThreshold))
    (Development|PrintString "DESPAWN THRESHOLD REACHED! GATE IS DOWN!" false true "(R=1.000000,G=0.176471,B=0.396078,A=1.000000)")
    (CallFunction|MaterialFade false)
    (Utilities|FlowControl|Delay 1.0)
    (Actor|DestroyActor)))

(event Custom|MaterialFade
  (params (FadeIN :type Boolean))
  ;[0.4503 0.91 1] Fade Timeline - If Fade IN is true, play start to finish; else, play in reverse!
  (if FadeIN
    (bind _matopacity (Timeline|fadeTime PlayFromStart)
      (:Update
        (Rendering|Material|SetScalarParameterValueonMaterials (Variables|Default|GetGateVisual) "fadeOut" (Math|Float|Lerp 1.0 0.9 _matopacity))))
    (else
      (Timeline|fadeTime ReverseFromEnd))))

(event Custom|PlayerSpawnedInside
  (bind _gatevisual (Variables|Default|GetGateVisual))
  ;[1 0.426 0.02583] When Enemies are Detected or Killed inside the gate, calculate the total amount of enemies within!
  ;;[0.2423 0.005605 0.004391] If Player is spawned inside the combat zone, calls the necessary code that was skipped over in intial spawning
  (Utilities|FlowControl|Sequence
    (:then_0
      ;[1 0.5284 0.868] When the player enters the gate, it turns on and displays the amount of enemies inside!
      (Variables|Default|SetGateTriggeredByPlayer true)
      (Utilities|FlowControl|Sequence
        (:then_0
          (Utilities|FlowControl|DoOnce false
            (:Completed
              (CallFunction|AddtoRespawnble)
              (CallFunction|AddEnemiestoRespawnable))))
        (:then_1
          (Rendering|SetActorHiddenInGame false)
          (Development|PrintString "ENTERING ENEMY GATE! ENEMIES INSIDE: " true true "(R=1.000000,G=0.176471,B=0.396078,A=1.000000)")
          ;;[1 0.6902 0] See bottom right!
          (CallFunction|EnemyMatOverlay)
          (Collision|SetCollisionResponsetoChannel _gatevisual "ECC_Pawn" "ECR_Block")
          (Collision|SetCollisionResponsetoChannel _gatevisual "ECC_WorldStatic" "ECR_Block")
          (Collision|SetCollisionResponsetoChannel _gatevisual "ECC_GameTraceChannel1" "ECR_Block")
          (CallFunction|CounterBobbing true)
          (CallFunction|MaterialFade true))))
    (:then_1
      (bind _output_get (Variables|Default|SetEnemiesWithin (Utilities|Array|Length (Variables|Default|GetOverlapping%20Actors))))
      ;;[0.5469 1 0.5704] See bottom left!
      (CallFunction|EnemyCleared _output_get)
      (Rendering|Components|TextRender|SetText (Variables|Default|GetEnemyCounter) (Utilities|Text|ToText(Integer) (Variables|Default|GetEnemiesWithin)))
      (CallFunction|FacePlayer))))

(event Custom|Test%20For%20Loop
  ;[0.4503 0.91 1] Fade Timeline - If Fade IN is true, play start to finish; else, play in reverse!
  (for _array_element (Variables|Default|GetOverlapping%20Actors)
    (Development|PrintString (Utilities|GetDisplayName _array_element) true true "(R=0.000000,G=0.660000,B=1.000000,A=1.000000)" 15.0)))

(event Custom|FacePlayer
  (bind _returnvalue (Game|GetPlayerCharacter 0))
  (bind _enemycounter (Variables|Default|GetEnemyCounter))
  ;[0.003922 0 0.05882] Text Face Player Conditions
  (Utilities|IsValid _returnvalue
    (:Is%20Valid
      (Transformation|SetRelativeRotation _enemycounter (Math|Rotator|MakeRotator 0.0 0.0 (.yaw (Math|Interpolation|RInterpTo (Transformation|GetSocketRotation _enemycounter "EnemyCounter") (Math|Rotator|FindLookatRotation (Transformation|GetSocketLocation _enemycounter "EnemyCounter") (Transformation|GetActorLocation _returnvalue)) (Utilities|Time|GetWorldDeltaSeconds) 1e+01))) false false)
      (Utilities|FlowControl|Delay 0.01)
      (CallFunction|FacePlayer))))

(event Custom|CounterBobbing
  (params (BobbingUP :type Boolean))
  ;[0.003922 0 0.05882] Text Face Player Conditions
  (if BobbingUP
    (bind _texttransform (Timeline|counterBob PlayFromStart)
      (:Update
        (Transformation|SetRelativeLocation (Variables|Default|GetEnemyCounter) (Math|Vector|Lerp(Vector) "0, 0, 0" _texttransform 2.0) false false))
      (:Finished
        (bind _output_get (Variables|Default|SetCounterMovesUp (not (Variables|Default|GetCounterMovesUp))))
        (CallFunction|CounterBobbing _output_get)))
    (else
      (Timeline|counterBob ReverseFromEnd))))

(event Custom|EnemyMatOverlay
  ;[1 0.6902 0] Enemies inside the gate's confines will be outlined for ease of visibility!
  (for _array_element (Variables|Default|GetOverlapping%20Actors)
    (bind _asbp_enemy_base_class (Utilities|Casting|CastToBP_EnemyBaseClass _array_element))
    (Rendering|SetCustomDepthStencilValue (Variables|/Script/Engine.Character|GetMesh _asbp_enemy_base_class) 1)))

(event Custom|AutoScaleLight
  (bind _self self)
  (bind _pointlight (Variables|Default|GetPointLight))
  (bind _pointlight_2 (Variables|Default|GetPointLight))
  (bind _returnvalue (Transformation|GetActorScale3D _self))
  ;[0.2326 0.2396 0.06209] Automatically adjust the scale of the lights to fit the radius!
  (Rendering|Lighting|SetAttenuationRadius _pointlight_2 (* (Variables|/Script/Engine.LocalLightComponent|GetAttenuationRadius _pointlight_2) (.x _returnvalue)))
  (Class|PointLightComponent|SetSourceRadius _pointlight (* (Variables|/Script/Engine.PointLightComponent|GetSourceRadius _pointlight) (.y _returnvalue))))

(event Custom|AddToRespawnble
  ;[0 0.09759 0.5841] Adds to Respawnable Struct Array so that EnemyGate respawns on player death
  (bind _asbp_third_person_game_mode (Utilities|Casting|CastToBP_ThirdPersonGameMode (Game|GetGameMode)))
  (Utilities|Array|AddUnique (Variables|/Game/LevelStuff/ThirdPerson/Blueprints/Movement/BP_ThirdPersonGameMode.BP_ThirdPersonGameMode_C|GetRespawnableActors _asbp_third_person_game_mode) (Utilities|Struct|MakeStruct_RespawnableActors "/Game/LevelStuff/EnemyGate/BP_EnemyGate.BP_EnemyGate_C" self (Variables|Default|GetInitialTransform))))

(event Custom|AddEnemiesToRespawnable
  (bind _initialoverlappingactors (Variables|Default|GetInitialOverlappingActors))
  ;[0 0.3882 0.8784] Adds Enemies within Enemy Gate to the Respawnable Struct Array so that Enemies respawn on player death
  (bind _asbp_third_person_game_mode (Utilities|Casting|CastToBP_ThirdPersonGameMode (Game|GetGameMode)))
  (for _array_element _initialoverlappingactors
    (if (Utilities|IsValid _array_element)
      (bind _asbp_enemy_base_class (Utilities|Casting|CastToBP_EnemyBaseClass _array_element))
      (Utilities|Array|AddUnique (Variables|/Game/LevelStuff/ThirdPerson/Blueprints/Movement/BP_ThirdPersonGameMode.BP_ThirdPersonGameMode_C|GetRespawnableActors _asbp_third_person_game_mode) (Utilities|Struct|MakeStruct_RespawnableActors (Utilities|GetClass _array_element) _array_element (Variables|/Game/Users/Dylan/EnemyBlueprints/BaseEnemy/BP_EnemyBaseClass.BP_EnemyBaseClass_C|GetInitialTransform _asbp_enemy_base_class)))))
  (Utilities|Array|Clear _initialoverlappingactors))

(event EventBeginPlay
  (bind _enemydetector (Variables|Default|GetEnemyDetector))
  ;[0.08806 0.07434 0.2396] Enemy Gates Begin Hidden!
  (Rendering|SetActorHiddenInGame true)
  (Rendering|Material|CreateDynamicMaterialInstance (Variables|Default|GetGateVisual) 0 "/Game/LevelStuff/EnemyGate/MI_EnemyGateTEST.MI_EnemyGateTEST" "None" :!class /Script/Engine.PrimitiveComponent)
  (CallFunction|AutoScaleLight)
  (Variables|Default|SetInitialTransform (Transformation|GetActorTransform))
  (Utilities|FlowControl|Delay 0.1)
  (Collision|SetCollisionEnabled (Variables|Default|GetGateVisual) "QueryAndPhysics")
  (Collision|SetCollisionEnabled (Variables|Default|GetEnemyDetector) "QueryOnly")
  (Collision|SetCollisionEnabled (Variables|Default|GetPlayerDetector) "QueryOnly")
  (bind _output_get (Variables|Default|SetInitialOverlappingActors (Collision|GetOverlappingActors _enemydetector "/Game/Users/Dylan/EnemyBlueprints/Erg_AI/BP_ErgCrawlerEnemy.BP_ErgCrawlerEnemy_C" :!class /Script/Engine.PrimitiveComponent)))
  (Utilities|Array|AppendArray _output_get (Collision|GetOverlappingActors _enemydetector "/Game/Users/Dylan/EnemyBlueprints/Shroombo_AI/BP_ShroomboEnemyNEW.BP_ShroomboEnemyNEW_C" :!class /Script/Engine.PrimitiveComponent))
  (bind _output_get_2 (Variables|Default|SetOverlappingPlayers (Collision|GetOverlappingActors (Variables|Default|GetPlayerDetector) "/Game/LevelStuff/ThirdPerson/Blueprints/Movement/BP_ThirdPersonCharacter.BP_ThirdPersonCharacter_C" :!class /Script/Engine.PrimitiveComponent)))
  (for _array_element _output_get_2
    (if (Actor|ActorHasTag _array_element "Player")
      (Variables|Default|SetIfPlayerSpawnedInside true)))
  (if (Variables|Default|GetIfPlayerSpawnedInside)
    (if (Utilities|Array|IsNotEmpty (Variables|Default|GetOverlappingPlayers))
      (CallFunction|PlayerSpawnedInside))))

(event Collision|EventActorBeginOverlap
  (params (OtherActor :type Actor%20Object%20Reference))
  (bind _enemydetector (Variables|Default|GetEnemyDetector))
  ;[1 0.426 0.02583] When Enemies are Detected or Killed inside the gate, calculate the total amount of enemies within!
  (bind _output_get (Variables|Default|SetOverlapping%20Actors (Collision|GetOverlappingActors _enemydetector "/Game/Users/Dylan/EnemyBlueprints/Erg_AI/BP_ErgCrawlerEnemy.BP_ErgCrawlerEnemy_C" :!class /Script/Engine.PrimitiveComponent)))
  (Utilities|Array|AppendArray _output_get (Collision|GetOverlappingActors _enemydetector "/Game/Users/Dylan/EnemyBlueprints/Shroombo_AI/BP_ShroomboEnemyNEW.BP_ShroomboEnemyNEW_C" :!class /Script/Engine.PrimitiveComponent))
  (if (Variables|Default|GetGateTriggeredByPlayer)
    ;;[1 0.6902 0] See bottom right!
    (CallFunction|EnemyMatOverlay)
    (bind _output_get_2 (Variables|Default|SetEnemiesWithin (Utilities|Array|Length (Variables|Default|GetOverlapping%20Actors))))
    ;;[0.5469 1 0.5704] See bottom left!
    (CallFunction|EnemyCleared _output_get_2)
    (Rendering|Components|TextRender|SetText (Variables|Default|GetEnemyCounter) (Utilities|Text|ToText(Integer) (Variables|Default|GetEnemiesWithin)))
    (CallFunction|FacePlayer)))

(event Collision|EventActorEndOverlap
  (params (OtherActor :type Actor%20Object%20Reference))
  (bind _enemydetector (Variables|Default|GetEnemyDetector))
  ;[1 0.426 0.02583] When Enemies are Detected or Killed inside the gate, calculate the total amount of enemies within!
  (bind _output_get (Variables|Default|SetOverlapping%20Actors (Collision|GetOverlappingActors _enemydetector "/Game/Users/Dylan/EnemyBlueprints/Erg_AI/BP_ErgCrawlerEnemy.BP_ErgCrawlerEnemy_C" :!class /Script/Engine.PrimitiveComponent)))
  (Utilities|Array|AppendArray _output_get (Collision|GetOverlappingActors _enemydetector "/Game/Users/Dylan/EnemyBlueprints/Shroombo_AI/BP_ShroomboEnemyNEW.BP_ShroomboEnemyNEW_C" :!class /Script/Engine.PrimitiveComponent))
  (if (Variables|Default|GetGateTriggeredByPlayer)
    ;;[1 0.6902 0] See bottom right!
    (CallFunction|EnemyMatOverlay)
    (bind _output_get_2 (Variables|Default|SetEnemiesWithin (Utilities|Array|Length (Variables|Default|GetOverlapping%20Actors))))
    ;;[0.5469 1 0.5704] See bottom left!
    (CallFunction|EnemyCleared _output_get_2)
    (Rendering|Components|TextRender|SetText (Variables|Default|GetEnemyCounter) (Utilities|Text|ToText(Integer) (Variables|Default|GetEnemiesWithin)))
    (CallFunction|FacePlayer)))

(fn ConstructionScript)