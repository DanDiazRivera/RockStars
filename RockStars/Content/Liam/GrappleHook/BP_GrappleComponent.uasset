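; Grappling hook component that pulls its owning Character toward whatever the fired hook hits.
; FireGrapple spawns a hook projectile and a cable linking it to the owner.
; On hit, it overrides friction, gravity and air control, launches the character, then applies pulling force each Tick.
; The hook is destroyed on cancel, proximity or overshoot (2D dot-product check), which removes the cable and restores the cached movement settings.
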(event EventTick
  (params (DeltaSeconds :type Float%20%28single-precision%29))
  (switch Utilities|FlowControl|Switch|SwitchonE_GrappleState (Variables|Default|GetGrappleState)
    (:NewEnumerator2
      (bind _ascharacter (Utilities|Casting|CastToCharacter (Components|GetOwner)))
      (Physics|AddForce (Variables|/Script/Engine.Character|GetCharacterMovement _ascharacter) (* (Utilities|ToGrappleHook) (Variables|Constants|GetGrapplePullForce)))
      (if (< (Math|Vector|Distance(Vector) (Transformation|GetActorLocation (Variables|Default|GetGrappleHook)) (Transformation|GetActorLocation (Components|GetOwner))) 2.5e+02)
        (Actor|DestroyActor (Variables|Default|GetGrappleHook))
        (elif (< (Math|Vector|DotProduct (Variables|Default|GetInitialHookDirection2D) (Utilities|ToGrappleHook2D)) 0.0)
          (Actor|DestroyActor (Variables|Default|GetGrappleHook)))))))

(event EventBeginPlay
  (bind _ascharacter (Utilities|Casting|CastToCharacter (Components|GetOwner)))
  (Variables|Default|SetOriginalGroundFriction (Variables|/Script/Engine.CharacterMovementComponent|GetGroundFriction (Variables|/Script/Engine.Character|GetCharacterMovement _ascharacter)))
  (Variables|Default|SetOriginalGravityScale (Variables|/Script/Engine.CharacterMovementComponent|GetGravityScale (Variables|/Script/Engine.Character|GetCharacterMovement _ascharacter)))
  (Variables|Default|SetOriginalAirControl (Variables|/Script/Engine.CharacterMovementComponent|GetAirControl (Variables|/Script/Engine.Character|GetCharacterMovement _ascharacter))))

(fn IsinUse?
  (return (Utilities|Select :Index (Variables|Default|GetGrappleState) :NewEnumerator0 false :NewEnumerator1 true :NewEnumerator2 true)))

(fn FireGrapple
  (params (TargetLocation :type Vector) (LocalOffset :type Vector))
  (if (not (CallFunction|IsinUse?))
    (Variables|Default|SetGrappleState "NewEnumerator1")
    (LocalVariables|SetFireDirection (Math|Vector|Normalize (- TargetLocation (Utilities|CableStartLocation LocalOffset))))
    (bind _returnvalue (Game|SpawnActorfromClass "/Game/Liam/GrappleHook/BP_GrappleHook.BP_GrappleHook_C" (Math|Transform|MakeTransform (Utilities|CableStartLocation LocalOffset) "0, 0, 0" "1.000000,1.000000,1.000000") "Undefined" "MultiplyWithRoot" 0 (* (LocalVariables|GetFireDirection) (Variables|Constants|GetGrapleHookSpeed)) 3.5e+03 0))
    (bind _output_get (Variables|Default|SetGrappleHook _returnvalue))
    (Collision|BindEventtoOnActorHit _output_get (EventDispatchers|CreateEvent :!event OnGrappleHookHit))
    (Game|BindEventtoOnDestroyed (Variables|Default|GetGrappleHook) (EventDispatchers|CreateEvent :!event OnGrappleHookDestroyed))
    (bind _returnvalue_2 (Game|SpawnActorfromClass "/Game/Liam/GrappleHook/BP_GrappleCable.BP_GrappleCable_C" (Math|Transform|MakeTransform (Utilities|CableStartLocation LocalOffset) (Math|Rotator|MakeRotfromX (LocalVariables|GetFireDirection)) "1.000000,1.000000,1.000000") "Undefined" "MultiplyWithRoot" 0 0))
    (bind _output_get_2 (Variables|Default|SetGrappleCable _returnvalue_2))
    (Transformation|AttachActorToActor _output_get_2 (Components|GetOwner) "None" "KeepWorld" "KeepWorld" "KeepWorld" true)
    (Class|CableComponent|SetAttachEndto (Variables|/Script/CableComponent.CableActor|GetCableComponent (Variables|Default|GetGrappleCable)) (Variables|Default|GetGrappleHook) "None" "None")
    (Variables|/Script/CableComponent.CableComponent|SetEndLocation (Variables|/Script/CableComponent.CableActor|GetCableComponent (Variables|Default|GetGrappleCable)) "0, 0, 0")))

(fn CancelGrapple
  (bind _grapplehook (Variables|Default|GetGrappleHook)
    (:then
      (Actor|DestroyActor _grapplehook))
    (:else)))

(fn OnGrappleHookHit
  (params (SelfActor :type Actor%20Object%20Reference) (OtherActor :type Actor%20Object%20Reference) (NormalImpulse :type Vector) (Hit :type Hit%20Result%20Structure%20%28by%20ref%29))
  (Variables|Default|SetGrappleState "NewEnumerator2")
  (bind _ascharacter (Utilities|Casting|CastToCharacter (Components|GetOwner)))
  (Variables|/Script/Engine.CharacterMovementComponent|SetGroundFriction (Variables|/Script/Engine.Character|GetCharacterMovement _ascharacter) 0.0)
  (Variables|/Script/Engine.CharacterMovementComponent|SetGravityScale (Variables|/Script/Engine.Character|GetCharacterMovement _ascharacter) 0.0)
  (Variables|/Script/Engine.CharacterMovementComponent|SetAirControl (Variables|/Script/Engine.Character|GetCharacterMovement _ascharacter) 0.2)
  (Variables|/Script/Engine.MovementComponent|SetVelocity (Variables|/Script/Engine.Character|GetCharacterMovement _ascharacter) (* (Utilities|ToGrappleHook) (Variables|Constants|GetInitialGrapplePullForce)))
  (Variables|Default|SetInitialHookDirection2D (Utilities|ToGrappleHook2D)))

(fn OnGrappleHookDestroyed
  (params (DestroyedActor :type Actor%20Object%20Reference))
  (Variables|Default|SetGrappleHook 0)
  (Variables|Default|SetGrappleState "NewEnumerator0")
  (Utilities|FlowControl|Sequence
    (:then_0
      (bind _grapplecable (Variables|Default|GetGrappleCable)
        (:then
          (Actor|DestroyActor _grapplecable)
          (Variables|Default|SetGrappleCable 0))
        (:else)))
    (:then_1
      (bind _ascharacter (Utilities|Casting|CastToCharacter (Components|GetOwner)))
      (Variables|/Script/Engine.CharacterMovementComponent|SetGroundFriction (Variables|/Script/Engine.Character|GetCharacterMovement _ascharacter) (Variables|Default|GetOriginalGroundFriction))
      (Variables|/Script/Engine.CharacterMovementComponent|SetGravityScale (Variables|/Script/Engine.Character|GetCharacterMovement _ascharacter) (Variables|Default|GetOriginalGravityScale))
      (Variables|/Script/Engine.CharacterMovementComponent|SetAirControl (Variables|/Script/Engine.Character|GetCharacterMovement _ascharacter) (Variables|Default|GetOriginalAirControl)))))