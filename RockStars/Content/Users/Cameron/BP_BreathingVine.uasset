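; BP_BreathingVine is a vine prop whose glow and point light pulse together in a breathing effect.
; On BeginPlay it creates a dynamic material instance for the static mesh, stores the light's starting intensity, then waits a random delay so instances vary in timing.
; The BREATHE timeline then drives both the VineEmissive material parameter and the light intensity, scaling the latter between zero and its starting value.
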(event EventTick
  (params (DeltaSeconds :type Float%20%28single-precision%29)))

(event EventBeginPlay
  (bind _staticmesh (Variables|Default|GetStaticMesh))
  ;[0.04964 1 0] Creates dynamic material instance for the static mesh to control its emissive
  (bind _returnvalue (Rendering|Material|CreateDynamicMaterialInstance _staticmesh 0 (Rendering|Material|GetMaterial _staticmesh 0) "None" :!class /Script/Engine.PrimitiveComponent))
  (Variables|Default|SetVine%20Material _returnvalue)
  ;[0.3012 1 0.6906] Sets default point light intensity
  (Variables|Default|SetInitialIntensity (Variables|/Script/Engine.LightComponentBase|GetIntensity (Variables|Default|GetPointLight)))
  ;[0.1978 0.9901 1] Delay for random variance
  (Utilities|FlowControl|Delay (Math|Random|RandomFloatinRange 0.5 4.0))
  ;[1 0.3958 0.3958] Timeline that controls material emissive, and point light intensity
  (bind _breathing (Timeline|BREATHE Play)
    (:Update
      ;[0.8322 0.4238 1] Manipulation of material emissive and point light intensity
      (Rendering|Material|SetScalarParameterValue (Variables|Default|GetVine%20Material) "VineEmissive" (Math|Float|Lerp 0.0 1.0 _breathing) :!class /Script/Engine.MaterialInstanceDynamic)
      (Rendering|Components|Light|SetIntensity (Variables|Default|GetPointLight) (Math|Float|Lerp 0.0 (Variables|Default|GetInitialIntensity) _breathing)))))

(fn ConstructionScript)