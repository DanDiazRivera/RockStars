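; Crystal actor whose point light and emissive glow respond to player distance, dimming as the player gets closer.
; BeginPlay creates a dynamic material instance and stores the light's starting intensity as the maximum.
; Tick scales light intensity and emissive tint from distance, with clamping.
; A Reaction timeline plays within ReactionDistance and reverses outside it, lerping emissive between zero and the distance-based value.
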(event EventTick
  (params (DeltaSeconds :type Float%20%28single-precision%29))
  (bind _crystal_material (Variables|Default|GetCrystal%20Material))
  ;[0.11 0.5168 1] Run time
  (bind _output_get (Variables|Default|SetPlayerDistance (Transformation|GetDistanceTo self (Game|GetPlayerCharacter 0))))
  (bind _output_get_2 (Variables|Default|SetCurrent%20intensity _output_get))
  (Rendering|Components|Light|SetIntensity (Variables|Default|GetPointLight) (Math|Float|Clamp(Float) (* _output_get_2 5.0) 0.0 (Variables|Default|GetMaxIntensity)))
  (bind _output_get_3 (Variables|Default|SetCrystal%20Emissive (Math|Float|Clamp(Float) (/ (Variables|Default|GetPlayerDistance) 1e+02) 0.0 1e+01)))
  (Rendering|Material|SetScalarParameterValue _crystal_material "Emissive Tint Intensity" _output_get_3 :!class /Script/Engine.MaterialInstanceDynamic)
  (if (>= (Variables|Default|GetReactionDistance) (Variables|Default|GetPlayerDistance))
    (bind _reaction (Timeline|Reaction Play)
      (:Update
        (Rendering|Material|SetScalarParameterValue _crystal_material "Emissive Tint Intensity" (Math|Float|Lerp 0.0 (Variables|Default|GetCrystal%20Emissive) _reaction) :!class /Script/Engine.MaterialInstanceDynamic)))
    (else
      (Timeline|Reaction Reverse))))

(event EventBeginPlay
  (bind _staticmesh (Variables|Default|GetStaticMesh))
  ;[1 1 1] Set up
  (bind _returnvalue (Rendering|Material|CreateDynamicMaterialInstance _staticmesh 0 (Rendering|Material|GetMaterial _staticmesh 0) "None" :!class /Script/Engine.PrimitiveComponent))
  (Variables|Default|SetCrystal%20Material _returnvalue)
  (Variables|Default|SetMaxIntensity (Variables|/Script/Engine.LightComponentBase|GetIntensity (Variables|Default|GetPointLight))))

(fn ConstructionScript)