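; BP_DynamicVine is a Blueprint that moves a point light along a spline over time.
; Each Tick advances a distance by SplineSpeed scaled by delta time, samples the spline in local space, and sets the light's relative location there with a fixed rotation.
; When Loop is enabled, the distance resets to zero after it passes the spline's length.
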(event EventTick
  (params (DeltaSeconds :type Float%20%28single-precision%29))
  (Variables|Default|SetDistance%20Along%20Spline (+ (* DeltaSeconds (Variables|Default|GetSpline%20Speed)) (Variables|Default|GetDistance%20Along%20Spline)))
  (Transformation|SetRelativeTransform (Variables|Default|GetPointLight) (Math|Transform|MakeTransform (.location (Spline|GetTransformatDistanceAlongSpline (Variables|Default|GetSpline) (Variables|Default|GetDistance%20Along%20Spline) "Local" false)) "0.000000,90.000000,0.000000" "1.000000,1.000000,1.000000") false false)
  (if (Variables|Default|GetLoop?)
    (if (> (Variables|Default|GetDistance%20Along%20Spline) (Spline|GetSplineLength (Variables|Default|GetSpline)))
      (Variables|Default|SetDistance%20Along%20Spline 0.0))))

(fn ConstructionScript)