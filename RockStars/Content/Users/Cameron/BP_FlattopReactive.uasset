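; BP_FlattopReactive is a flattop mushroom prop that glows when the third-person player character comes near.
; On BeginPlay it creates a dynamic material instance from the static mesh and zeroes its Emissive parameter.
; Entering the Trigger volume plays the React timeline, which lerps Emissive up to a soft glow, and leaving reverses it so the glow fades out.
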(event OnComponentBeginOverlap(Trigger)
  (params (OverlappedComponent :type Primitive%20Component%20Object%20Reference) (OtherActor :type Actor%20Object%20Reference) (OtherComp :type Primitive%20Component%20Object%20Reference) (OtherBodyIndex :type Integer) (bFromSweep :type Boolean) (SweepResult :type Hit%20Result%20Structure%20%28by%20ref%29))
  (Utilities|Casting|CastToBP_ThirdPersonCharacter OtherActor)
  (bind _react (Timeline|react Play)
    (:Update
      (Rendering|Material|SetScalarParameterValue (Variables|Default|GetMushroom%20Material) "Emissive" (Math|Float|Lerp 0.0 0.55 _react) :!class /Script/Engine.MaterialInstanceDynamic))))

(event OnComponentEndOverlap(Trigger)
  (params (OverlappedComponent :type Primitive%20Component%20Object%20Reference) (OtherActor :type Actor%20Object%20Reference) (OtherComp :type Primitive%20Component%20Object%20Reference) (OtherBodyIndex :type Integer))
  (Utilities|Casting|CastToBP_ThirdPersonCharacter OtherActor)
  (bind _react (Timeline|react Reverse)
    (:Update
      (Rendering|Material|SetScalarParameterValue (Variables|Default|GetMushroom%20Material) "Emissive" (Math|Float|Lerp 0.0 0.55 _react) :!class /Script/Engine.MaterialInstanceDynamic))))

(event EventBeginPlay
  (bind _staticmesh (Variables|Default|GetStaticMesh))
  (bind _returnvalue (Rendering|Material|CreateDynamicMaterialInstance _staticmesh 0 (Rendering|Material|GetMaterial _staticmesh 0) "None" :!class /Script/Engine.PrimitiveComponent))
  (bind _output_get (Variables|Default|SetMushroom%20Material _returnvalue))
  (Rendering|Material|SetScalarParameterValue _output_get "Emissive" 0.0 :!class /Script/Engine.MaterialInstanceDynamic))

(fn ConstructionScript)