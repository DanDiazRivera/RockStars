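; Glowing plant actor that pulses its emissive materials and point light like a heartbeat.
; BeginPlay creates dynamic materials for mesh slots 1 and 2 and stores the light's starting intensity.
; Tick plays the Heartbeat timeline through a random Delay to vary timing.
; The timeline curve drives both PlantEmissive parameters and scales the light between off and its starting intensity.
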(event EventTick
  (params (DeltaSeconds :type Float%20%28single-precision%29))
  ;[1 1 1] Creates a delay for random variance in execution
  (Utilities|FlowControl|Delay (Math|Random|RandomFloatinRange 0.5 4.0))
  ;[1 0.7742 0] Timeline controls the emissive values and also point light intensity
  (bind _heartbeat (Timeline|Heartbeat Play)
    (:Update
      (Rendering|Material|SetScalarParameterValue (Variables|Default|GetPlant%20Material) "PlantEmissive" (Math|Float|Lerp 0.0 1.0 _heartbeat) :!class /Script/Engine.MaterialInstanceDynamic)
      (Rendering|Material|SetScalarParameterValue (Variables|Default|GetPlant%20Material2) "PlantEmissive" (Math|Float|Lerp 0.0 1.0 _heartbeat) :!class /Script/Engine.MaterialInstanceDynamic)
      (Rendering|Components|Light|SetIntensity (Variables|Default|GetPointLight) (Math|Float|Lerp 0.0 (Variables|Default|GetInitial%20Intensity) _heartbeat)))))

(event EventBeginPlay
  (bind _staticmesh (Variables|Default|GetStaticMesh))
  (bind _staticmesh_2 (Variables|Default|GetStaticMesh))
  ;[0.2157 1 0.2198] Get Static mesh, and then create a dynamic material of SLOT 1
  (bind _returnvalue (Rendering|Material|CreateDynamicMaterialInstance _staticmesh 1 (Rendering|Material|GetMaterial _staticmesh 1) "None" :!class /Script/Engine.PrimitiveComponent))
  (Variables|Default|SetPlant%20Material _returnvalue)
  ;[0 0.6908 1] Creating a dynamic material instance of Mat. Slot 2
  (bind _returnvalue_2 (Rendering|Material|CreateDynamicMaterialInstance _staticmesh_2 2 (Rendering|Material|GetMaterial _staticmesh_2 2) "None" :!class /Script/Engine.PrimitiveComponent))
  (Variables|Default|SetPlant%20Material2 _returnvalue_2)
  ;[0.1056 0 1] Initial Point Light Intensity
  (Variables|Default|SetInitial%20Intensity (Variables|/Script/Engine.LightComponentBase|GetIntensity (Variables|Default|GetPointLight))))

(fn ConstructionScript)