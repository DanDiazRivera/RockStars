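; Boss finishing-blow component that plays a cinematic hit-stop on a boss and its attacker.
; StartSequence snaps a camera spawned at BeginPlay toward the boss, enables a post-process material, marks both actors with custom depth stencil, box-traces to hide surrounding actors and spawns an emitter.
; ManageTime applies stop dilation per actor, then switches to slow dilation while blending back to the player, clearing the material and unhiding actors.
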(event Custom|StartSequence
  (params (TargetActor :type Actor%20Object%20Reference) (DistanceAlpha :type Float%20%28single-precision%29) (AttackingActor :type Actor%20Object%20Reference) (StopDilation :type Float%20%28single-precision%29) (StopDuration :type Float%20%28single-precision%29) (SlowDilation :type Float%20%28single-precision%29) (SlowDuration :type Float%20%28single-precision%29))
  (bind _array (Utilities|Array|MakeArray TargetActor AttackingActor))
  ;[0.9107 0.3733 1] When the sequence begins, snap the camera to the boss and play out the sequence!
  (CallFunction|FunctSnapCamtoBoss TargetActor DistanceAlpha)
  (CallFunction|ManageTime _array StopDilation StopDuration SlowDilation SlowDuration)
  (CallFunction|FunctSetPostProcessMat true)
  (CallFunction|FunctApplyDepthtoMeshes _array)
  (CallFunction|FunctHideMeshes TargetActor _array)
  (CallFunction|FunctSpawnEffects TargetActor))

(event Custom|ManageTime
  (params (AffectedActors :type Array%20of%20Actor%20Object%20References) (StopDilation :type Float%20%28single-precision%29) (StopDuration :type Float%20%28single-precision%29) (SlowDilation :type Float%20%28single-precision%29) (SlowDuration :type Float%20%28single-precision%29))
  ;[0.7047 0.6108 1] Time stops, then progresses slowly, then resumes to the standard!
  (CallFunction|FunctSetActorTimeDilation AffectedActors StopDilation)
  (Utilities|FlowControl|Delay StopDuration)
  (Game|Player|SetViewTargetwithBlend (Game|GetPlayerController 0) (Game|Player|GetPlayerPawn 0) SlowDuration "VTBlend_Linear" 0.0 false)
  (CallFunction|FunctSetPostProcessMat false)
  (CallFunction|FunctResetHiddenActors)
  (CallFunction|FunctSetActorTimeDilation AffectedActors SlowDilation)
  (Utilities|FlowControl|Delay SlowDuration))

(event EventBeginPlay
  ;[0.5059 1 0.5446] On Begin Play, create a camera to zoom onto the boss with!
  (Utilities|FlowControl|Sequence
    (:then_0
      (bind _returnvalue (Game|SpawnActorfromClass "/Script/Engine.CameraActor" (Math|Transform|MakeTransform "0, 0, 0" "0, 0, 0" "1.000000,1.000000,1.000000") "Undefined" "MultiplyWithRoot" 0 0))
      (bind _output_get (Variables|Default|SetBossDeathCam _returnvalue))
      (Class|CameraComponent|SetConstraintAspectRatio (Variables|/Script/Engine.CameraActor|GetCameraComponent _output_get) false))
    (:then_1
      (bind _returnvalue_2 (Actor|GetActorOfClass "/Script/Engine.PostProcessVolume"))
      (bind _output_get_2 (Variables|Default|SetPostProcessVolume _returnvalue_2))
      (Utilities|IsValid _output_get_2
        (:Is%20Not%20Valid
          (Development|PrintString "PPV not found in this Level!"))))))

(fn FunctSnapCamtoBoss
  (params (TargetActor :type Actor%20Object%20Reference) (DistanceAlpha :type Float%20%28single-precision%29))
  (bind _returnvalue (Game|GetPlayerCameraManager 0))
  (bind _returnvalue_2 (Camera|GetCameraLocation _returnvalue))
  (Transformation|SetActorLocation (Variables|Default|GetBossDeathCam) (Math|Vector|Lerp(Vector) (Transformation|GetActorLocation TargetActor) _returnvalue_2 DistanceAlpha) false false)
  (Transformation|SetActorRotation (Variables|Default|GetBossDeathCam) (Math|Rotator|FindLookatRotation _returnvalue_2 (Transformation|GetActorLocation TargetActor)))
  (Game|Player|SetViewTargetwithBlend (Game|GetPlayerController 0) (Variables|Default|GetBossDeathCam) 0.0 "VTBlend_Linear" 0.0 false))

(fn FunctSetActorTimeDilation
  (params (Array :type Array%20of%20Actor%20Object%20References) (Custom%20Time%20Dilation :type Float%20%28single-precision%29))
  (for _array_element Array
    (Variables|/Script/Engine.Actor|SetCustomTimeDilation _array_element Custom%20Time%20Dilation))
  (return))

(fn FunctSetPostProcessMat
  (params (SetActive :type Boolean))
  (Utilities|Struct|SetmembersinPostProcessSettings (Variables|/Script/Engine.PostProcessVolume|GetSettings (Variables|Default|GetPostProcessVolume)) (Utilities|Struct|MakeWeightedBlendables (Utilities|Array|MakeArray (Utilities|Struct|MakeWeightedBlendable (select SetActive 1.0 0.0) "/Game/Users/Dylan/EnemyBlueprints/BossStopMats/PPMI_BossStop.PPMI_BossStop")))))

(fn FunctApplyDepthtoMeshes
  (params (AffectedActors :type Array%20of%20Actor%20Object%20References))
  (for _array_element AffectedActors
    (for _array_element_2 (Actor|GetComponentsByClass _array_element "/Script/Engine.StaticMeshComponent")
      (Rendering|SetRenderCustomDepth _array_element_2 true)
      (Rendering|SetCustomDepthStencilValue _array_element_2 1))
    (for _array_element_3 (Actor|GetComponentsByClass _array_element "/Script/Engine.SkeletalMeshComponent")
      (Rendering|SetRenderCustomDepth _array_element_3 true)
      (Rendering|SetCustomDepthStencilValue _array_element_3 1))))

(fn FunctHideMeshes
  (params (TargetActor :type Actor%20Object%20Reference) (ActorsToIgnore :type Array%20of%20Actor%20Object%20References))
  (bind _bossdeathcam (Variables|Default|GetBossDeathCam))
  (bind _returnvalue (Transformation|GetActorLocation TargetActor))
  (bind _returnvalue_2 (Transformation|GetActorLocation _bossdeathcam))
  (bind _outhits (Class|KismetSystemLibrary|BoxTraceMultiforObjects _returnvalue_2 _returnvalue "2000.000000,2000.000000,2000.000000" (Math|Rotator|FindLookatRotation _returnvalue_2 _returnvalue) (Utilities|Array|MakeArray "ObjectTypeQuery1" "ObjectTypeQuery2" "ObjectTypeQuery4") false 0 "ForDuration" true))
  (for _array_element _outhits
    (Utilities|Array|Add (Variables|Default|GetHiddenActors) (.HitActor (Collision|BreakHitResult _array_element)))
    (Rendering|SetActorHiddenInGame (.HitActor (Collision|BreakHitResult _array_element)) true)))

(fn FunctResetHiddenActors
  (bind _hiddenactors (Variables|Default|GetHiddenActors))
  (for _array_element _hiddenactors
    (Rendering|SetActorHiddenInGame _array_element false))
  (Utilities|Array|Clear _hiddenactors))

(fn FunctSpawnEffects
  (params (TargetActor :type Actor%20Object%20Reference))
  (Effects|SpawnEmitteratLocation 0 (+ (Transformation|GetActorLocation TargetActor) (* (Math|Vector|GetForwardVector (Math|Rotator|FindLookatRotation (Transformation|GetActorLocation (Variables|Default|GetBossDeathCam)) (Transformation|GetActorLocation TargetActor))) (Variables|Default|GetEffectDistance))) "0, 0, 0" "10.000000,10.000000,10.000000"))