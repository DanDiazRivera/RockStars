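; Base enemy character with an overridable attack event, driving AI through Blackboard keys for detection, aggro, damage and stun.
; Pawn Sensing sets aggro, and retriggerable delays drop it once sightings stop.
; ModelSwap uses aggro to toggle hiding and full meshes, health bar, noise and smoke puff.
; Player strikes on aggro enemies cause knockback, hit stun or ragdoll death; a separate stun temporarily freezes them; hitstop is unfinished.
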(event OnSeePawn(PawnSensing)
  (params (Pawn :type Pawn%20Object%20Reference))
  ;[1 0.05881 0.009047] CONTROL AI VIA PAWN SENSING!
  (bind _aliveandhealthy (CallFunction|AliveandHealthyCheck))
  (if _aliveandhealthy
    (Utilities|FlowControl|Sequence
      (:then_0
        (CallFunction|SetEnemyPursueMode Pawn))
      (:then_1
        (CallFunction|SetEnemyRoamMode))
      (:then_2
        (CallFunction|SetEnemyHideMode)))))

(event Custom|SetEnemyPursueMode
  (params (3PC :type Pawn%20Object%20Reference))
  (bind _self self)
  (bind _returnvalue (AI|GetAIController _self))
  (bind _returnvalue_2 (AI|GetBlackboard _returnvalue))
  ;[1 0.2345 0.1747] Player is Detected - Aggro!
  (Variables|BoolChecks|SetAggro true)
  (Utilities|Casting|CastToBP_ThirdPersonCharacter 3PC)
  (AI|Components|Blackboard|SetValueasBool _returnvalue_2 (Utilities|Name|MakeLiteralName "PlayerDetected") true)
  (AI|Components|Blackboard|SetValueasBool _returnvalue_2 (Utilities|Name|MakeLiteralName "IsEnemyAggro") true))

(event Custom|Enemy%20Knockback
  ;[1 0.2471 0.1255 0.353] EXTRA DAMAGE CONTROL
  ;;[1 0.7294 0.2588] (TO DO) MAD SCIENCE: Knockback 1st Pass - FIX BUGS!
  (CallFunction|RegisterDamage)
  (Character|LaunchCharacter (+ (* (Transformation|GetActorForwardVector) -1e+02) "0.000000,0.000000,100.000000") true false))

(event Custom|LeadElectricStun
  (bind _self self)
  (bind _returnvalue (AI|GetAIController _self))
  ;[0.9098 1 0.2078] When enemies are stunned, they freeze in place, become vulnerable and lose sight of player until healthy again!
  (if (and (not (Variables|BoolChecks|GetIsStunned)) (Variables|BoolChecks|GetAggro))
    (Audio|Components|Audio|Stop (Variables|Default|GetBaseNoise))
    (AI|Navigation|StopMovement _returnvalue)
    (Development|PrintString "Enemy Stun Successful!" true true "(R=0.660055,G=1.000000,B=0.140704,A=1.000000)" 3.0)
    (bind _output_get (Variables|BoolChecks|SetIsStunned true))
    (Animation|Montage|PlayMontage (Variables|Character|GetMesh) (Variables|Montages|GetLE%20Stun%20Montage) 2.0
      (:then
        (AI|Components|Blackboard|SetValueasBool (AI|GetBlackboard _returnvalue) (Utilities|Name|MakeLiteralName "IsEnemyStunned") _output_get)
        (Utilities|FlowControl|RetriggerableDelay (Variables|BaseVariables|GetStunPause))
        (CallFunction|LeadElectricStunEnd)))))

(event Custom|LeadElectricStunEnd
  (bind _self self)
  (bind _returnvalue (AI|GetAIController _self))
  (bind _returnvalue_2 (AI|GetBlackboard _returnvalue))
  ;[0.2031 0.1407 0.05699] Trigger Once Stun Duration Finishes!
  (Development|PrintString "Enemy Stun Concluded!" true true "(R=0.660055,G=1.000000,B=0.140704,A=1.000000)" 3.0)
  (bind _output_get (Variables|BoolChecks|SetIsStunned false))
  (AI|Components|Blackboard|SetValueasBool _returnvalue_2 (Utilities|Name|MakeLiteralName "IsEnemyStunned") _output_get)
  (bind _output_get_2 (Variables|BoolChecks|SetAggro true))
  (AI|Components|Blackboard|SetValueasBool _returnvalue_2 (Utilities|Name|MakeLiteralName "IsEnemyAggro") _output_get_2)
  (AI|Components|Blackboard|SetValueasBool _returnvalue_2 (Utilities|Name|MakeLiteralName "PlayerDetected") false))

(event Custom|Set%20Health%20Bar%20Name
  ;[0.016 0.2831 0.0319] Enemy's name is set inside Health Bar!
  (bind _aswbp_enemy_health_indicator (Utilities|Casting|CastToWBP_EnemyHealthIndicator (UserInterface|GetWidget (Variables|Default|GetHealth%20Bar))))
  (Variables|/Game/Assets/Enemies/EnemyUI/WBP_EnemyHealthIndicator.WBP_EnemyHealthIndicator_C|SetNameOfEnemy _aswbp_enemy_health_indicator (Variables|BaseVariables|GetNameOfEnemy)))

(event Custom|EnemyAttack
  ;[0.698 0.09412 0.1216] OVERRIDABLE ATTACK FUNCTION!
)

(event Custom|Face%20Player
  ;[1 0.6667 0.6745] Rotation Handling!
  (bind _aliveandhealthy (CallFunction|AliveandHealthyCheck))
  (if _aliveandhealthy
    (if (or (Variables|BoolChecks|GetSearchingForPlayer) (Variables|BoolChecks|GetTakingDamage))
      (Transformation|SetActorRotation (Math|Rotator|MakeRotator 0.0 0.0 (.yaw (Math|Interpolation|RInterpTo (Transformation|GetActorRotation) (Math|Rotator|FindLookatRotation (Transformation|GetActorLocation) (Transformation|GetActorLocation (Game|GetPlayerCharacter 0))) 0.0 1e+01))))
      (Utilities|FlowControl|Delay 0.01))))

(event Custom|SearchConditions
  ;[1 0.6667 0.6745] Rotation Handling!
  (if (Variables|BoolChecks|GetAggro)
    (Variables|BoolChecks|SetSearchingForPlayer true)
    (CallFunction|FacePlayer)
    (else
      (Variables|BoolChecks|SetSearchingForPlayer false)))
  (Utilities|FlowControl|Delay 0.01)
  (CallFunction|SearchConditions))

(event Custom|Register%20Damage
  (bind _self self)
  (bind _takingdamage (Variables|BoolChecks|GetTakingDamage))
  (bind _returnvalue (AI|GetAIController _self))
  ;[1 0.2471 0.1255 0.353] EXTRA DAMAGE CONTROL
  (AI|Components|Blackboard|SetValueasBool (AI|GetBlackboard _returnvalue) (Utilities|Name|MakeLiteralName "IsEnemyDamaged") _takingdamage)
  (if _takingdamage
    (AI|Navigation|StopMovement _returnvalue)
    (else
      (Pawn|Components|CharacterMovement|SetMovementMode (Variables|Character|GetCharacterMovement) "MOVE_Walking" 0))))

(event Custom|SetEnemyRoamMode
  ;[1 0.7554 0.3604] Player Out of Sight - Return to Roaming!
  (Utilities|FlowControl|RetriggerableDelay 3.0)
  (AI|Components|Blackboard|SetValueasBool (AI|GetBlackboard (AI|GetAIController self)) (Utilities|Name|MakeLiteralName "PlayerDetected") false))

(event Custom|SetEnemyHideMode
  (bind _self self)
  (bind _returnvalue (AI|GetAIController _self))
  ;[0.415 0.2753 1] No Longer Aggro - Hide!
  (Utilities|FlowControl|RetriggerableDelay 3.0)
  (Variables|BoolChecks|SetAggro false)
  (AI|Components|Blackboard|SetValueasBool (AI|GetBlackboard _returnvalue) (Utilities|Name|MakeLiteralName "IsEnemyAggro") (Variables|BoolChecks|GetAggro))
  (AI|Navigation|StopMovement _returnvalue))

(event Custom|SmokePuff
  (params (VFX :type Actor%20Class%20Reference))
  ;[1 0.7134 0.1637] VFX Spawn
  (Game|SpawnActorfromClass VFX (Transformation|GetActorTransform 0) "Undefined" "MultiplyWithRoot" 0 0))

(event Custom|Model%20Swap
  (params (VFX :type Actor%20Class%20Reference))
  (bind _aggro (Variables|BoolChecks|GetAggro))
  (bind _hidemesh (Variables|Default|GetHideMesh))
  (bind _hidemesh_2 (Variables|Default|GetHideMesh))
  (bind _mesh (Variables|Character|GetMesh))
  (bind _mesh_2 (Variables|Character|GetMesh))
  ;[0.7013 1 0.669] Model Swapping Command!
  (if (not (Variables|BoolChecks|GetIsDead))
    (CallFunction|DisplayHealthBar _aggro)
    (if _aggro
      ;;[1 0.3365 0.5813] Turn Full Model On & Hiding Model Off!
      (Rendering|SetVisibility _hidemesh false false)
      (Components|Activation|SetActive _hidemesh false false)
      (Rendering|SetVisibility _mesh_2 true false)
      (Components|Activation|SetActive _mesh_2 true false)
      (Audio|Components|Audio|Play (Variables|Default|GetBaseNoise) 0.0)
      (Utilities|FlowControl|DoOnce false :!label _label
        (:Completed
          ;;[1 0.7134 0.1637] VFX Spawn
          (CallFunction|SmokePuff VFX)))
      (else
        ;;[0.3594 0.2708 0.09624] Turn Full Model Off & Hiding Model On!
        (Rendering|SetVisibility _hidemesh_2 true false)
        (Components|Activation|SetActive _hidemesh_2 true false)
        (Rendering|SetVisibility _mesh false false)
        (Components|Activation|SetActive _mesh false false)
        (Audio|Components|Audio|Stop (Variables|Default|GetBaseNoise))
        (goto _label Reset)))))

(event Custom|Display%20Health%20Bar
  (params (Should%20Display :type Boolean))
  ;[0.372 1 0.3197] Health Bar should be visible when aggro!
  (Rendering|SetVisibility (Variables|Default|GetHealth%20Bar) Should%20Display false))

(event Custom|Rotate%20Health%20Bar
  (bind _health_bar (Variables|Default|GetHealth%20Bar))
  ;[0.6437 1 0.7751] Adjust Health Bar Rotation!
  (Transformation|SetWorldRotation _health_bar (Math|Rotator|FindLookatRotation (Transformation|GetWorldLocation _health_bar) (Transformation|GetWorldLocation (Variables|/Script/Engine.PlayerCameraManager|GetTransformComponent (Game|GetPlayerCameraManager 0)))) false false)
  (if (Variables|BoolChecks|GetAggro)
    (CallFunction|RotateHealthBar)))

(event Custom|Update%20Health%20Bar
  (params (CurrentHealth :type Float%20%28double-precision%29))
  ;[1 0.4375 0.4375] When an enemy takes damage, update the health bar's fill!
  (bind _aswbp_enemy_health_indicator (Utilities|Casting|CastToWBP_EnemyHealthIndicator (UserInterface|GetWidget (Variables|Default|GetHealth%20Bar))))
  (Progress|SetPercent (Variables|/Game/Assets/Enemies/EnemyUI/WBP_EnemyHealthIndicator.WBP_EnemyHealthIndicator_C|GetHealthBar _aswbp_enemy_health_indicator) (/ CurrentHealth 75.0)))

(event Custom|HitReact
  ;[0.7725 0.06667 0.3529] Enemy Takes Damage
  (if (Math|Boolean|ANDBoolean (not (Variables|BoolChecks|GetIsDead)) (not (Variables|BoolChecks|GetTakingDamage)) (Variables|BoolChecks|GetAggro))
    (Variables|BoolChecks|SetTakingDamage true)
    (bind _output_get (Variables|BaseVariables|SetHealthOfCharacter (- (Variables|BaseVariables|GetHealthOfCharacter) (stale EventStruckbyPlayer DamageOutput))))
    (CallFunction|UpdateHealthBar _output_get)
    (CallFunction|EnemyKnockback)
    (if (<= (Variables|BaseVariables|GetHealthOfCharacter) 0.0)
      (CallFunction|EnemyDeath)
      (Collision|SetCollisionResponsetoChannel (Variables|Collision|GetCapsuleComponent) "ECC_Pawn" "ECR_Ignore")
      (else
        ;;[0.05185 0.1405 1] HIT STUN!
        (Animation|Montage|PlayMontage (Variables|Character|GetMesh) (Variables|Montages|GetHit%20Stun%20Montage)
          (:then
            (Utilities|FlowControl|RetriggerableDelay 0.25)
            (Variables|BoolChecks|SetTakingDamage false)
            (CallFunction|RegisterDamage)))))))

(event Custom|EnemyDeath
  ;[0.188 0.1351 0.1351] Enemy is Dead
  (if (not (Variables|BoolChecks|GetIsDead))
    (bind _output_get (Variables|BoolChecks|SetIsDead true))
    (Variables|BoolChecks|SetIsDead _output_get) ; Blackboard Value!
    (Collision|SetCollisionEnabled (Variables|Character|GetMesh) "QueryAndPhysics") ; These three sequential steps are used to ragdoll the player mesh when HealthOfCharacter hits 0.
    (Physics|SetSimulatePhysics (Variables|Character|GetMesh) true)
    (Class|SkeletalMeshComponent|SetPhysicsBlendWeight (Variables|Character|GetMesh) 1.0)
    (Audio|Components|Audio|Stop (Variables|Default|GetBaseNoise))
    (Utilities|FlowControl|Delay 1.0)
    (Actor|DestroyActor)))

(event EventBeginPlay
  ;[0.276 0.01036 0.05452] Health Bar turns OFF until seen!
  (CallFunction|DisplayHealthBar false)
  (CallFunction|SetHealthBarName)
  ;[0.9734 0.1683 0] Saves Initial Transform for respawning
  (Variables|BaseVariables|SetInitialTransform (Transformation|GetActorTransform)))

(event EventStartHitstop
  (params (HitstopDuration :type Float%20%28double-precision%29) (3PC :type BP%20Third%20Person%20Character%20Object%20Reference))
  ;[0.1294 1 0.9098] EXPERIMENTAL: Hitstop 1st Pass - Freeze based on perfect hit timing and weapon index (SEE HIT DETECT FUNCTION IN 3PC -- CURRENTLY BUGGED)!
)

(event EventStruckbyPlayer
  (params (Player :type BP%20Third%20Person%20Character%20Object%20Reference) (DamageOutput :type Float%20%28double-precision%29))
  ;[1 0.4844 0.7588] Refer to BP_ThirdPersonCharacter's Hit Detect Function!
  (CallFunction|PlayHitSound)
  (CallFunction|HitReact))

(event EventStunnedbyPlayer
  (params (Player :type BP%20Third%20Person%20Character%20Object%20Reference) (ProjectileVelocity :type Vector :default "0, 0, 0") (ProjectileLocation :type Vector :default "0, 0, 0"))
  ;[0.902 0.8824 0.4941] Sound Wave puts enemy in Stun State!
  (CallFunction|LeadElectricStun))

(event EventEndHitstop
  ;[0.1294 1 0.9098] EXPERIMENTAL: Hitstop 1st Pass - Freeze based on perfect hit timing and weapon index (SEE HIT DETECT FUNCTION IN 3PC -- CURRENTLY BUGGED)!
  (Variables|Default|SetCustomTimeDilation 1.0))

(fn ConstructionScript)

(fn AliveandHealthyCheck
  (return (and (not (Variables|BoolChecks|GetIsDead)) (not (Variables|BoolChecks|GetIsStunned)))))

(fn AttackValidityCheck
  (bind _aliveandhealthy (CallFunction|AliveandHealthyCheck))
  (return (Math|Boolean|ANDBoolean _aliveandhealthy (not (Variables|BoolChecks|GetTakingDamage)) (not (Variables|BoolChecks|GetAttacking)))))

(fn PlayHitSound
  (bind _hit (Variables|Default|GetHit))
  (if (not (Audio|Components|Audio|IsPlaying _hit))
    (Audio|Components|Audio|Play _hit 0.0)))