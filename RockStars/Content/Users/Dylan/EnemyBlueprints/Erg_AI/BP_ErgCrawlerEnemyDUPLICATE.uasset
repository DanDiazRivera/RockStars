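; Duplicate Erg Crawler enemy that switches between hiding and pursuing the player, with a pounce attack.
; Mode changes set AI blackboard flags and call ModelSwap with a poof VFX; first pursuit registers it with the game mode for respawn as BP_ErgCrawlerEnemy.
; Valid attacks show anger VFX, then after a short delay lunge if the edge check passes, sphere-trace to trigger player HitReact, play the pounce montage and cool down.
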(event Custom|AddToRespawnable
  ;[0 0.09759 0.5841] Adds to Respawnable Struct Array so that Erg Crawler respawns on player death
  (bind _asbp_third_person_game_mode (Utilities|Casting|CastToBP_ThirdPersonGameMode (Game|GetGameMode)))
  (Utilities|Array|AddUnique (Variables|/Game/LevelStuff/ThirdPerson/Blueprints/Movement/BP_ThirdPersonGameMode.BP_ThirdPersonGameMode_C|GetRespawnableActors _asbp_third_person_game_mode) (Utilities|Struct|MakeStruct_RespawnableActors "/Game/Users/Dylan/EnemyBlueprints/Erg_AI/BP_ErgCrawlerEnemy.BP_ErgCrawlerEnemy_C" self (Variables|Default|GetInitialTransform))))

(event EventSetEnemyPursueMode
  (params (3PC :type Pawn%20Object%20Reference))
  (bind _self self)
  (bind _returnvalue (AI|GetAIController _self))
  (bind _returnvalue_2 (AI|GetBlackboard _returnvalue))
  ;[1 0.2345 0.1747] Player is Detected - Aggro!
  (Variables|Default|SetAggro true)
  (Utilities|Casting|CastToBP_ThirdPersonCharacter 3PC)
  (AI|Components|Blackboard|SetValueasBool _returnvalue_2 (Utilities|Name|MakeLiteralName "PlayerDetected") true)
  (AI|Components|Blackboard|SetValueasBool _returnvalue_2 (Utilities|Name|MakeLiteralName "IsEnemyAggro") true)
  (CallFunction|ModelSwap "/Game/Assets/VFX/ErgReveal/BP_ErgPoofVFX.BP_ErgPoofVFX_C")
  (CallFunction|SearchConditions)
  ;;[0 0.09804 0.5843] Calls Add to Respawnable once
  (Utilities|FlowControl|DoOnce false
    (:Completed
      (CallFunction|AddtoRespawnable))))

(event EventEnemyAttack
  ;[0.698 0.09412 0.1216] Sphere Trace for Pounce - TO REFINE WHEN ANIMATIONS ARE ADDED!
  (bind _attackisvalid (CallFunction|AttackValidityCheck))
  (if _attackisvalid
    (Game|SpawnActorfromClass "/Game/Assets/VFX/ShroomboAngerSymbol/BP_ShroomboAngerVFX.BP_ShroomboAngerVFX_C" (Utilities|AngryVFXSpawn) "Undefined" "MultiplyWithRoot" 0 0)
    (Utilities|FlowControl|Delay 0.5)
    (CallFunction|AttackingPlayer)
    (Variables|Default|SetAttacking true)
    (Animation|Montage|PlayMontage (Variables|Character|GetMesh) "/Game/Assets/Enemies/ErgCrawler/NewAnimation/ANM_ergAnimsRedo_Crab_rig_ergPounce_Montage.ANM_ergAnimsRedo_Crab_rig_ergPounce_Montage"
      (:OnCompleted
        _)
      (:OnInterrupted
        _))
    (Audio|Components|Audio|Play (Variables|Default|GetBaseNoise) 0.0)
    (Utilities|FlowControl|Delay (Variables|Default|GetAttackCooldown))
    (Variables|Default|SetAttacking false)))

(event EventSetEnemyHideMode
  (bind _self self)
  (bind _returnvalue (AI|GetAIController _self))
  ;[0.415 0.2753 1] No Longer Aggro - Hide!
  (Utilities|FlowControl|RetriggerableDelay 3.0)
  (Variables|Default|SetAggro false)
  (AI|Components|Blackboard|SetValueasBool (AI|GetBlackboard _returnvalue) (Utilities|Name|MakeLiteralName "IsEnemyAggro") (Variables|Default|GetAggro))
  (AI|Navigation|StopMovement _returnvalue)
  (CallFunction|ModelSwap "/Game/Assets/VFX/ErgReveal/BP_ErgPoofVFX.BP_ErgPoofVFX_C"))

(event EventAttackingPlayer
  (params (Player :type BP%20Third%20Person%20Character%20Object%20Reference))
  (bind _returnvalue (Transformation|GetActorLocation))
  ;[0.698 0.09412 0.1216] Sphere Trace for Pounce - TO REFINE WHEN ANIMATIONS ARE ADDED!
  ;;[0.202 1 0.5216] Attacking Message is Received - Attack Info!
  (Audio|Components|Audio|Stop (Variables|Default|GetBaseNoise))
  (bind _willstayinbounds (CallFunction|ChargeEdgeValidityCheck)) ; Only permits charge force if true!
  (if _willstayinbounds
    (CallFunction|ChargingLunge))
  (bind _outhit (Collision|SphereTraceForObjects _returnvalue _returnvalue 1e+02 (Utilities|Array|MakeArray "ObjectTypeQuery3") false 0 "None")) ; Hit Sphere for Pounce
  (bind _asbp_third_person_character (Utilities|Casting|CastToBP_ThirdPersonCharacter (.HitActor (Collision|BreakHitResult _outhit))))
  (Default|HitReact _asbp_third_person_character))

(fn ConstructionScript)