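; Erg Crawler enemy character that hides as a rock until it spots the player.
; PawnSensing sets aggro, swaps rock and creature meshes, and updates AI blackboard keys, with retriggerable delays dropping pursuit once sight is lost.
; A delayed pounce uses sphere traces to find and hit the player alongside a montage.
; Player strikes damage it only while aggro, stuns halt it briefly, and death ragdolls then destroys it.
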(event OnSeePawn(PawnSensing)
  (params (Pawn :type Pawn%20Object%20Reference))
  (bind _self self)
  (bind _self_2 self)
  (bind _returnvalue (AI|GetAIController _self))
  (bind _returnvalue_2 (AI|GetAIController _self_2))
  (bind _returnvalue_3 (AI|GetBlackboard _returnvalue_2))
  (if (and (not (Variables|Default|GetErgIsDead)) (not (Variables|Default|GetErgIsStunned)))
    (Utilities|FlowControl|Sequence
      (:then_0
        ;[1 0.2345 0.1747] Player is Detected - Pursue!
        (Variables|Default|SetAggro true)
        (CallFunction|ModelSwap self)
        (Utilities|Casting|CastToBP_ThirdPersonCharacter Pawn)
        (AI|Components|Blackboard|SetValueasBool _returnvalue_3 (Utilities|Name|MakeLiteralName "PlayerDetected") true)
        (AI|Components|Blackboard|SetValueasBool _returnvalue_3 (Utilities|Name|MakeLiteralName "IsEnemyAggro") true))
      (:then_1
        ;[1 0.7554 0.3604] Player Out of Sight - Return to Roaming!
        (Utilities|FlowControl|RetriggerableDelay 3.0)
        (AI|Components|Blackboard|SetValueasBool (AI|GetBlackboard (AI|GetAIController self)) (Utilities|Name|MakeLiteralName "PlayerDetected") false))
      (:then_2
        ;[0.415 0.2753 1] Erg No Longer Aggro - Hide in Shell!
        (Utilities|FlowControl|RetriggerableDelay 3.0)
        (Variables|Default|SetAggro false)
        (CallFunction|ModelSwap self)
        (AI|Components|Blackboard|SetValueasBool (AI|GetBlackboard _returnvalue) (Utilities|Name|MakeLiteralName "IsEnemyAggro") false)
        (AI|Navigation|StopMovement _returnvalue)))))

(event Custom|HitReact
  ;[0.774 0.06771 0.351] Enemy Takes Damage
  (if (Math|Boolean|ANDBoolean (not (Variables|Default|GetErgIsDead)) (not (Variables|Default|GetTakingDamage)) (Variables|Default|GetAggro))
    (Variables|Default|SetTakingDamage true)
    (bind _output_get (Variables|Default|SetHealthOfCharacter (- (Variables|Default|GetHealthOfCharacter) (Variables|/Game/LevelStuff/ThirdPerson/Blueprints/Movement/BP_ThirdPersonCharacter.BP_ThirdPersonCharacter_C|GetDamageOutput (stale EventStruckbyPlayer Player)))))
    (Development|PrintString (Utilities|String|ToString(Float) _output_get))
    (if (<= (Variables|Default|GetHealthOfCharacter) 0.0)
      (CallFunction|ErgDeath)
      (else
        (Utilities|FlowControl|RetriggerableDelay 0.25)
        (Variables|Default|SetTakingDamage false)))))

(event Custom|Model%20Swap
  (bind _rockhidemesh (Variables|Default|GetRockHideMesh))
  (bind _mesh (Variables|Character|GetMesh))
  (bind _rockhidemesh_2 (Variables|Default|GetRockHideMesh))
  (bind _mesh_2 (Variables|Character|GetMesh))
  (if (not (Variables|Default|GetErgIsDead))
    (if (Variables|Default|GetAggro)
      ;[1 0.3365 0.5813] Turn Full Model On & Rock Model Off!
      (Rendering|SetVisibility _rockhidemesh_2 false false)
      (Components|Activation|SetActive _rockhidemesh_2 false false)
      (Rendering|SetVisibility _mesh_2 true false)
      (Components|Activation|SetActive _mesh_2 true false)
      (else
        ;[0.3594 0.2708 0.09624] Turn Full Model Off & Rock Model On!
        (Rendering|SetVisibility _rockhidemesh true false)
        (Components|Activation|SetActive _rockhidemesh true false)
        (Rendering|SetVisibility _mesh false false)
        (Components|Activation|SetActive _mesh false false)))))

(event Custom|Erg%20Pounce
  (bind _mesh (Variables|Character|GetMesh))
  (bind _returnvalue (Transformation|GetWorldLocation _mesh))
  (if (not (Variables|Default|GetErgIsDead))
    ;[0.6979 0.09381 0.1216] Sphere Trace for Pounce - TO REFINE WHEN ANIMATIONS ARE ADDED!
    (bind _outhit (Collision|SphereTraceForObjects _returnvalue _returnvalue 5e+02 (Utilities|Array|MakeArray "ObjectTypeQuery3") false 0 "None")) ; This sphere is meant to find the player's mesh, using its coordinates for the pounce.
    (Utilities|Casting|CastToBP_ThirdPersonCharacter (.HitActor (Collision|BreakHitResult _outhit)))
    (Utilities|FlowControl|Delay 1.0)
    (if (Math|Boolean|ANDBoolean (not (Variables|Default|GetErgIsDead)) (not (Variables|Default|GetErgIsStunned)) (not (Variables|Default|GetPouncing)))
      (CallFunction|AttackingPlayer)
      (Variables|Default|SetPouncing true)
      (Animation|Montage|PlayMontage (Variables|Character|GetMesh) "/Game/Assets/Enemies/ErgCrawler/Animations/erg-Stun_Walk_Pounce-Anims_Anim_Crab_rig_ergPounce_Montage.erg-Stun_Walk_Pounce-Anims_Anim_Crab_rig_ergPounce_Montage"
        (:OnCompleted
          _)
        (:OnInterrupted
          _))
      (Variables|Default|SetPouncing false))))

(event Custom|ErgDeath
  ;[0.188 0.1351 0.1351] Erg is Dead
  (if (not (Variables|Default|GetErgIsDead))
    (bind _output_get (Variables|Default|SetErgIsDead true))
    (Variables|Default|SetErgIsDead _output_get) ; Blackboard Value!
    (Collision|SetCollisionEnabled (Variables|Character|GetMesh) "QueryAndPhysics") ; These three sequential steps are used to ragdoll the player mesh when HealthOfCharacter hits 0.
    (Physics|SetSimulatePhysics (Variables|Character|GetMesh) true)
    (Class|SkeletalMeshComponent|SetPhysicsBlendWeight (Variables|Character|GetMesh) 1.0)
    (Utilities|FlowControl|Delay 1.0)
    (Actor|DestroyActor)))

(event Custom|LeadElectricStun
  (bind _self self)
  (bind _returnvalue (AI|GetAIController _self))
  ;[0.9098 1 0.2078] When Erg Crawlers are Stunned, they freeze in place, become vulnerable and lose sight of player until healthy again!
  (AI|Navigation|StopMovement _returnvalue)
  (Development|PrintString "Enemy Stun Successful!" true true "(R=0.660055,G=1.000000,B=0.140704,A=1.000000)" 3.0)
  (bind _output_get (Variables|Default|SetErgIsStunned true))
  (AI|Components|Blackboard|SetValueasBool (AI|GetBlackboard _returnvalue) (Utilities|Name|MakeLiteralName "IsEnemyStunned") _output_get)
  (Utilities|FlowControl|Delay 2.0)
  (CallFunction|LeadElectricStunEnd))

(event Custom|LeadElectricStunEnd
  (bind _self self)
  (bind _returnvalue (AI|GetAIController _self))
  (bind _returnvalue_2 (AI|GetBlackboard _returnvalue))
  ;[0.2031 0.1407 0.05699] Trigger Once Stun Duration Finishes!
  (Development|PrintString "Enemy Stun Concluded!" true true "(R=0.660055,G=1.000000,B=0.140704,A=1.000000)" 3.0)
  (bind _output_get (Variables|Default|SetErgIsStunned false))
  (AI|Components|Blackboard|SetValueasBool _returnvalue_2 (Utilities|Name|MakeLiteralName "IsEnemyStunned") _output_get)
  (bind _output_get_2 (Variables|Default|SetAggro true))
  (AI|Components|Blackboard|SetValueasBool _returnvalue_2 (Utilities|Name|MakeLiteralName "IsEnemyAggro") _output_get_2)
  (AI|Components|Blackboard|SetValueasBool _returnvalue_2 (Utilities|Name|MakeLiteralName "PlayerDetected") false))

(event EventBeginPlay)

(event Collision|EventActorBeginOverlap
  (params (OtherActor :type Actor%20Object%20Reference)))

(event EventTick
  (params (DeltaSeconds :type Float%20%28single-precision%29)))

(event EventStruckbyPlayer
  (params (Player :type BP%20Third%20Person%20Character%20Object%20Reference))
  ;[1 0.4844 0.7588] Refer to BP_ThirdPersonCharacter's Hit Detect Function!
  (CallFunction|HitReact))

(event EventStunnedbyPlayer
  (params (Player :type BP%20Third%20Person%20Character%20Object%20Reference))
  ;[0.902 0.8824 0.4941] Sound Wave puts Erg in Stun State!
  (CallFunction|LeadElectricStun))

(event EventAttackingPlayer
  (params (Player :type BP%20Third%20Person%20Character%20Object%20Reference))
  (bind _returnvalue (Transformation|GetActorLocation))
  ;[0.6979 0.09381 0.1216] Sphere Trace for Pounce - TO REFINE WHEN ANIMATIONS ARE ADDED!
  ;;[0.202 1 0.5216] Attacking Message is Received - Attack Info!
  (bind _outhit (Collision|SphereTraceForObjects _returnvalue _returnvalue 1e+02 (Utilities|Array|MakeArray "ObjectTypeQuery3") false 0 "ForDuration")) ; Hit Sphere for Pounce
  (bind _asbp_third_person_character (Utilities|Casting|CastToBP_ThirdPersonCharacter (.HitActor (Collision|BreakHitResult _outhit))))
  (Default|HitReact _asbp_third_person_character))

(fn ConstructionScript)