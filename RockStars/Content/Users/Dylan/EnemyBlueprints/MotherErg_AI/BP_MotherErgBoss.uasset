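; Mother Erg boss enemy: a three-phase fight opened by a reveal montage and dialogue, ending in achievements and a cutscene.
; Blackboard-driven AI runs random left/right claw swipes and eye slams, toggling claw and eye hurtboxes so eyes become vulnerable during slams and stuns.
; Damage clamps at each phase's health threshold; after an eye slam or stun, she throws a tantrum and timeline-rotates toward the next platform.
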(event OnComponentBeginOverlap(WinkerSideClaw)
  (params (OverlappedComponent :type Primitive%20Component%20Object%20Reference) (OtherActor :type Actor%20Object%20Reference) (OtherComp :type Primitive%20Component%20Object%20Reference) (OtherBodyIndex :type Integer) (bFromSweep :type Boolean) (SweepResult :type Hit%20Result%20Structure%20%28by%20ref%29))
  ;[0.2039 1 0.5216] Attacking Message is Received - Attack Info for EYES!
  (if (and (Utilities|DoesObjectImplementInterface OtherActor "/Game/LevelStuff/ThirdPerson/Blueprints/Weapons/BPI_CombatInterface.BPI_CombatInterface_C") (Variables|Default|GetClawsCanHurtPawn))
    (Class|BPICombatInterface|StruckbyPlayer(Message) OtherActor 0 25.0)))

(event OnComponentBeginOverlap(PeeperSideClaw)
  (params (OverlappedComponent :type Primitive%20Component%20Object%20Reference) (OtherActor :type Actor%20Object%20Reference) (OtherComp :type Primitive%20Component%20Object%20Reference) (OtherBodyIndex :type Integer) (bFromSweep :type Boolean) (SweepResult :type Hit%20Result%20Structure%20%28by%20ref%29))
  ;[0.2039 1 0.5216] Attacking Message is Received - Attack Info for EYES!
  (if (and (Utilities|DoesObjectImplementInterface OtherActor "/Game/LevelStuff/ThirdPerson/Blueprints/Weapons/BPI_CombatInterface.BPI_CombatInterface_C") (Variables|Default|GetClawsCanHurtPawn))
    (Class|BPICombatInterface|StruckbyPlayer(Message) OtherActor 0 25.0)))

(event OnComponentBeginOverlap(Peeper)
  (params (OverlappedComponent :type Primitive%20Component%20Object%20Reference) (OtherActor :type Actor%20Object%20Reference) (OtherComp :type Primitive%20Component%20Object%20Reference) (OtherBodyIndex :type Integer) (bFromSweep :type Boolean) (SweepResult :type Hit%20Result%20Structure%20%28by%20ref%29))
  ;[0.2039 1 0.5216] Attacking Message is Received - Attack Info for EYES!
  (if (and (Utilities|DoesObjectImplementInterface OtherActor "/Game/LevelStuff/ThirdPerson/Blueprints/Weapons/BPI_CombatInterface.BPI_CombatInterface_C") (Utilities|Enum|Equal(Enum) (Collision|GetCollisionObjectType (Variables|Default|GetPeeper)) "ECC_Vehicle"))
    (Class|BPICombatInterface|StruckbyPlayer(Message) OtherActor 0 25.0)))

(event OnComponentBeginOverlap(Winker)
  (params (OverlappedComponent :type Primitive%20Component%20Object%20Reference) (OtherActor :type Actor%20Object%20Reference) (OtherComp :type Primitive%20Component%20Object%20Reference) (OtherBodyIndex :type Integer) (bFromSweep :type Boolean) (SweepResult :type Hit%20Result%20Structure%20%28by%20ref%29))
  ;[0.2039 1 0.5216] Attacking Message is Received - Attack Info for EYES!
  (if (and (Utilities|DoesObjectImplementInterface OtherActor "/Game/LevelStuff/ThirdPerson/Blueprints/Weapons/BPI_CombatInterface.BPI_CombatInterface_C") (Utilities|Enum|Equal(Enum) (Collision|GetCollisionObjectType (Variables|Default|GetPeeper)) "ECC_Vehicle"))
    (Class|BPICombatInterface|StruckbyPlayer(Message) OtherActor 0 25.0)))

(event Custom|ToggleEyeHurtboxes
  (params (Enabled :type Boolean))
  (bind _winker (Variables|Default|GetWinker))
  ;[0.3542 0.03136 0.04792] During/after attacking, Mother Erg's eyes become vulnerable/invulnerable to damage!
  (if Enabled
    (Default|CallOnEyeHitBoxActive)
    (Collision|SetCollisionObjectType _winker "ECC_GameTraceChannel1")
    (else
      (Default|CallOnEyeHitBoxDeActive)
      (Collision|SetCollisionObjectType _winker "ECC_Vehicle"))))

(event Custom|AddToRespawnable
  ;[0 0.09759 0.5841] Adds to Respawnable Struct Array so that Erg Crawler respawns on player death
  (bind _asbp_third_person_game_mode (Utilities|Casting|CastToBP_ThirdPersonGameMode (Game|GetGameMode)))
  (Utilities|Array|AddUnique (Variables|/Game/LevelStuff/ThirdPerson/Blueprints/Movement/BP_ThirdPersonGameMode.BP_ThirdPersonGameMode_C|GetRespawnableActors _asbp_third_person_game_mode) (Utilities|Struct|MakeStruct_RespawnableActors "BP_MotherErgBoss_C" self (Variables|Default|GetInitialTransform))))

(event Custom|ToggleClawHurtboxes
  (params (Enabled :type Boolean))
  (bind _winkersideclaw (Variables|Default|GetWinkerSideClaw))
  ;[0.1302 0.0217 0.0217] As Mother Erg turns, Claw Hitboxes are turned off to prevent cheap shots!
  (if Enabled
    (Collision|SetCollisionResponsetoChannel _winkersideclaw "ECC_Pawn" "ECR_Overlap")
    (Variables|Default|SetClawsCanHurtPawn true)
    (else
      (if (Variables|Default|GetActiveTantrum)
        (Collision|SetCollisionResponsetoChannel _winkersideclaw "ECC_Pawn" "ECR_Ignore")
        (else
          (Collision|SetCollisionResponsetoChannel (Variables|Default|GetPeeperSideClaw) "ECC_Pawn" "ECR_Block")))
      (Variables|Default|SetClawsCanHurtPawn false))))

(event Custom|CastingTestForBT
  ;[0.698 0.09412 0.1216] RANDOM CLAW SWIPE MONTAGES!
  (Default|CallOnBossAttack)
  (bind _attackisvalid (CallFunction|AttackValidityCheck))
  (if _attackisvalid
    (Variables|Default|SetAttacking true)
    (Development|PrintString "CLAW SWIPE DIALOGUE" true true "(R=0.129164,G=0.226884,B=1.000000,A=1.000000)")
    (CallFunction|ActionDialogue 0 0 (Utilities|Array|MakeArray 16 18 20 22 24)) ; claw swipe
    (Animation|Montage|PlayMontage (Variables|Character|GetMesh) (select (Variables|Default|GetSwingLeftClaw) "/Game/Assets/Enemies/MotherErg/Animations/ANM_MotherErg-ClawL_Montage.ANM_MotherErg-ClawL_Montage" "/Game/Assets/Enemies/MotherErg/Animations/ANM_MotherErg-ClawR_Montage.ANM_MotherErg-ClawR_Montage") (Utilities|Select :Index (Variables|BossHP|GetPhaseIndex) :Option%200 0.75 :Option%201 1.0 :Option%202 1.25)
      (:then
        (CallFunction|ToggleClawHurtboxes true))
      (:OnCompleted
        (Default|CallOnBossAttackEnd :!label _label)
        (Utilities|FlowControl|Delay (Variables|Default|GetAttackCooldown))
        (Variables|Default|SetAttacking false))
      (:OnInterrupted
        (goto _label)))))

(event Custom|BossPhaseTransition
  (bind _phaseindex (Variables|BossHP|GetPhaseIndex))
  ;[0.188 0.1351 0.1351] Enemy is Dead
  ;;[0.1049 0.1458 0.07856] Mother Erg transitions to a new phase if her health is equal to one of the phase shift quotas.
  (if (== (Variables|Default|GetHealthOfCharacter) (Utilities|Select :Index _phaseindex :Option%200 3.2e+02 :Option%201 1.6e+02 :Option%202 0.0))
    ;;;[0.0549 0.09412 0.03922] See below!
    (CallFunction|BeginTantrum)
    (Utilities|FlowControl|Delay 0.5)
    (switch int _phaseindex
      (:0
        (CallFunction|ActionDialogue 0 0 (Utilities|Array|MakeArray 32)))
      (:1
        (CallFunction|ActionDialogue 0 0 (Utilities|Array|MakeArray 34))))))

(event Custom|AttackLeftOrRight
  (bind _returnvalue (Math|Random|RandomIntegerinRange 0 1))
  (bind _self self)
  (bind _returnvalue_2 (AI|GetAIController _self))
  (bind _returnvalue_3 (== _returnvalue 0))
  (bind _returnvalue_4 (AI|GetBlackboard _returnvalue_2))
  (bind _returnvalue_5 (select _returnvalue_3 false true))
  ;[0.372 1 0.3197] Health Bar should be visible when aggro!
  (if (Utilities|IsValid _returnvalue_4)
    (AI|Components|Blackboard|SetValueasBool _returnvalue_4 (Utilities|Name|MakeLiteralName "SwingLeftClaw") _returnvalue_5)
    (bind _output_get (Variables|Default|SetSwingLeftClaw _returnvalue_5))))

(event Custom|Action%20Dialogue
  (params (Min :type Integer) (Max :type Integer) (Main%20Dialogue%20Indexes :type Array%20of%20Integers))
  (if (== (Math|Random|RandomIntegerinRange Min Max) 0)
    (Default|CustomEnterDialogue (Variables|Default|GetBPC_Dialogue) (.OutItem (Utilities|Array|Random Main%20Dialogue%20Indexes)) "NewEnumerator1" false)))

(event Custom|MotherErgRevealAnim
  (params (Unplayed :type Boolean))
  (bind _bpc_dialogue (Variables|Default|GetBPC_Dialogue))
  ;[0.7865 1 0.6729] Reveal Animation Controller!
  (if Unplayed
    (Animation|Montage|PlayMontage (Variables|Character|GetMesh) "/Game/Assets/Enemies/MotherErg/Animations/ANM_MotherErg-Reveal.ANM_MotherErg-Reveal"
      (:then
        (Class|BPIDialogue|BPITalk(Message) (Components|SkeletalMesh|GetAnimInstance (Variables|Character|GetMesh))))
      (:OnBlendOut
        ;;[0.9062 0.057 0.01888] enter dialogue
        (Variables|/Game/Users/Stanley/BPC_Dialogue.BPC_Dialogue_C|SetcanEnterBossDialogue _bpc_dialogue true)
        (Default|EnterDialogue _bpc_dialogue 0 (Game|GetPlayerCharacter 0) 0 0 false)))))

(event Custom|BeginTantrum
  ;[0.0549 0.09412 0.03922] Mother Erg has a justified crashout and destroys the platform in front of her!
  (if (not (Variables|Default|GetIsDead))
    (Variables|Default|SetActiveTantrum true)
    (Animation|Montage|PlayMontage (Variables|Character|GetMesh) "/Game/Assets/Enemies/MotherErg/Animations/ANM_MotherErg-Tantrum.ANM_MotherErg-Tantrum"
      (:then
        (CallFunction|ToggleClawHurtboxes false))
      (:OnCompleted
        (Variables|Default|SetActiveTantrum false :!label _label)
        (Variables|Default|SetIsTurning true)
        (CallFunction|SearchConditions))
      (:OnInterrupted
        (goto _label)))))

(event Custom|StunSequenceEnd
  (bind _healthofcharacter (Variables|Default|GetHealthOfCharacter))
  (bind _precyclehealth (Variables|BossHP|GetPreCycleHealth))
  (bind _returnvalue (< _healthofcharacter _precyclehealth))
  ;[0.6302 0 0.02865] EYE SLAM MONTAGES!
  (Animation|Montage|PlayMontage (Variables|Character|GetMesh) (select _returnvalue "/Game/Assets/Enemies/MotherErg/Animations/ANM_MotherErg-Hurt.ANM_MotherErg-Hurt" "/Game/Assets/Enemies/MotherErg/Animations/ANM_MotherErg-EyeSlam_pt3_Montage.ANM_MotherErg-EyeSlam_pt3_Montage")
    (:then
      (if _returnvalue
        (CallFunction|ActionDialogue 0 0 (Utilities|Array|MakeArray 28)) ; damage
      ))
    (:OnCompleted
      (Variables|Default|SetAttacking false)
      (CallFunction|ToggleClawHurtboxes true)
      (CallFunction|ToggleEyeHurtboxes false)
      ;;[0.1049 0.1458 0.07856] See below!
      (CallFunction|BossPhaseTransition))))

(event Custom|ReconfigurePSQ
  ;[1 0.4706 0.08235] After rotation handling is finished, turn off the Is Turning bool and reconfigure the next Phase Shift Quota based on Phase Index!
  (CallFunction|ToggleClawHurtboxes false)
  (Variables|Default|SetIsTurning false)
  (AI|Components|Blackboard|SetValueasFloat (AI|GetBlackboard (AI|GetAIController self)) (Utilities|Name|MakeLiteralName "PhaseShiftQuota") (Utilities|Select :Index (Variables|BossHP|GetPhaseIndex) :Option%200 1.6e+02 :Option%201 0.0))
  (bind _output_get (Variables|BossHP|SetPhaseIndex (+ (Variables|BossHP|GetPhaseIndex) 1)))
  (Class|BlackboardComponent|SetValueasInt (AI|GetBlackboard (AI|GetAIController self)) (Utilities|Name|MakeLiteralName "PhaseIndex") _output_get))

(event EventSetEnemyPursueMode
  (params (3PC :type Pawn%20Object%20Reference))
  ;[1 0.2345 0.1747] Player is Detected - Aggro!
  (Variables|Default|Set3PC 3PC)
  (CallFunction|MotherErgRevealAnim (not (Variables|Default|GetAggro)))
  (Utilities|FlowControl|DoOnce false
    (:Completed
      ;;[0 0.09804 0.5843] Respawnable!
      (CallFunction|AddtoRespawnable))))

(event EventUpdateHealthBar
  (params (CurrentHealth :type Float%20%28double-precision%29))
  (bind _maxhealthofcharacter (Variables|Default|GetMaxHealthOfCharacter))
  (bind _bosshealthbar (Variables|BossHP|GetBossHealthBar))
  (bind _returnvalue (/ CurrentHealth _maxhealthofcharacter))
  ;[1 0.4375 0.4375] When Mother Erg takes damage, update the health bar's fill!
  (Progress|SetPercent (Variables|/Game/Assets/Enemies/EnemyUI/WBP_BossHealthIndicator.WBP_BossHealthIndicator_C|GetHealthBar _bosshealthbar) _returnvalue)
  (Default|UpdateRecentlyLostBar self 0 _bosshealthbar _returnvalue))

(event EventEnemyDeath
  (bind _returnvalue (Game|GetPlayerController 0))
  ;[0.188 0.1351 0.1351] Enemy is Dead
  (if (not (Variables|Default|GetIsDead))
    (Variables|Default|SetIsDead true)
    (|SteamAchievements)
    (Animation|Montage|PlayMontage (Variables|Character|GetMesh) "/Game/Assets/Enemies/MotherErg/Animations/ANM_MotherErg-DeathInFight_Montage.ANM_MotherErg-DeathInFight_Montage"
      (:then
        (Collision|SetCollisionResponsetoAllChannels (Variables|Default|GetPeeper) "ECR_Ignore"))
      (:OnBlendOut
        ;;[0 0 0] TRANSITION TO END SCREEN!
        (Game|SetGamePaused true)
        (bind _asbp_player_controller (Utilities|Casting|CastToBP_PlayerController _returnvalue))
        (Default|ChangeIMC _asbp_player_controller "/Game/LevelStuff/ThirdPerson/Input/IMC_Default.IMC_Default" "/Game/LevelStuff/ThirdPerson/Input/IMC_UI.IMC_UI")
        (bind _returnvalue_2 (UserInterface|CreateWidget "/Game/Users/Stanley/UW_OpeningCutscene.UW_OpeningCutscene_C" _returnvalue "/Game/Movies/Intro_MediaPlayer.Intro_MediaPlayer" "NewEnumerator1"))
        (bind _output_get (Variables|Default|SetCutsceneRef _returnvalue_2))
        (UserInterface|Viewport|AddtoViewport _output_get 0)))))

(event EventBossAttackingPlayer
  ;[0.698 0.09412 0.1216] RANDOM CLAW SWIPE MONTAGES!
  (Default|CallOnBossAttack)
  (bind _attackisvalid (CallFunction|AttackValidityCheck))
  (if _attackisvalid
    (Variables|Default|SetAttacking true)
    (Development|PrintString "CLAW SWIPE DIALOGUE" true true "(R=0.129164,G=0.226884,B=1.000000,A=1.000000)")
    (CallFunction|ActionDialogue 0 0 (Utilities|Array|MakeArray 16 18 20 22 24)) ; claw swipe
    (Animation|Montage|PlayMontage (Variables|Character|GetMesh) (select (Variables|Default|GetSwingLeftClaw) "/Game/Assets/Enemies/MotherErg/Animations/ANM_MotherErg-ClawL_Montage.ANM_MotherErg-ClawL_Montage" "/Game/Assets/Enemies/MotherErg/Animations/ANM_MotherErg-ClawR_Montage.ANM_MotherErg-ClawR_Montage") (Utilities|Select :Index (Variables|BossHP|GetPhaseIndex) :Option%200 0.75 :Option%201 1.0 :Option%202 1.25)
      (:then
        (CallFunction|ToggleClawHurtboxes true))
      (:OnCompleted
        (Default|CallOnBossAttackEnd :!label _label)
        (Utilities|FlowControl|Delay (Variables|Default|GetAttackCooldown))
        (Variables|Default|SetAttacking false))
      (:OnInterrupted
        (goto _label)))))

(event EventEnemyAttack
  (bind _mesh (Variables|Character|GetMesh))
  ;[0.6302 0 0.02865] EYE SLAM MONTAGES!
  (Default|CallOnEyeAttack)
  (Variables|BossHP|SetPreCycleHealth (Variables|Default|GetHealthOfCharacter))
  (bind _attackisvalid (CallFunction|AttackValidityCheck))
  (if _attackisvalid
    (Variables|Default|SetAttacking true)
    (CallFunction|ActionDialogue 0 0 (Utilities|Array|MakeArray 26)) ; eye slam
    (Animation|Montage|PlayMontage _mesh "/Game/Assets/Enemies/MotherErg/Animations/ANM_MotherErg-EyeSlam_pt1_Montage.ANM_MotherErg-EyeSlam_pt1_Montage"
      (:then
        (CallFunction|ToggleClawHurtboxes false))
      (:OnBlendOut
        (Animation|Montage|PlayMontage _mesh "/Game/Assets/Enemies/MotherErg/Animations/ANM_MotherErg-EyeSlam_pt2_Montage.ANM_MotherErg-EyeSlam_pt2_Montage" 0.5
          (:then
            (CallFunction|ToggleEyeHurtboxes true))
          (:OnCompleted
            (Animation|Montage|PlayMontage _mesh (select (< (Variables|Default|GetHealthOfCharacter) (Variables|BossHP|GetPreCycleHealth)) "/Game/Assets/Enemies/MotherErg/Animations/ANM_MotherErg-Hurt.ANM_MotherErg-Hurt" "/Game/Assets/Enemies/MotherErg/Animations/ANM_MotherErg-EyeSlam_pt3_Montage.ANM_MotherErg-EyeSlam_pt3_Montage")
              (:then
                (if (< (Variables|Default|GetHealthOfCharacter) (Variables|BossHP|GetPreCycleHealth))
                  (CallFunction|ActionDialogue 0 0 (Utilities|Array|MakeArray 28)) ; damage
                ))
              (:OnCompleted
                (Variables|Default|SetAttacking false)
                (CallFunction|ToggleClawHurtboxes true)
                (CallFunction|ToggleEyeHurtboxes false)
                ;;[0.1049 0.1458 0.07856] See below!
                (CallFunction|BossPhaseTransition)))))))))

(event EventStunnedbyPlayer
  (params (Player :type BP%20Third%20Person%20Character%20Object%20Reference) (ProjectileVelocity :type Vector :default "0, 0, 0") (ProjectileLocation :type Vector :default "0, 0, 0"))
  ;[0.9098 1 0.2078] When stunned, play the new stun montage!
  (if (not (Variables|Default|GetIsStunned))
    (bind _output_get (Variables|Default|SetIsStunned true))
    (AI|Components|Blackboard|SetValueasBool (AI|GetBlackboard (AI|GetAIController self)) (Utilities|Name|MakeLiteralName "IsEnemyStunned") _output_get)
    (Animation|Montage|PlayMontage (Variables|Character|GetMesh) "/Game/Assets/Enemies/MotherErg/Animations/ANM_MotherErg-StunBegin_PH.ANM_MotherErg-StunBegin_PH"
      (:then
        (CallFunction|ToggleClawHurtboxes false)
        (CallFunction|ToggleEyeHurtboxes true))
      (:OnBlendOut
        (Animation|Montage|PlayMontage (Variables|Character|GetMesh) "/Game/Assets/Enemies/MotherErg/Animations/ANM_MotherErg-Stunned_PH.ANM_MotherErg-Stunned_PH"
          (:OnCompleted
            (CallFunction|StunSequenceEnd)
            (Utilities|FlowControl|Delay (Variables|Default|GetStunPause))
            (bind _output_get_2 (Variables|Default|SetIsStunned false))
            (AI|Components|Blackboard|SetValueasBool (AI|GetBlackboard (AI|GetAIController self)) (Utilities|Name|MakeLiteralName "IsEnemyStunned") _output_get_2)))))))

(event EventBPIStopTalking
  ;[0.3712 0.02315 0.008023] Gets called upon finishing main dialogue
  (if (Variables|/Game/Users/Stanley/BPC_Dialogue.BPC_Dialogue_C|GetfinishedMainDialogue? (Variables|Default|GetBPC_Dialogue))
    (bind _output_get (Variables|Default|SetAggro true))
    (AI|Components|Blackboard|SetValueasBool (AI|GetBlackboard (AI|GetAIController self)) (Utilities|Name|MakeLiteralName "PlayerDetected") _output_get)
    (CallFunction|DisplayHealthBar true)
    (CallFunction|ChangeCTD true)
    (CallFunction|PlayBGM "/Game/Users/Liam/BackgroundMusic/Audio/BossBattle_MED_Cue.BossBattle_MED_Cue")
    (Collision|SetCollisionEnabled (Variables|Default|GetBox) "NoCollision")))

(event EventStruckbyPlayer
  (params (Player :type BP%20Third%20Person%20Character%20Object%20Reference) (DamageOutput :type Float%20%28double-precision%29))
  ;[0.7725 0.06667 0.3529] Enemy Takes Damage - OVERRIDEN FOR BOSS BATTLE
  ;;[1 0.4863 0.7569] Refer to BP_ThirdPersonCharacter's Hit Detect Function!
  (|CallParentFunction Player DamageOutput))

(event EventHitReact
  (bind _phaseindex (Variables|BossHP|GetPhaseIndex))
  (bind _returnvalue (Utilities|Select :Index _phaseindex :Option%200 3.2e+02 :Option%201 1.6e+02 :Option%202 0.0))
  ;[0.7725 0.06667 0.3529] Enemy Takes Damage - OVERRIDEN FOR BOSS BATTLE
  (if (Math|Boolean|ANDBoolean (not (Variables|Default|GetIsDead)) (not (Variables|Default|GetTakingDamage)) (Variables|Default|GetCanTakeDamage))
    (if (Variables|Default|GetAggro)
      (Variables|Default|SetTakingDamage true)
      (bind _output_get (Variables|Default|SetHealthOfCharacter (- (Variables|Default|GetHealthOfCharacter) (stale EventStruckbyPlayer DamageOutput))))
      (CallFunction|UpdateHealthBar _output_get)
      (AI|Components|Blackboard|SetValueasFloat (AI|GetBlackboard (AI|GetAIController self)) (Utilities|Name|MakeLiteralName "HealthOfEnemy") _output_get)
      (if (<= _output_get _returnvalue)
        (bind _output_get_2 (Variables|Default|SetHealthOfCharacter _returnvalue))
        (CallFunction|UpdateHealthBar _output_get_2)
        (AI|Components|Blackboard|SetValueasFloat (AI|GetBlackboard (AI|GetAIController self)) (Utilities|Name|MakeLiteralName "HealthOfEnemy") _returnvalue)
        (if (== (Variables|BossHP|GetPhaseIndex) 2)
          (CallFunction|EnemyDeath)
          (Collision|SetCollisionResponsetoChannel (Variables|Default|GetCapsuleComponent) "ECC_Pawn" "ECR_Ignore")
          (else
            (Utilities|FlowControl|RetriggerableDelay 0.25 :!label _label)
            (Variables|Default|SetTakingDamage false)
            (CallFunction|ResetDoOnce)))
        (else
          (goto _label)))
      (else
        (Variables|Default|SetAggro true)
        (CallFunction|SearchConditions)))))

(event EventUpdateRecentlyLostBar
  (params (HealthIndicatorRef :type WBP%20Enemy%20Health%20Indicator%20Object%20Reference) (BossIndicatorRef :type WBP%20Boss%20Health%20Indicator%20Object%20Reference) (NewPercent :type Float%20%28double-precision%29))
  ;[0.3278 0.2086 0.02029] After the health bar is updated, call this function. This function will wait for a set time, then decrease the recently lost part of the health bar over a short duration.
  (Utilities|FlowControl|Delay (Variables|Default|GetRecentlyLostUpdateDelay))
  (Variables|Default|SetStartingPercent (Variables|/Script/UMG.ProgressBar|GetPercent (Variables|/Game/Assets/Enemies/EnemyUI/WBP_BossHealthIndicator.WBP_BossHealthIndicator_C|GetRecentlyLostHealthBar BossIndicatorRef)))
  (bind _alpha (Timeline|Timeline PlayFromStart)
    (:Update
      (Progress|SetPercent (Variables|/Game/Assets/Enemies/EnemyUI/WBP_BossHealthIndicator.WBP_BossHealthIndicator_C|GetRecentlyLostHealthBar (Variables|BossHP|GetBossHealthBar)) (Math|Float|Lerp (Variables|Default|GetStartingPercent) NewPercent _alpha)))))

(event EventSetEnemyRoamMode
  ;[0 0 0] THE EVENT GRAVEYARD: ALL FUNCTIONS NOT INTENDED FOR USE ARE OVERRIDEN TO DO NOTHING HERE!
)

(event EventSetEnemyHideMode
  ;[0 0 0] THE EVENT GRAVEYARD: ALL FUNCTIONS NOT INTENDED FOR USE ARE OVERRIDEN TO DO NOTHING HERE!
)

(event EventBeginPlay
  (|CallParentFunction))

(event EventSearchConditions
  ;[1 0.6667 0.6745] After crashing out and once a player reaches a trigger box, this event makes Mother Erg rotate to the designated platform!
  (if (Variables|Default|GetIsTurning)
    (switch int (Variables|BossHP|GetPhaseIndex)
      (:0
        (Animation|Montage|PlayMontage (Variables|Character|GetMesh) "/Game/Assets/Enemies/MotherErg/Animations/ANM_MotherErg-TurnL.ANM_MotherErg-TurnL" 0.4
          (:then
            (bind _turntofacepsp (Timeline|TL_RotateToPeeperSidePlatform PlayFromStart)
              (:Update
                (Transformation|SetWorldRotation (Variables|Default|GetCapsuleComponent) (Math|Rotator|MakeRotator 0.0 0.0 _turntofacepsp) false false))
              (:Finished
                (CallFunction|ReconfigurePSQ))))))
      (:1
        (Animation|Montage|PlayMontage (Variables|Character|GetMesh) "/Game/Assets/Enemies/MotherErg/Animations/ANM_MotherErg-TurnL.ANM_MotherErg-TurnL" 0.4
          (:then
            (bind _turntofacewsp (Timeline|TL_RotateToWinkerSidePlatform PlayFromStart)
              (:Update
                (Transformation|SetWorldRotation (Variables|Default|GetCapsuleComponent) (Math|Rotator|MakeRotator 0.0 0.0 _turntofacewsp) false false))
              (:Finished
                (CallFunction|ReconfigurePSQ)))))))))

(event EventDisplayHealthBar
  (params (Should%20Display :type Boolean))
  ;[0.372 1 0.3197] Health Bar should be visible when aggro!
  (Utilities|Time|SetTimerbyEvent (delegate Custom|AttackLeftOrRight) 5.0 true)
  (bind _bosshealthbar (Variables|BossHP|GetBossHealthBar)
    (:then
      (UserInterface|Viewport|AddtoViewport _bosshealthbar 0)
      (Utilities|Array|AddUnique (Variables|/Game/LevelStuff/ThirdPerson/Blueprints/Movement/BP_ThirdPersonGameMode.BP_ThirdPersonGameMode_C|GetConstantGameplayUI (CallFunction|ValidGameMode)) _bosshealthbar))
    (:else)))

(event EventSetHealthBarName
  ;[0.016 0.2831 0.0319] Enemy's name is set inside Health Bar, and the health bars for eyes are given names as well!
  (bind _returnvalue (UserInterface|CreateWidget "/Game/Assets/Enemies/EnemyUI/WBP_BossHealthIndicator.WBP_BossHealthIndicator_C"))
  (Variables|/Game/Assets/Enemies/EnemyUI/WBP_BossHealthIndicator.WBP_BossHealthIndicator_C|SetNameOfEnemy _returnvalue (Variables|Default|GetNameOfEnemy))
  (bind _output_get (Variables|BossHP|SetBossHealthBar _returnvalue))
  (Utilities|Array|AddUnique (Variables|/Game/LevelStuff/ThirdPerson/Blueprints/Movement/BP_ThirdPersonGameMode.BP_ThirdPersonGameMode_C|GetConstantGameplayUI (CallFunction|ValidGameMode)) _output_get))

(fn ConstructionScript
  (|CallParentFunction))