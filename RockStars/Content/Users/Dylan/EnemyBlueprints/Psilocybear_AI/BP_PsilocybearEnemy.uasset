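; Psilocybear enemy that stays hidden until it detects a player at 70% or higher hallucination, then reveals and turns aggressive.
; Hide and pursue events drive Blackboard aggro keys, model swaps, collision channels and a DoOnce-gated smoke reveal.
; Attacks chain prep and swipe montages with VFX and cooldown, though the lunge and jaw sphere trace are unwired.
; Hits while aggro cause stun or death, and first aggro registers it for respawning.
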(event Custom|HideShortcut
  (bind _self self)
  (bind _returnvalue (AI|GetAIController _self))
  ;[0.415 0.2753 1] No Longer Aggro - Hide!
  (Variables|Default|SetAggro false)
  (CallFunction|ResetReveal)
  (AI|Components|Blackboard|SetValueasBool (AI|GetBlackboard _returnvalue) (Utilities|Name|MakeLiteralName "IsEnemyAggro") (Variables|Default|GetAggro))
  (AI|Navigation|StopMovement _returnvalue)
  (CallFunction|ModelSwap "/Game/Assets/VFX/ErgReveal/BP_ErgPoofVFX.BP_ErgPoofVFX_C")
  (CallFunction|ChangeCTD false)
  (Utilities|FlowControl|Sequence
    (:then_0
      (CallFunction|CollisionSwitchReset))
    (:then_1
      (CallFunction|CollisionSwitch false))))

(event Custom|AddToRespawnable
  ;[0 0.09759 0.5841] Adds to Respawnable Struct Array so that Erg Crawler respawns on player death
  (bind _asbp_third_person_game_mode (Utilities|Casting|CastToBP_ThirdPersonGameMode (Game|GetGameMode)))
  (Utilities|Array|AddUnique (Variables|/Game/LevelStuff/ThirdPerson/Blueprints/Movement/BP_ThirdPersonGameMode.BP_ThirdPersonGameMode_C|GetRespawnableActors _asbp_third_person_game_mode) (Utilities|Struct|MakeStruct_RespawnableActors "BP_PsilocybearEnemy_C" self (Variables|Default|GetInitialTransform))))

(event Custom|ResetReveal
  ;[1 0.702 0.8235] Psilocybear Reveal Animation Controller!
  (Utilities|FlowControl|DoOnce false) ; enters at Reset
)

(event Custom|CollisionSwitch
  (params (On :type Boolean))
  ;[0 0.2013 1] Psilocybear's collision turns ON/OFF when revealed/hiding!
  (if On
    (Utilities|FlowControl|DoOnce false
      (:Completed
        (Collision|SetCollisionObjectType (Variables|Character|GetMesh) "ECC_GameTraceChannel1")))
    (else
      (Collision|SetCollisionObjectType (Variables|Character|GetMesh) "ECC_Vehicle"))))

(event Custom|RevealAnim
  ;[1 0.702 0.8235] Psilocybear Reveal Animation Controller!
  (Utilities|FlowControl|DoOnce false
    (:Completed
      (Niagara|SpawnSystemAttached "/Game/Assets/VFX/Smoke/NS_BearSmoke.NS_BearSmoke" (Variables|Default|GetSmokeReveal) "None" "0, 0, 0" "0, 0, 0" "KeepRelativeOffset" true)
      (Pawn|Components|CharacterMovement|DisableMovement (Variables|Character|GetCharacterMovement))
      (Animation|Montage|PlayMontage (Variables|Character|GetMesh) "/Game/Assets/Enemies/Bear/Animations/ANM_Psilocybear_Reveal.ANM_Psilocybear_Reveal"
        (:OnCompleted
          _)
        (:OnInterrupted
          _))
      (Pawn|Components|CharacterMovement|SetMovementMode (Variables|Character|GetCharacterMovement) "MOVE_Walking" 0))))

(event Custom|CollisionSwitchReset
  ;[0 0.2013 1] Psilocybear's collision turns ON/OFF when revealed/hiding!
  (Utilities|FlowControl|DoOnce false) ; enters at Reset
)

(event EventSetEnemyPursueMode
  (params (3PC :type Pawn%20Object%20Reference))
  (bind _self self)
  (bind _returnvalue (AI|GetAIController _self))
  (bind _returnvalue_2 (AI|GetBlackboard _returnvalue))
  ;[1 0.2345 0.1747] Player is Detected (and tripping) - Aggro!
  (bind _asbp_third_person_character (Utilities|Casting|CastToBP_ThirdPersonCharacter 3PC))
  (if (>= (Variables|/Game/LevelStuff/ThirdPerson/Blueprints/Movement/BP_ThirdPersonCharacter.BP_ThirdPersonCharacter_C|GetHallucinationPercentage _asbp_third_person_character) 7e+01)
    (Variables|Default|SetAggro true)
    (AI|Components|Blackboard|SetValueasBool _returnvalue_2 (Utilities|Name|MakeLiteralName "PlayerDetected") true)
    (AI|Components|Blackboard|SetValueasBool _returnvalue_2 (Utilities|Name|MakeLiteralName "IsEnemyAggro") true)
    (CallFunction|ModelSwap "/Game/Assets/VFX/ErgReveal/BP_ErgPoofVFX.BP_ErgPoofVFX_C")
    (CallFunction|RevealAnim)
    (Utilities|FlowControl|Sequence
      (:then_0
        (CallFunction|SearchConditions))
      (:then_1
        (CallFunction|ChangeCTD true))
      (:then_2
        (CallFunction|CollisionSwitch true))
      (:then_3
        ;;[0 0.09804 0.5843] Calls Add to Respawnable once
        (Utilities|FlowControl|DoOnce false
          (:Completed
            (CallFunction|AddtoRespawnable)))))
    (else
      (CallFunction|HideShortcut))))

(event EventEnemyAttack
  (bind _charactermovement (Variables|Character|GetCharacterMovement))
  ;[0.698 0.09412 0.1216] Sphere Trace for Pounce - TO REFINE WHEN ANIMATIONS ARE ADDED!
  (bind _attackisvalid (CallFunction|AttackValidityCheck))
  (if _attackisvalid
    (Variables|Default|SetAttacking true)
    (Game|SpawnActorfromClass "/Game/Assets/VFX/ShroomboAngerSymbol/BP_ShroomboAngerVFX.BP_ShroomboAngerVFX_C" (Utilities|AngryVFXSpawn) "Undefined" "MultiplyWithRoot" 0 0)
    (CallFunction|EyeFireVFXVisibility true)
    (Pawn|Components|CharacterMovement|DisableMovement _charactermovement)
    (Animation|Montage|PlayMontage (Variables|Character|GetMesh) "/Game/Assets/Enemies/Bear/Animations/ANM_Psilocybear_Prep_Montage.ANM_Psilocybear_Prep_Montage"
      (:OnCompleted
        _)
      (:OnBlendOut
        _)
      (:OnInterrupted
        _))
    (Pawn|Components|CharacterMovement|SetMovementMode _charactermovement "MOVE_NavWalking" 0)
    (CallFunction|EyeFireVFXVisibility false)
    (CallFunction|AttackingPlayer)
    (Animation|Montage|PlayMontage (Variables|Character|GetMesh) "/Game/Assets/Enemies/Bear/Animations/ANM_Psilocybear_Attack_Montage.ANM_Psilocybear_Attack_Montage" 2.0
      (:OnCompleted
        _)
      (:OnInterrupted
        _))
    (Audio|Components|Audio|Play (Variables|Default|GetBaseNoise) 0.0)
    (Utilities|FlowControl|Delay (Variables|Default|GetAttackCooldown))
    (Variables|Default|SetAttacking false)))

(event EventLeadElectricStun
  ;[0.7725 0.06667 0.3529] Enemy Takes Damage
  ;;[0.902 0.8824 0.4941] NOTHING!!!!!!!!!
)

(event EventStruckbyPlayer
  (params (Player :type BP%20Third%20Person%20Character%20Object%20Reference) (DamageOutput :type Float%20%28double-precision%29))
  ;[1 0.4844 0.7588] Refer to BP_ThirdPersonCharacter's Hit Detect Function!
  (CallFunction|PlayHitSound)
  (CallFunction|HitReact))

(event EventBeginPlay
  (|CallParentFunction))

(event EventAttackingPlayer
  (params (Player :type BP%20Third%20Person%20Character%20Object%20Reference))
  ;[0.698 0.09412 0.1216] Sphere Trace for Pounce - TO REFINE WHEN ANIMATIONS ARE ADDED!
  ;;[0.202 1 0.5216] Attacking Message is Received - Attack Info!
  (Utilities|FlowControl|DoOnce false) ; enters at Reset
)

(event EventHitReact
  ;[0.7725 0.06667 0.3529] Enemy Takes Damage
  (if (Math|Boolean|ANDBoolean (not (Variables|Default|GetIsDead)) (not (Variables|Default|GetTakingDamage)) (Variables|Default|GetAggro))
    (Variables|Default|SetTakingDamage true)
    (bind _output_get (Variables|Default|SetHealthOfCharacter (- (Variables|Default|GetHealthOfCharacter) (stale EventStruckbyPlayer DamageOutput))))
    (CallFunction|UpdateHealthBar _output_get)
    (if (<= (Variables|Default|GetHealthOfCharacter) 0.0)
      (CallFunction|EnemyDeath)
      (Collision|SetCollisionResponsetoChannel (Variables|Default|GetCapsuleComponent) "ECC_Pawn" "ECR_Ignore")
      (else
        ;;[0.05185 0.1405 1] HIT STUN!
        (Animation|Montage|PlayMontage (Variables|Character|GetMesh) (Variables|Default|GetHit%20Stun%20Montage)
          (:then
            (Utilities|FlowControl|RetriggerableDelay 0.25)
            (Variables|Default|SetTakingDamage false)))))))

(event EventSetEnemyHideMode
  (bind _self self)
  (bind _returnvalue (AI|GetAIController _self))
  ;[0.415 0.2753 1] No Longer Aggro - Hide!
  (Utilities|FlowControl|RetriggerableDelay 3.0)
  (Variables|Default|SetAggro false)
  (CallFunction|ResetReveal)
  (AI|Components|Blackboard|SetValueasBool (AI|GetBlackboard _returnvalue) (Utilities|Name|MakeLiteralName "IsEnemyAggro") (Variables|Default|GetAggro))
  (AI|Navigation|StopMovement _returnvalue)
  (CallFunction|ModelSwap "/Game/Assets/VFX/ErgReveal/BP_ErgPoofVFX.BP_ErgPoofVFX_C")
  (CallFunction|ChangeCTD false)
  (Utilities|FlowControl|Sequence
    (:then_0
      (CallFunction|CollisionSwitchReset))
    (:then_1
      (CallFunction|CollisionSwitch false))))

(fn ConstructionScript
  (|CallParentFunction))

(fn EyeFireVFXVisibility
  (params (Visible :type Boolean))
  (for _array_element (Utilities|Array|MakeArray (Variables|Default|GetLeftEyeFire) (Variables|Default|GetRightEyeFire) (Variables|Default|GetMiddleEyeFire))
    (Rendering|SetVisibility _array_element Visible false)))

(fn PlayClawSwipeVFX
  (switch int (Math|Random|RandomInteger 2)
    (:0
      (LocalVariables|SetFlipbook "/Game/Assets/VFX/BearAttack/ClawSwipeLEFT.ClawSwipeLEFT"))
    (:1
      (LocalVariables|SetFlipbook "/Game/Assets/VFX/BearAttack/ClawSwipeRIGHT.ClawSwipeRIGHT"))
    (:2
      (LocalVariables|SetFlipbook "/Game/Assets/VFX/BearAttack/ClawSwipeTOP.ClawSwipeTOP")))
  (Game|SpawnActorfromClass "/Game/Assets/VFX/BP_SpawnVFX.BP_SpawnVFX_C" (Transformation|GetActorTransform) "AlwaysSpawn" "MultiplyWithRoot" 0 (LocalVariables|GetFlipbook) (Math|Transform|MakeTransform "255.000000,0.000000,56.500000" "0.000000,90.000000,0.000000" "0.250000,0.250000,0.250000") true 0))