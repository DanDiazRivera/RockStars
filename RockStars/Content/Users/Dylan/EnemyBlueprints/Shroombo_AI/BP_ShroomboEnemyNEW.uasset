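; Shroombo enemy that switches between hidden and aggro modes and attacks the player by firing Sporb projectiles.
; Pursue and hide events set Blackboard aggro state, call model swaps, and gate the reveal montage, with hiding delayed by a retriggerable timer.
; Attacks spawn anger VFX before the montage, while pursuit interpolates the spawner arrow's pitch toward the player.
; First aggro registers it with the GameMode for respawning at its initial transform.
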(event Custom|SporbAttack
  ;[0.9263 1 0.7322] Fire a Sporb!
  (if (not (Variables|Default|GetIsDead))
    (Game|SpawnActorfromClass "/Game/Users/Dylan/ProjectileData/BP_ShroomboSporbProj.BP_ShroomboSporbProj_C" (Transformation|GetWorldTransform (Variables|Default|GetSporbSpawner)) "Undefined" "MultiplyWithRoot" 0 0)))

(event Custom|AddToRespawnable
  ;[0 0.09759 0.5841] Adds to Respawnable Struct Array so that Shroombo respawns on player death
  (bind _asbp_third_person_game_mode (Utilities|Casting|CastToBP_ThirdPersonGameMode (Game|GetGameMode)))
  (Utilities|Array|AddUnique (Variables|/Game/LevelStuff/ThirdPerson/Blueprints/Movement/BP_ThirdPersonGameMode.BP_ThirdPersonGameMode_C|GetRespawnableActors _asbp_third_person_game_mode) (Utilities|Struct|MakeStruct_RespawnableActors "BP_ShroomboEnemyNEW_C" self (Variables|Default|GetInitialTransform))))

(event Custom|ResetReveal
  ;[1 0.702 0.8235] Shroombo Reveal Animation Controller!
  (Utilities|FlowControl|DoOnce false) ; enters at Reset
)

(event Custom|RevealAnim
  ;[1 0.702 0.8235] Shroombo Reveal Animation Controller!
  (Utilities|FlowControl|DoOnce false
    (:Completed
      (Animation|Montage|PlayMontage (Variables|Character|GetMesh) "/Game/Assets/Enemies/Shroombo/Animations/ANM_shroombo_Reveal_Montage.ANM_shroombo_Reveal_Montage"))))

(event Custom|AdjustFiringPath
  (params (3PC :type BP%20Third%20Person%20Character%20Object%20Reference))
  (bind _returnvalue (Utilities|Time|GetWorldDeltaSeconds))
  (bind _returnvalue_2 (Transformation|GetActorLocation 3PC))
  (bind _returnvalue_3 (Transformation|GetActorLocation))
  (bind _sporbspawner (Variables|Default|GetSporbSpawner))
  (bind _returnvalue_4 (Transformation|GetWorldRotation _sporbspawner))
  (bind _returnvalue_5 (Math|Rotator|FindLookatRotation _returnvalue_3 _returnvalue_2))
  (bind _returnvalue_6 (Math|Interpolation|RInterpTo (Math|Rotator|MakeRotator 0.0 (.pitch _returnvalue_4) 0.0) (Math|Rotator|MakeRotator 0.0 (.pitch _returnvalue_5) 0.0) _returnvalue 1e+01))
  ;[0.1406 0 0.002633] Depending on the Player's vertical position, the Sporb Spawner arrow will rotate to face it while in Aggro Mode!
  (Transformation|SetWorldRotation _sporbspawner (Math|Rotator|MakeRotator (.roll _returnvalue_4) (.pitch _returnvalue_6) (.yaw _returnvalue_4)) false false)
  (Development|PrintString (Utilities|String|ToString(Float) (.pitch _returnvalue_6))))

(event EventSetEnemyPursueMode
  (params (3PC :type Pawn%20Object%20Reference))
  (bind _self self)
  (bind _returnvalue (AI|GetAIController _self))
  (bind _returnvalue_2 (AI|GetBlackboard _returnvalue))
  ;[1 0.2345 0.1747] Player is Detected - Aggro!
  (Variables|Default|SetAggro true)
  (bind _asbp_third_person_character (Utilities|Casting|CastToBP_ThirdPersonCharacter 3PC))
  (CallFunction|AdjustFiringPath _asbp_third_person_character)
  (AI|Components|Blackboard|SetValueasBool _returnvalue_2 (Utilities|Name|MakeLiteralName "PlayerDetected") true)
  (AI|Components|Blackboard|SetValueasBool _returnvalue_2 (Utilities|Name|MakeLiteralName "IsEnemyAggro") true)
  (CallFunction|ModelSwap "/Game/Assets/VFX/ShroomboNotice/BP_ShroomboNoticeVFX.BP_ShroomboNoticeVFX_C")
  (CallFunction|RevealAnim)
  (Utilities|FlowControl|Sequence
    (:then_0
      (CallFunction|SearchConditions))
    (:then_1
      (CallFunction|ChangeCTD true))
    (:then_2
      ;;[0 0.09804 0.5843] Calls Add to Respawnable once
      (Utilities|FlowControl|DoOnce false
        (:Completed
          (CallFunction|AddtoRespawnable))))))

(event EventSetEnemyHideMode
  (bind _self self)
  (bind _returnvalue (AI|GetAIController _self))
  ;[0.415 0.2753 1] No Longer Aggro - Hide!
  (Utilities|FlowControl|RetriggerableDelay 3.0)
  (Variables|Default|SetAggro false)
  (AI|Components|Blackboard|SetValueasBool (AI|GetBlackboard _returnvalue) (Utilities|Name|MakeLiteralName "IsEnemyAggro") (Variables|Default|GetAggro))
  (AI|Navigation|StopMovement _returnvalue)
  (CallFunction|ModelSwap "/Game/Assets/VFX/ShroomboNotice/BP_ShroomboNoticeVFX.BP_ShroomboNoticeVFX_C")
  (CallFunction|ResetReveal))

(event EventAttackingPlayer
  (params (Player :type BP%20Third%20Person%20Character%20Object%20Reference))
  ;[0.698 0.09412 0.1216] Enemy Attacks and Faces Player!
  (Game|SpawnActorfromClass "/Game/Assets/VFX/ShroomboAngerSymbol/BP_ShroomboAngerVFX.BP_ShroomboAngerVFX_C" (Utilities|AngryVFXSpawn) "Undefined" "MultiplyWithRoot" 0 0)
  (Utilities|FlowControl|Delay 0.6)
  (Animation|Montage|PlayMontage (Variables|Character|GetMesh) "/Game/Assets/Enemies/Shroombo/Animations/ANM_shroombo_Attack_Montage.ANM_shroombo_Attack_Montage"))

(event EventEnemyAttack
  ;[0.698 0.09412 0.1216] Enemy Attacks and Faces Player!
  (CallFunction|AttackingPlayer))

(fn ConstructionScript
  (|CallParentFunction)
  (Development|PrintString (Utilities|GetDisplayName self)))