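; Shroombo enemy Blueprint that toggles between aggro pursuit and hiding, and attacks with spore projectiles.
; Pursue and hide events set blackboard keys, call a model swap with a notice VFX, and play or re-arm a one-shot reveal montage.
; Attacks spawn anger VFX before the attack montage, while a separate event fires Sporbs if alive.
; First aggro registers it with the game mode for respawn as BP_ShroomboEnemyNEW.
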(event Custom|SporbAttack
  ;[0.9263 1 0.7322] Fire a Sporb!
  (if (not (Variables|Default|GetIsDead))
    (Game|SpawnActorfromClass "/Game/Users/Dylan/ProjectileData/BP_ShroomboSporbProj.BP_ShroomboSporbProj_C" (Transformation|GetWorldTransform (Variables|Default|GetSporbSpawner)) "Undefined" "MultiplyWithRoot" 0 0)))

(event Custom|AddToRespawnable
  ;[0 0.09759 0.5841] Adds to Respawnable Struct Array so that Shroombo respawns on player death
  (bind _asbp_third_person_game_mode (Utilities|Casting|CastToBP_ThirdPersonGameMode (Game|GetGameMode)))
  (Utilities|Array|AddUnique (Variables|/Game/LevelStuff/ThirdPerson/Blueprints/Movement/BP_ThirdPersonGameMode.BP_ThirdPersonGameMode_C|GetRespawnableActors _asbp_third_person_game_mode) (Utilities|Struct|MakeStruct_RespawnableActors "/Game/Users/Dylan/EnemyBlueprints/Shroombo_AI/BP_ShroomboEnemyNEW.BP_ShroomboEnemyNEW_C" self (Variables|Default|GetInitialTransform))))

(event Custom|ResetReveal
  ;[1 0.7017 0.8249] Shroombo Reveal Animation Controller!
  (Utilities|FlowControl|DoOnce false) ; enters at Reset
)

(event Custom|RevealAnim
  ;[1 0.7017 0.8249] Shroombo Reveal Animation Controller!
  (Utilities|FlowControl|DoOnce false
    (:Completed
      (Animation|Montage|PlayMontage (Variables|Character|GetMesh) "/Game/Assets/Enemies/Shroombo/Animations/ANM_shroombo_Reveal_Montage.ANM_shroombo_Reveal_Montage"))))

(event EventSetEnemyPursueMode
  (params (3PC :type Pawn%20Object%20Reference))
  (bind _self self)
  (bind _returnvalue (AI|GetAIController _self))
  (bind _returnvalue_2 (AI|GetBlackboard _returnvalue))
  ;[1 0.2345 0.1747] Player is Detected - Aggro!
  (Variables|Default|SetAggro true)
  (Utilities|Casting|CastToBP_ThirdPersonCharacter 3PC)
  (AI|Components|Blackboard|SetValueasBool _returnvalue_2 (Utilities|Name|MakeLiteralName "PlayerDetected") true)
  (AI|Components|Blackboard|SetValueasBool _returnvalue_2 (Utilities|Name|MakeLiteralName "IsEnemyAggro") true)
  (CallFunction|ModelSwap "/Game/Assets/VFX/ShroomboNotice/BP_ShroomboNoticeVFX.BP_ShroomboNoticeVFX_C")
  (CallFunction|SearchConditions)
  (CallFunction|RevealAnim)
  ;;[0 0.09804 0.5843] Calls Add to Respawnable once
  (Utilities|FlowControl|DoOnce false
    (:Completed
      (CallFunction|AddtoRespawnable))))

(event EventSetEnemyHideMode
  (bind _self self)
  (bind _returnvalue (AI|GetAIController _self))
  ;[0.415 0.2753 1] No Longer Aggro - Hide!
  (Utilities|FlowControl|RetriggerableDelay 3.0)
  (Variables|Default|SetAggro false)
  (AI|Components|Blackboard|SetValueasBool (AI|GetBlackboard _returnvalue) (Utilities|Name|MakeLiteralName "IsEnemyAggro") (Variables|Default|GetAggro))
  (AI|Navigation|StopMovement _returnvalue)
  (CallFunction|ModelSwap "/Game/Assets/VFX/ShroomboNotice/BP_ShroomboNoticeVFX.BP_ShroomboNoticeVFX_C")
  (CallFunction|ResetReveal))

(event EventAttackingPlayer
  (params (Player :type BP%20Third%20Person%20Character%20Object%20Reference))
  ;[0.698 0.09412 0.1216] Enemy Attacks and Faces Player!
  (Game|SpawnActorfromClass "/Game/Assets/VFX/ShroomboAngerSymbol/BP_ShroomboAngerVFX.BP_ShroomboAngerVFX_C" (Utilities|AngryVFXSpawn) "Undefined" "MultiplyWithRoot" 0 0)
  (Utilities|FlowControl|Delay 0.5)
  (Animation|Montage|PlayMontage (Variables|Character|GetMesh) "/Game/Assets/Enemies/Shroombo/Animations/ANM_shroombo_Attack_Montage.ANM_shroombo_Attack_Montage"))

(event EventEnemyAttack
  ;[0.698 0.09412 0.1216] Enemy Attacks and Faces Player!
  (CallFunction|AttackingPlayer))

(fn ConstructionScript
  (|CallParentFunction)
  (Development|PrintString (Utilities|GetDisplayName self)))