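; Placeholder-stage Shroombo enemy that detects the player, tracks damage and shows a camera-facing health bar.
; Pawn sensing sets aggro and detection Blackboard keys, then clears them through retriggerable delays and stops movement.
; Player strikes route to HitReact, which updates the health widget and plays a hit montage, though its gate requires ShroomboIsDead to be true.
; Attack, stun and death events are empty stubs.
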(event OnSeePawn(PawnSensing)
  (params (Pawn :type Pawn%20Object%20Reference))
  (bind _self self)
  (bind _self_2 self)
  (bind _returnvalue (AI|GetAIController _self))
  (bind _returnvalue_2 (AI|GetAIController _self_2))
  (bind _returnvalue_3 (AI|GetBlackboard _returnvalue_2))
  (if (and (not (Variables|Default|GetShroomboIsDead)) (not (Variables|Default|GetShroomboIsStunned)))
    (Utilities|FlowControl|Sequence
      (:then_0
        ;[1 0.2345 0.1747] Player is Detected - Strafe & Shoot!
        (Variables|Default|SetAggro true)
        (Utilities|Casting|CastToBP_ThirdPersonCharacter Pawn)
        (AI|Components|Blackboard|SetValueasBool _returnvalue_3 (Utilities|Name|MakeLiteralName "PlayerDetected") true)
        (AI|Components|Blackboard|SetValueasBool _returnvalue_3 (Utilities|Name|MakeLiteralName "IsEnemyAggro") true))
      (:then_1
        ;[1 0.7554 0.3604] Player Out of Sight - Return to Roaming!
        (Utilities|FlowControl|RetriggerableDelay 3.0)
        (AI|Components|Blackboard|SetValueasBool (AI|GetBlackboard (AI|GetAIController self)) (Utilities|Name|MakeLiteralName "PlayerDetected") false))
      (:then_2
        ;[0.415 0.2753 1] Shroombo No Longer Aggro - Hide!
        (Utilities|FlowControl|RetriggerableDelay 3.0)
        (Variables|Default|SetAggro false)
        (AI|Components|Blackboard|SetValueasBool (AI|GetBlackboard _returnvalue) (Utilities|Name|MakeLiteralName "IsEnemyAggro") false)
        (AI|Navigation|StopMovement _returnvalue)))))

(event Custom|Rotate%20Health%20Bar
  (bind _shroombo_health_bar (Variables|Default|GetShroombo%20Health%20Bar))
  ;[0.6437 1 0.7751] EXPERIMENTAL - ADJUST HEALTH BAR ROTATION
  (Transformation|SetWorldRotation _shroombo_health_bar (Math|Rotator|FindLookatRotation (Transformation|GetWorldLocation _shroombo_health_bar) (Transformation|GetWorldLocation (Variables|/Script/Engine.PlayerCameraManager|GetTransformComponent (Game|GetPlayerCameraManager 0)))) false false))

(event Custom|Update%20Health%20Bar
  (params (Current%20Health :type Float%20%28double-precision%29))
  ;[1 0.4375 0.4375] When an Erg takes damage, update the health bar's fill!
  (bind _aswbp_enemy_health_indicator (Utilities|Casting|CastToWBP_EnemyHealthIndicator (UserInterface|GetWidget (Variables|Default|GetShroombo%20Health%20Bar))))
  (Progress|SetPercent (Variables|/Game/Assets/Enemies/EnemyUI/WBP_EnemyHealthIndicator.WBP_EnemyHealthIndicator_C|GetHealthBar _aswbp_enemy_health_indicator) (/ Current%20Health 75.0)))

(event Custom|Display%20Health%20Bar
  (params (ShouldDisplay :type Boolean))
  ;[0.372 1 0.3197] Health Bar is visible when Erg is revealed!
  (Rendering|SetVisibility (Variables|Default|GetShroombo%20Health%20Bar) ShouldDisplay false))

(event Custom|Hit%20React
  ;[0.7725 0.06667 0.3529] Enemy Takes Damage
  (if (Math|Boolean|ANDBoolean (Variables|Default|GetShroomboIsDead) (not (Variables|Default|GetTakingDamage)) (Variables|Default|GetAggro))
    (Variables|Default|SetTakingDamage true)
    (bind _output_get (Variables|Default|SetHealthOfCharacter (- (Variables|Default|GetHealthOfCharacter) (stale EventStruckbyPlayer DamageOutput))))
    (CallFunction|UpdateHealthBar _output_get)
    (if (<= (Variables|Default|GetHealthOfCharacter) 0.0)
      (CallFunction|EnemyDeath)
      (else
        ;;[0.05185 0.1405 1] HIT STUN!
        (Animation|Montage|PlayMontage (Variables|Character|GetMesh) 0
          (:then
            (Utilities|FlowControl|RetriggerableDelay 0.25)
            (Variables|Default|SetTakingDamage false)))))))

(event Custom|Enemy%20Death)

(event Custom|Lead%20Electric%20Stun
  ;[0.9098 1 0.2078] When Enemies are Stunned, they freeze in place, become vulnerable and lose sight of player until healthy again!
)

(event EventBeginPlay)

(event Collision|EventActorBeginOverlap
  (params (OtherActor :type Actor%20Object%20Reference)))

(event EventTick
  (params (DeltaSeconds :type Float%20%28single-precision%29)))

(event EventStruckbyPlayer
  (params (Player :type BP%20Third%20Person%20Character%20Object%20Reference) (DamageOutput :type Float%20%28double-precision%29))
  ;[1 0.4844 0.7588] Refer to BP_ThirdPersonCharacter's Hit Detect Function!
  (CallFunction|HitReact))

(event EventStunnedbyPlayer
  (params (Player :type BP%20Third%20Person%20Character%20Object%20Reference) (ProjectileVelocity :type Vector :default "0, 0, 0") (ProjectileLocation :type Vector :default "0, 0, 0"))
  ;[0.902 0.8824 0.4941] Sound Wave puts Enemy in Stun State!
  (CallFunction|LeadElectricStun))

(event EventAttackingPlayer
  (params (Player :type BP%20Third%20Person%20Character%20Object%20Reference))
  ;[0.6979 0.09381 0.1216] Sphere Trace for Fire - TO REFINE WHEN ANIMATIONS ARE ADDED!
  ;;[0.202 1 0.5216] Attacking Message is Received - Attack Info!
)

(fn ConstructionScript)