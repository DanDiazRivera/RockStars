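; Sporrus Maw enemy that chases and chomps the player and becomes a bounce platform when stunned.
; Pawn sensing sets blackboard aggro flags, cleared by retriggerable delays, while a self-calling loop turns it toward the player.
; Hits deal no damage but provoke a sphere-traced chomp; stuns swap pawn collision to a head platform that launches characters and ends the stun.
; First sighting or stun registers it with the GameMode for respawning.
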(event OnSeePawn(PawnSensing)
  (params (Pawn :type Pawn%20Object%20Reference))
  (bind _self self)
  (bind _self_2 self)
  (bind _returnvalue (AI|GetAIController _self))
  (bind _returnvalue_2 (AI|GetAIController _self_2))
  (bind _returnvalue_3 (AI|GetBlackboard _returnvalue_2))
  (if (and (not (Variables|Default|GetMawIsDead)) (not (Variables|Default|GetMawIsStunned)))
    (Utilities|FlowControl|Sequence
      (:then_0
        ;[1 0.2353 0.1765] Player is Detected - Turn Aggro!
        (Utilities|Casting|CastToBP_ThirdPersonCharacter Pawn)
        (bind _output_get (Variables|Default|SetAggro true))
        (AI|Components|Blackboard|SetValueasBool _returnvalue_3 (Utilities|Name|MakeLiteralName "PlayerDetected") true)
        (AI|Components|Blackboard|SetValueasBool _returnvalue_3 (Utilities|Name|MakeLiteralName "IsEnemyAggro") _output_get)
        (Development|PrintString "Player Detected!")
        (CallFunction|SearchConditions)
        ;;[0 0.09804 0.5843] Calls Add to Respawnable once
        (Utilities|FlowControl|DoOnce false
          (:Completed
            (CallFunction|AddtoRespawnable))))
      (:then_1
        ;[1 0.7554 0.3604] Player Out of Sight - Return to Roaming!
        (Utilities|FlowControl|RetriggerableDelay 3.0)
        (AI|Components|Blackboard|SetValueasBool (AI|GetBlackboard (AI|GetAIController self)) (Utilities|Name|MakeLiteralName "PlayerDetected") false)
        (Development|PrintString "Player No Longer Found!"))
      (:then_2
        ;[0.415 0.2753 1] Maw No Longer Aggro - Return to Rest!
        (Utilities|FlowControl|RetriggerableDelay 3.0)
        (bind _output_get_2 (Variables|Default|SetAggro false))
        (AI|Components|Blackboard|SetValueasBool (AI|GetBlackboard _returnvalue) (Utilities|Name|MakeLiteralName "IsEnemyAggro") _output_get_2)
        (AI|Navigation|StopMovement _returnvalue)
        (Development|PrintString "Maw No Longer Aggro!")))))

(event OnComponentBeginOverlap(StunPlatform)
  (params (OverlappedComponent :type Primitive%20Component%20Object%20Reference) (OtherActor :type Actor%20Object%20Reference) (OtherComp :type Primitive%20Component%20Object%20Reference) (OtherBodyIndex :type Integer) (bFromSweep :type Boolean) (SweepResult :type Hit%20Result%20Structure%20%28by%20ref%29))
  ;[0.2447 0.4008 0.4219] Create Bounce Mushroom Platform on Stunned Head!
  (bind _ascharacter (Utilities|Casting|CastToCharacter OtherActor))
  (Character|LaunchCharacter _ascharacter (Math|Vector|MakeVector 0.0 0.0 (Variables|Private|GetLaunchForceZ)) false true)
  ;;[0.2604 0.1841 0.08812] CHANGE BOUNCE COUNTER FOR ANIMATIONS AND CALL FOR STUN TO END
  (bind _output_get (Variables|Default|SetPlayerBounced (+ (Variables|Default|GetPlayerBounced) 1)))
  (Development|PrintString (Utilities|String|ToString(Integer) _output_get) true true "(R=0.660055,G=1.000000,B=0.140704,A=1.000000)" 3.0)
  (CallFunction|LeadElectricStunEnd)
  (CallFunction|StunCollisionsChange))

(event Custom|LeadElectricStun
  (bind _self self)
  (bind _returnvalue (AI|GetAIController _self))
  ;[0.9098 1 0.2078] When Sporrus Maws are Stunned, they freeze in place, stop attacking and can be platformed on until healthy again!
  (if (and (not (Variables|Default|GetMawIsDead)) (not (Variables|Default|GetMawIsStunned)))
    (Utilities|FlowControl|Sequence
      (:then_0
        ;;[0 0.09804 0.5843] Calls Add to Respawnable once
        (Utilities|FlowControl|DoOnce false
          (:Completed
            (CallFunction|AddtoRespawnable))))
      (:then_1
        (Variables|Default|SetPlayerBounced 0)
        (Audio|Components|Audio|Stop (Variables|Default|GetAudio))
        (AI|Navigation|StopMovement _returnvalue)
        (Development|PrintString "Enemy Stun Successful!" true true "(R=0.660055,G=1.000000,B=0.140704,A=1.000000)" 3.0)
        (bind _output_get (Variables|Default|SetMawIsStunned true))
        (Animation|Montage|PlayMontage (Variables|Character|GetMesh) "/Game/Assets/Enemies/SporrusMaw/Animations/sporrus-mawAnims_Anim_SporrusMaw_rig_SporMawStunPt1_Montage.sporrus-mawAnims_Anim_SporrusMaw_rig_SporMawStunPt1_Montage"
          (:then
            (AI|Components|Blackboard|SetValueasBool (AI|GetBlackboard _returnvalue) (Utilities|Name|MakeLiteralName "IsEnemyStunned") _output_get)
            (CallFunction|StunCollisionsChange)
            (Class|BPICombatInterface|StunnedbyPlayer(Message) (Components|SkeletalMesh|GetAnimInstance (Variables|Character|GetMesh)) 0 "0, 0, 0" "0, 0, 0")
            (Utilities|FlowControl|RetriggerableDelay (Variables|Default|GetStunPause))
            (if _output_get
              (CallFunction|LeadElectricStunEnd))))))))

(event Custom|AddToRespawnable
  ;[0 0.09759 0.5841] Adds to Respawnable Struct Array so that Sporrus Maws respawn on player death
  (Utilities|FlowControl|DoOnce false
    (:Completed
      (bind _asbp_third_person_game_mode (Utilities|Casting|CastToBP_ThirdPersonGameMode (Game|GetGameMode)))
      (Utilities|Array|Add (Variables|/Game/LevelStuff/ThirdPerson/Blueprints/Movement/BP_ThirdPersonGameMode.BP_ThirdPersonGameMode_C|GetRespawnableActors _asbp_third_person_game_mode) (Utilities|Struct|MakeStruct_RespawnableActors "BP_SporrusMawEnemy_C" self (Variables|Default|GetInitialTransform))))))

(event Custom|StunCollisionsChange
  (if (not (Variables|Default|GetMawIsDead))
    (if (Variables|Default|GetMawIsStunned)
      ;[1 0.3365 0.5813] Turn StunPlatform Collision with Pawn On & Capsule Collision With Pawn Off!
      (Collision|SetCollisionResponsetoChannel (Variables|Collision|GetCapsuleComponent) "ECC_Pawn" "ECR_Ignore")
      (Utilities|FlowControl|Delay 0.5)
      (Collision|SetCollisionResponsetoChannel (Variables|Default|GetStunPlatform) "ECC_Pawn" "ECR_Overlap")
      (else
        ;[0.3608 0.3137 0.2235] Turn StunPlatform Collision with Pawn Off & Capsule Collision With Pawn On!
        (Collision|SetCollisionResponsetoChannel (Variables|Default|GetStunPlatform) "ECC_Pawn" "ECR_Ignore")
        (Utilities|FlowControl|Delay 0.5)
        (Collision|SetCollisionResponsetoChannel (Variables|Collision|GetCapsuleComponent) "ECC_Pawn" "ECR_Block")))))

(event Custom|LeadElectricStunEnd
  ;[0.2031 0.1407 0.05699] Trigger Once Stun Duration Finishes!
  (if (and (not (Variables|Default|GetMawIsDead)) (Variables|Default|GetMawIsStunned))
    (Development|PrintString "Enemy Stun Concluded!" true true "(R=0.660055,G=1.000000,B=0.140704,A=1.000000)" 3.0)
    (Audio|Components|Audio|Play (Variables|Default|GetAudio) 0.0)
    (Animation|Montage|PlayMontage (Variables|Character|GetMesh) (Utilities|Select :Index (Variables|Default|GetPlayerBounced) :Option%200 "/Game/Assets/Enemies/SporrusMaw/Animations/sporrus-mawAnims_Anim_SporrusMaw_rig_SporMawStunPt3_Montage.sporrus-mawAnims_Anim_SporrusMaw_rig_SporMawStunPt3_Montage" :Option%201 "/Game/Assets/Enemies/SporrusMaw/Animations/sporrus-mawAnims_Anim_SporrusMaw_rig_SporMawStunPt4_Montage.sporrus-mawAnims_Anim_SporrusMaw_rig_SporMawStunPt4_Montage")
      (:then
        (bind _output_get (Variables|Default|SetMawIsStunned false))
        (AI|Components|Blackboard|SetValueasBool (AI|GetBlackboard (AI|GetAIController self)) (Utilities|Name|MakeLiteralName "IsEnemyStunned") _output_get)
        (Variables|Default|SetPlayerBounced 0)
        (Class|BPICombatInterface|EndHitstop(Message) (Components|SkeletalMesh|GetAnimInstance (Variables|Character|GetMesh)))))))

(event Custom|Face%20Player
  ;[1 0.6667 0.6745] Rotation Handling!
  (if (and (not (Variables|Default|GetMawIsDead)) (not (Variables|Default|GetMawIsStunned)))
    (if (or (Variables|Default|GetSearchingForPlayer) (Variables|Default|GetTakingDamage))
      (Transformation|SetActorRotation (Math|Rotator|MakeRotator 0.0 0.0 (.yaw (Math|Interpolation|RInterpTo (Transformation|GetActorRotation) (Math|Rotator|FindLookatRotation (Transformation|GetActorLocation) (Transformation|GetActorLocation (Game|GetPlayerCharacter 0))) (Utilities|Time|GetWorldDeltaSeconds) 1e+01))))
      (Utilities|FlowControl|Delay 0.01))))

(event Custom|HitReact
  ;[0.7725 0.06667 0.3529] When hit, the Sporrus Maw shrugs off the damage!
  (Development|PrintString "Sporrus Maw Struck!" true true "(R=0.772549,G=0.066667,B=0.352941,A=1.000000)" 3.0)
  (bind _output_get (Variables|Default|SetTakingDamage true))
  (Variables|Default|SetAggro _output_get)
  (CallFunction|SearchConditions)
  (Animation|Montage|PlayMontage (Variables|Character|GetMesh) "/Game/Assets/Enemies/SporrusMaw/Animations/sporrus-maw_hit-stun_01_Montage.sporrus-maw_hit-stun_01_Montage"
    (:OnCompleted
      _)
    (:OnInterrupted
      _))
  (CallFunction|MawChomp)
  (Variables|Default|SetTakingDamage false))

(event Custom|SearchConditions
  ;[1 0.6667 0.6745] Rotation Handling!
  (if (Variables|Default|GetAggro)
    (Variables|Default|SetSearchingForPlayer true)
    (CallFunction|FacePlayer)
    (else
      (Variables|Default|SetSearchingForPlayer false)))
  (Utilities|FlowControl|Delay 0.01)
  (CallFunction|SearchConditions))

(event Custom|Maw%20Chomp
  (bind _capsulecomponent (Variables|Collision|GetCapsuleComponent))
  (bind _returnvalue (Transformation|GetWorldLocation _capsulecomponent))
  (if (and (not (Variables|Default|GetMawIsDead)) (not (Variables|Default|GetMawIsStunned)))
    ;[0.6979 0.09381 0.1216] Sphere Trace for Chomp - TO REFINE WHEN ANIMATIONS ARE ADDED!
    (bind _outhit (Collision|SphereTraceForObjects _returnvalue _returnvalue 7.5e+02 (Utilities|Array|MakeArray "ObjectTypeQuery3") false 0 "None")) ; This sphere is meant to find the player's mesh, using its coordinates for the chomp.
    (Utilities|Casting|CastToBP_ThirdPersonCharacter (.HitActor (Collision|BreakHitResult _outhit)))
    (Utilities|FlowControl|Delay 1.0)
    (if (and (not (Variables|Default|GetMawIsStunned)) (not (Variables|Default|GetChomping))) ; ADJUST FOR ANIMS LATER!
      (Variables|Default|SetChomping true)
      (CallFunction|AttackingPlayer)
      (Animation|Montage|PlayMontage (Variables|Character|GetMesh) "/Game/Assets/Enemies/SporrusMaw/Animations/sporrus-mawAnims_Anim_SporrusMaw_rig_SporMawAttack_Montage.sporrus-mawAnims_Anim_SporrusMaw_rig_SporMawAttack_Montage"
        (:OnCompleted
          _)
        (:OnInterrupted
          _))
      (Variables|Default|SetChomping false))))

(event EventBeginPlay
  ;[0.9734 0.1683 0] Saves Initial Transform for respawning
  (Variables|Default|SetInitialTransform (Transformation|GetActorTransform)))

(event Collision|EventActorBeginOverlap
  (params (OtherActor :type Actor%20Object%20Reference)))

(event EventTick
  (params (DeltaSeconds :type Float%20%28single-precision%29)))

(event EventStunnedbyPlayer
  (params (Player :type BP%20Third%20Person%20Character%20Object%20Reference) (ProjectileVelocity :type Vector :default "0, 0, 0") (ProjectileLocation :type Vector :default "0, 0, 0"))
  (CallFunction|LeadElectricStun))

(event EventStruckbyPlayer
  (params (Player :type BP%20Third%20Person%20Character%20Object%20Reference) (DamageOutput :type Float%20%28double-precision%29))
  (if (Math|Boolean|ANDBoolean (not (Variables|Default|GetMawIsStunned)) (not (Variables|Default|GetTakingDamage)) (not (Variables|Default|GetChomping)))
    (CallFunction|PlayMawHitSound)
    (CallFunction|HitReact)))

(event EventAttackingPlayer
  (params (Player :type BP%20Third%20Person%20Character%20Object%20Reference))
  (bind _mesh (Variables|Character|GetMesh))
  (bind _returnvalue (Transformation|GetSocketLocation _mesh "c_head_x"))
  ;[0.6979 0.09381 0.1216] Sphere Trace for Chomp - TO REFINE WHEN ANIMATIONS ARE ADDED!
  ;;[0.202 1 0.5216] Attacking Message is Received - Attack Info!
  (bind _outhit (Collision|SphereTraceForObjects _returnvalue _returnvalue 3e+02 (Utilities|Array|MakeArray "ObjectTypeQuery3") false 0 "None")) ; Hit Sphere for Chomp
  (bind _asbp_third_person_character (Utilities|Casting|CastToBP_ThirdPersonCharacter (.HitActor (Collision|BreakHitResult _outhit))))
  (Default|HitReact _asbp_third_person_character))

(fn ConstructionScript)

(fn PlayMawHitSound
  (bind _mawhit (Variables|Default|GetMawHit))
  (if (not (Audio|Components|Audio|IsPlaying _mawhit))
    (Audio|Components|Audio|Play _mawhit 0.0)))