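; BPC_ObjectPool is an object pool component that pre-spawns actors of a configurable class for reuse.
; On BeginPlay it spawns actors up to PoolSize, stores them in an array and flags each as not in use.
; SpawnFromPool finds the first free actor by linear search, moves it to the requested transform and marks it in use.
; An exhausted pool does not grow; it only prints a debug message.
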(event Custom|InitializePool
  (for _index (range 0 (Variables|Default|GetPoolSize))
    (bind _returnvalue (Game|SpawnActorfromClass (Variables|Default|GetPooledActorClass) (Math|Transform|MakeTransform "0, 0, 0" "0, 0, 0" "1.000000,1.000000,1.000000") "Undefined" "MultiplyWithRoot" 0 3.0 0))
    (Utilities|Array|AddUnique (Variables|Default|GetPooledActor) _returnvalue)
    (Default|SetinUse _returnvalue false)))

(event EventBeginPlay
  (CallFunction|InitializePool))

(fn FindFirstAvailableActor
  (for _array_element (Variables|Default|GetPooledActor)
    (if (not (Variables|/Game/Users/Dylan/ObjectPoolData/BP_PooledActor.BP_PooledActor_C|GetInUse _array_element))
      (return _array_element))))

(fn SpawnfromPool
  (params (SpawnTransform :type Transform))
  (bind _pooledactor (CallFunction|FindFirstAvailableActor))
  (Utilities|IsValid _pooledactor
    (:Is%20Valid
      (Transformation|SetActorTransform _pooledactor SpawnTransform)
      (Default|SetinUse _pooledactor true)
      (return 0))
    (:Is%20Not%20Valid
      (Development|PrintString "OBJECT POOL INDEX SPAWN INVALID WOMP WOMP WOMP" true true "(R=0.171875,G=0.000000,B=0.032166,A=1.000000)"))))