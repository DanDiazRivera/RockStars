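; BP_PooledActor is an actor for object pooling that switches between in-use and idle states, starting idle.
; SetInUse toggles collision and visibility, and enables tick only while idle, the inverse of the in-use flag.
; Every SetInUse call restarts the TimeToLive timer, whose event calls SetInUse(false), so the timer keeps re-arming even while the actor is idle.
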(event Custom|SetInUse
  (params (InUse :type Boolean))
  (bind _returnvalue (not InUse))
  ;[0.255 0.1325 0.2552] If this pooled object is in use, activate it, move it to its spawn position, and set its life timer!
  (Variables|Default|SetInUse InUse)
  (Collision|SetActorEnableCollision InUse)
  (Rendering|SetActorHiddenInGame _returnvalue)
  (Actor|Tick|SetActorTickEnabled _returnvalue)
  (Utilities|Time|ClearandInvalidateTimerbyHandle (Variables|Default|GetTimeToLiveTimer))
  (bind _returnvalue_2 (Utilities|Time|SetTimerbyEvent (delegate Custom|ReturnToBool) (Variables|Default|GetTimeToLive)))
  (Variables|Default|SetTimeToLiveTimer _returnvalue_2))

(event Custom|ReturnToBool
  ;[0.255 0.1325 0.2552] If this pooled object is in use, activate it, move it to its spawn position, and set its life timer!
  (CallFunction|SetinUse false))

(event EventBeginPlay
  ;[0.255 0.1325 0.2552] If this pooled object is in use, activate it, move it to its spawn position, and set its life timer!
  (CallFunction|SetinUse false))

(fn ConstructionScript)