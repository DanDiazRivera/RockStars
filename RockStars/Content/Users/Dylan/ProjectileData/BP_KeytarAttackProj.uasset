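; Keytar attack projectile that homes in on nearby targets and damages actors implementing the combat interface.
; A looping timer sphere-traces around it, assigning a hit actor's skeletal mesh as homing target and restarting the self-destruct timer.
; Overlaps play impact effects, sending damage and hitstop through BPI_CombatInterface before destroying the projectile.
; It also destroys itself with impact effects when stopped, or fizzle effects when the timer expires without a valid target.
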(event OnProjectileStop(ProjectileMovement)
  (params (ImpactResult :type Hit%20Result%20Structure%20%28by%20ref%29))
  ;[1 0.7119 0.7721] If speed is too low, sound wave dissipates!
  ; * Liam added play impact sound here
  (CallFunction|PlayImpactSoundandVFX)
  (Actor|DestroyActor))

(event OnComponentBeginOverlap(SphereCollider)
  (params (OverlappedComponent :type Primitive%20Component%20Object%20Reference) (OtherActor :type Actor%20Object%20Reference) (OtherComp :type Primitive%20Component%20Object%20Reference) (OtherBodyIndex :type Integer) (bFromSweep :type Boolean) (SweepResult :type Hit%20Result%20Structure%20%28by%20ref%29))
  ;[0.7639 0.112 0.08541] **Liam Change: Whenever the projectile hits something, play the impact sound.
  ; Damage Target & Destroy Shot on Collision with Pawns!
  (CallFunction|PlayImpactSoundandVFX)
  (if (Utilities|DoesObjectImplementInterface OtherActor "/Game/LevelStuff/ThirdPerson/Blueprints/Weapons/BPI_CombatInterface.BPI_CombatInterface_C")
    (Class|BPICombatInterface|StruckbyPlayer(Message) OtherActor 0 (Variables|Default|GetDamage%20Output))
    (Class|BPICombatInterface|BeginHitstop(Message) OtherActor 0.04 0.1)
    (Actor|DestroyActor)))

(event Custom|FizzTimer
  ;[0.661 1 0.1625] When the projectile is spawned, it seeks a target and destroys itself if it fails to find one after 3 seconds.
  (bind _returnvalue (Utilities|Time|SetTimerbyEvent (delegate Custom|ProjSelfDestruct) 3.0))
  (Variables|Default|SetTimerSelfDestruct _returnvalue))

(event Custom|TargetTestFind
  ;[0.661 1 0.1625] When the projectile is spawned, it seeks a target and destroys itself if it fails to find one after 3 seconds.
  ;;[0.3864 1 0.5776] See Below!
  (CallFunction|TestingMethod))

(event Custom|TestingMethod
  (bind _projectilemovement (Variables|Default|GetProjectileMovement))
  (bind _projectile (Variables|Default|GetProjectile))
  (bind _returnvalue (Transformation|GetWorldLocation _projectile))
  ;[0.3864 1 0.5776] HOMING CODE
  (bind _outhit (Collision|SphereTraceForObjects _returnvalue _returnvalue 512.0 (Utilities|Array|MakeArray "ObjectTypeQuery7" "ObjectTypeQuery8") false 0 "None"))
  (Utilities|IsValid (.hitactor _outhit)
    (:Is%20Valid
      (Utilities|Time|ClearandInvalidateTimerbyHandle (Variables|Default|GetTimerSelfDestruct))
      (Variables|/Script/Engine.ProjectileMovementComponent|SetHomingTargetComponent _projectilemovement (Actor|GetComponentbyClass (.hitactor _outhit) "/Script/Engine.SkeletalMeshComponent"))
      (Variables|/Script/Engine.ProjectileMovementComponent|SetbIsHomingProjectile _projectilemovement true)
      (CallFunction|FizzTimer))))

(event Custom|ProjSelfDestruct
  ;[0.661 1 0.1625] When the projectile is spawned, it seeks a target and destroys itself if it fails to find one after 3 seconds.
  ;;[0.645 0.036 0.1042] If 3 seconds pass without finding a target, the projectile self-destructs!
  (Utilities|IsValid (Variables|Default|GetHoming%20Target%20Component)
    (:Is%20Not%20Valid
      (CallFunction|PlayFizzleSoundandVFX)
      (Actor|DestroyActor))))

(event EventBeginPlay
  ;[0.661 1 0.1625] When the projectile is spawned, it seeks a target and destroys itself if it fails to find one after 3 seconds.
  (Utilities|Time|SetTimerbyEvent (delegate Custom|TargetTestFind) 0.1 true)
  (CallFunction|FizzTimer)
  (bind _returnvalue (Utilities|Time|SetTimerbyEvent (delegate Custom|ProjSelfDestruct) 3.0))
  (Variables|Default|SetTimerSelfDestruct _returnvalue))

(fn ConstructionScript)

(fn PlayImpactSoundandVFX
  (Audio|SpawnSoundatLocation "/Game/Assets/Instruments/Keytar/Audio/Keytar_Impact.Keytar_Impact" (Transformation|GetActorLocation) "0, 0, 0" 1.0 1.0 0.0 0 0)
  (Game|SpawnActorfromClass "/Game/Assets/VFX/KeytarImpact/BP_KeytarImpactVFX.BP_KeytarImpactVFX_C" (Transformation|GetActorTransform) "Undefined" "MultiplyWithRoot" 0 0))

(fn PlayFizzleSoundandVFX
  (Audio|SpawnSoundatLocation "/Game/Assets/Instruments/Keytar/Audio/Keytar_Fizzle.Keytar_Fizzle" (Transformation|GetActorLocation) "0, 0, 0" 1.0 1.0 0.0 0 0)
  (Game|SpawnActorfromClass "/Game/Assets/VFX/KeytarFizzle/BP_KeytarFizzleVFX.BP_KeytarFizzleVFX_C" (Transformation|GetActorTransform) "Undefined" "MultiplyWithRoot" 0 0))

(fn StruckbyPlayer
  (params (Player :type BP%20Third%20Person%20Character%20Object%20Reference) (DamageOutput :type Float%20%28double-precision%29)))