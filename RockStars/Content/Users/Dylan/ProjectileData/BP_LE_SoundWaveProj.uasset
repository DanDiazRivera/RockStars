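; A sound wave projectile that stuns what it overlaps and breaks physics destructibles.
; Sphere overlaps with components not tagged Destructible send a stun message to the other actor and destroy the shot.
; Hits on simulating components tagged Destructible apply a velocity-scaled impulse, then spawn and trigger an FS_MasterField to fracture them before the projectile destroys itself.
; It also destroys itself after a short lifetime or when projectile movement stops.
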(event OnProjectileStop(ProjectileMovement)
  (params (ImpactResult :type Hit%20Result%20Structure%20%28by%20ref%29))
  ;[1 0.7119 0.7721] If speed is too low, sound wave dissipates!
  (Actor|DestroyActor))

(event OnComponentBeginOverlap(Sphere)
  (params (OverlappedComponent :type Primitive%20Component%20Object%20Reference) (OtherActor :type Actor%20Object%20Reference) (OtherComp :type Primitive%20Component%20Object%20Reference) (OtherBodyIndex :type Integer) (bFromSweep :type Boolean) (SweepResult :type Hit%20Result%20Structure%20%28by%20ref%29))
  ;[0.7639 1 0.08541] Stun Target & Destroy Shot on Collision with Pawns!
  (if (not (Components|ComponentHasTag OtherComp "Destructible"))
    (Class|BPICombatInterface|StunnedbyPlayer(Message) OtherActor)
    (Actor|DestroyActor)))

(event EventBeginPlay
  (Utilities|FlowControl|Delay 3.0)
  (Actor|DestroyActor))

(event Collision|EventActorBeginOverlap
  (params (OtherActor :type Actor%20Object%20Reference)))

(event EventTick
  (params (DeltaSeconds :type Float%20%28single-precision%29)))

(event Collision|EventHit
  (params (MyComp :type Primitive%20Component%20Object%20Reference) (Other :type Actor%20Object%20Reference) (OtherComp :type Primitive%20Component%20Object%20Reference) (bSelfMoved :type Boolean) (HitLocation :type Vector :default "0, 0, 0") (HitNormal :type Vector :default "0, 0, 0") (NormalImpulse :type Vector :default "0, 0, 0") (Hit :type Hit%20Result%20Structure%20%28by%20ref%29))
  ;[1 1 1] Destructible Damage (adds Impulse force and Master Field to break)
  (if (Components|ComponentHasTag OtherComp "Destructible")
    ;;[1 1 1] Adds an impulse force on the object using the velocity of the projectile
    (if (Physics|IsSimulatingPhysics OtherComp "None")
      (Physics|AddImpulseatLocation OtherComp (* (Transformation|GetVelocity) 5e+03) (Transformation|GetActorLocation) "None")
      (Utilities|FlowControl|Delay 0.01)
      ;;[1 1 1] Spawns a master field, which triggers the fracture all over the destructible
      (bind _returnvalue (Game|SpawnActorfromClass "/Engine/EditorResources/FieldNodes/FS_MasterField.FS_MasterField_C" (Math|Transform|MakeTransform HitLocation "0, 0, 0" "2.000000,2.000000,2.000000") "Undefined" "MultiplyWithRoot" 0 0))
      (Variables|/Engine/EditorResources/FieldNodes/FS_MasterField.FS_MasterField_C|SetActivationType _returnvalue "NewEnumerator4")
      (Default|CETrigger _returnvalue)
      (Actor|DestroyActor))))

(fn ConstructionScript)