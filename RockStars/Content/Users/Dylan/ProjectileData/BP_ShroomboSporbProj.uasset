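; Shroombo Sporb projectile that damages and triggers hallucinations in combat-interface actors it hits.
; It bursts on any component hit or two seconds after BeginPlay, spawning an actor commented as a hallucinogen smoke cloud, playing an impact sound and destroying itself.
; Hits pass trip duration, meter gain rate and damage through BPI_CombatInterface messages before the burst.
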(event OnComponentHit(Sporb)
  (params (HitComponent :type Primitive%20Component%20Object%20Reference) (OtherActor :type Actor%20Object%20Reference) (OtherComp :type Primitive%20Component%20Object%20Reference) (NormalImpulse :type Vector :default "0, 0, 0") (Hit :type Hit%20Result%20Structure%20%28by%20ref%29))
  ;[0.3906 0.07277 0.065] When the Sporb hits the player, add 50 to Hallucination Meter and burst with AOE!
  (if (Utilities|DoesObjectImplementInterface OtherActor "/Game/LevelStuff/ThirdPerson/Blueprints/Weapons/BPI_CombatInterface.BPI_CombatInterface_C")
    (Class|BPICombatInterface|InvokeHallucination(Message) OtherActor (Variables|Default|GetTripDuration) (Variables|Default|GetRateOfMeterGain))
    (Class|BPICombatInterface|StruckbyPlayer(Message) OtherActor 0 25.0)
    (CallFunction|EndOfProjLife)
    (else
      (CallFunction|EndOfProjLife))))

(event Custom|EndOfProjLife
  ;[0.3405 1 0.2532] After 2 seconds pass or a surface is hit, the Sporb bursts into a hallucinogen AOE smoke cloud!
  (Game|SpawnActorfromClass "/Game/Users/Dylan/ProjectileData/SporbAOE/BP_SporbAOE.BP_SporbAOE_C" (Transformation|GetActorTransform self) "Undefined" "MultiplyWithRoot" 0 0)
  (Audio|SpawnSoundatLocation "/Game/Assets/Enemies/Shroombo/Audio/Sporb_Impact.Sporb_Impact" (Transformation|GetActorLocation) "0, 0, 0" 1.0 1.0 0.0 0 0)
  (Actor|DestroyActor))

(event EventBeginPlay
  ;[0.3245 1 0.7009] Sporb Travels for 2 seconds before bursting!
  (Utilities|FlowControl|RetriggerableDelay 2.0)
  (CallFunction|EndOfProjLife))

(fn ConstructionScript)