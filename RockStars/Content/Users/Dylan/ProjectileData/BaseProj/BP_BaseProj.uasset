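; Base projectile Blueprint with Niagara visuals, toggled through an inherited in-use state that suggests pooled reuse.
; Entering use launches it along its forward vector by VelocityFactor and activates Niagara; leaving use stops both.
; Sphere overlaps store actors implementing BPI_CombatInterface as AffectedTarget and pass them to GetAffectedTarget, which only returns them, applying no effect here.
; CallFadeTimeline fades Niagara alpha, then releases the projectile from use.
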(event OnComponentBeginOverlap(Sphere)
  (params (OverlappedComponent :type Primitive%20Component%20Object%20Reference) (OtherActor :type Actor%20Object%20Reference) (OtherComp :type Primitive%20Component%20Object%20Reference) (OtherBodyIndex :type Integer) (bFromSweep :type Boolean) (SweepResult :type Hit%20Result%20Structure%20%28by%20ref%29))
  (if (Utilities|DoesObjectImplementInterface OtherActor "/Game/LevelStuff/ThirdPerson/Blueprints/Weapons/BPI_CombatInterface.BPI_CombatInterface_C")
    (bind _output_get (Variables|Default|SetAffectedTarget OtherActor))
    (CallFunction|GetAffectedTarget _output_get)))

(event Custom|CallFadeTimeline
  ;[0.4635 0.2073 0.4093] This timeline causes the projectile to fade away as its life ends!
  (bind _projalpha (Timeline|ProjFadeout_Timeline PlayFromStart)
    (:Update
      (Effects|Components|ParticleSystem|SetFloatParameter (Variables|Default|GetNiagara) "Scale Alpha" _projalpha))
    (:Finished
      (CallFunction|SetinUse false))))

(event EventBeginPlay
  (|CallParentFunction))

(event EventSetinUse
  (params (InUse :type Boolean))
  (|CallParentFunction InUse)
  (if InUse
    (Variables|/Script/Engine.MovementComponent|SetVelocity (Variables|Default|GetProjectileMovement) (* (Transformation|GetActorForwardVector) (Variables|Default|GetVelocityFactor)))
    (Components|Activation|Activate (Variables|Default|GetNiagara) false)
    (else
      (Variables|/Script/Engine.MovementComponent|SetVelocity (Variables|Default|GetProjectileMovement) "0, 0, 0")
      (Components|Activation|Deactivate (Variables|Default|GetNiagara)))))

(fn ConstructionScript
  (|CallParentFunction))

(fn GetAffectedTarget
  (params (Target :type Actor%20Object%20Reference))
  (return Target))