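; Mother Erg shockwave projectile that deals radial damage through an expanding ring mesh.
; On BeginPlay, a timeline widens the ring horizontally at a fixed height, then deactivates it when finished.
; Overlapping an actor with the combat interface sends it a fixed-damage struck-by-player message, deactivates the ring and calls a fade timeline.
; When the Niagara effect finishes, the projectile clears its in-use flag.
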(event OnComponentBeginOverlap(SM_RadialDamageRing)
  (params (OverlappedComponent :type Primitive%20Component%20Object%20Reference) (OtherActor :type Actor%20Object%20Reference) (OtherComp :type Primitive%20Component%20Object%20Reference) (OtherBodyIndex :type Integer) (bFromSweep :type Boolean) (SweepResult :type Hit%20Result%20Structure%20%28by%20ref%29))
  (if (Utilities|DoesObjectImplementInterface OtherActor "/Game/LevelStuff/ThirdPerson/Blueprints/Weapons/BPI_CombatInterface.BPI_CombatInterface_C")
    (Class|BPICombatInterface|StruckbyPlayer(Message) OtherActor 0 25.0)
    (Components|Activation|Deactivate (Variables|Default|GetSM_RadialDamageRing))
    (CallFunction|CallFadeTimeline)))

(event OnSystemFinished(Niagara)
  (params (PSystem :type Niagara%20Component%20Object%20Reference))
  (if (Variables|Default|GetInUse)
    (CallFunction|SetinUse false)))

(event Custom|WRDR
  (bind _sm_radialdamagering (Variables|Default|GetSM_RadialDamageRing))
  (bind _scalerdr (Timeline|TL_WidenRadialDamageRing PlayFromStart)
    (:Update
      (Transformation|SetRelativeScale3D _sm_radialdamagering (Math|Vector|MakeVector (* _scalerdr 3.0) (* _scalerdr 3.0) 0.5)))
    (:Finished
      (Components|Activation|Deactivate _sm_radialdamagering))))

(event EventBeginPlay
  (|CallParentFunction)
  (CallFunction|WRDR))

(fn ConstructionScript
  (|CallParentFunction))