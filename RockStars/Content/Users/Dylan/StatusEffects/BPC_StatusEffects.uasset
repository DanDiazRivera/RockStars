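; BPC_StatusEffects is a component that tracks the active status effects on its owner.
; Adding an effect stores it in the active collection, broadcasts an added event, then tells the effect to attempt its own application.
; Removing an effect takes it out and broadcasts a removed event, with no cleanup call on the effect itself.
; A getter exposes the collection, and the event graph holds no working logic.
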(event Custom|Signature
  (params (StatusEffectAdded :type BP%20Status%20Effects%20Object%20Reference)))

(event EventBeginPlay)

(event EventTick
  (params (DeltaSeconds :type Float%20%28single-precision%29)))

(fn GetStatusEffects
  (return (Variables|Default|GetActiveStatusEffects)))

(fn AddStatusEffect
  (params (StatusEffectToAdd :type BP%20Status%20Effects%20Object%20Reference%20%28by%20ref%29))
  (Utilities|Array|Add (Variables|Default|GetActiveStatusEffects) StatusEffectToAdd)
  (Default|CallStatusEffectWasAdded StatusEffectToAdd)
  (Default|AttemptApplication StatusEffectToAdd))

(fn RemoveStatusEffect
  (params (StatusEffectToRemove :type BP%20Status%20Effects%20Object%20Reference%20%28by%20ref%29))
  (Utilities|Array|RemoveItem (Variables|Default|GetActiveStatusEffects) StatusEffectToRemove)
  (Default|CallStatusEffectWasRemoved StatusEffectToRemove))