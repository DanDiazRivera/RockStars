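; BP_StatusEffects is a generic status effect that runs for a set duration with a periodic tick, with empty PeriodicEvent logic here.
; AttemptApplication starts it unconditionally, setting a looping periodic timer and a duration timer from StatusEffectsInfo.
; When the duration expires, it clears both timers and asks the owner's BPC_StatusEffects component, if valid, to remove it.
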(event Custom|AttemptApplication
  (CallFunction|StartStatusEffect))

(event Custom|StartStatusEffect
  (bind _statuseffectsinfo (Variables|Default|GetStatusEffectsInfo))
  (bind (_duration _periodictime) (Utilities|Struct|BreakS_StatusEffect _statuseffectsinfo))
  (bind _returnvalue (Utilities|Time|SetTimerbyEvent (delegate Custom|PeriodicEvent) _periodictime true))
  (Variables|Default|SetPeriodicTimerHandle _returnvalue)
  (bind _returnvalue_2 (Utilities|Time|SetTimerbyEvent (delegate Custom|EndStatusEffect) _duration false false 0.001))
  (Variables|Default|SetDurationTimerHandler _returnvalue_2))

(event Custom|PeriodicEvent)

(event Custom|EndStatusEffect
  (bind _returnvalue (Components|GetOwner))
  (bind _returnvalue_2 (Actor|GetComponentbyClass _returnvalue "/Game/Users/Dylan/StatusEffects/BPC_StatusEffects.BPC_StatusEffects_C"))
  (CallFunction|ClearTimers)
  (Utilities|IsValid _returnvalue_2
    (:Is%20Valid
      (Default|RemoveStatusEffect _returnvalue_2 self))))

(event EventBeginPlay)

(fn ConstructionScript)

(fn ClearTimers
  (Utilities|Time|ClearandInvalidateTimerbyHandle (Variables|Default|GetPeriodicTimerHandle))
  (Utilities|Time|ClearandInvalidateTimerbyHandle (Variables|Default|GetDurationTimerHandler))
  (return))