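; Trigger actor that changes the level when the third-person character enters its box, apparently to block a cave.
; On overlap it spawns BP_BlockRocks at a set transform, sets a relative rotation on every actor with the rotate tag, and destroys every actor with the remove tag.
; Tags, transform and rotation come from variables, and nothing guards against the trigger firing again on re-entry.
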(event OnComponentBeginOverlap(Box)
  (params (OverlappedComponent :type Primitive%20Component%20Object%20Reference) (OtherActor :type Actor%20Object%20Reference) (OtherComp :type Primitive%20Component%20Object%20Reference) (OtherBodyIndex :type Integer) (bFromSweep :type Boolean) (SweepResult :type Hit%20Result%20Structure%20%28by%20ref%29))
  (Utilities|Casting|CastToBP_ThirdPersonCharacter OtherActor)
  (Utilities|FlowControl|Sequence
    (:then_0
      (Game|SpawnActorfromClass "/Game/Users/John/BP_BlockRocks.BP_BlockRocks_C" (Variables|Default|GetSpawn%20Transform) "Undefined" "MultiplyWithRoot" 0 0))
    (:then_1
      (bind _outactors (Actor|GetAllActorswithTag (Variables|Default|GetTagRotate)))
      (Transformation|SetActorRelativeRotation _outactors (Variables|Default|GetActorRotate)))
    (:then_2
      (bind _outactors_2 (Actor|GetAllActorswithTag (Variables|Default|GetTagRemove)))
      (Actor|DestroyActor _outactors_2))))

(fn ConstructionScript)