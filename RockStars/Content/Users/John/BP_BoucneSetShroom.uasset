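; A bounce mushroom Blueprint that launches any Character overlapping its box collider into the air.
; The launch adds a hardcoded horizontal direction vector scaled by a forward force variable, while a separate Z force overrides vertical velocity.
; Each bounce also plays the Bounce sound, runs a one-shot skeletal mesh animation and spawns a Niagara spore effect at the actor's location.
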(event OnComponentBeginOverlap(BoxCollider)
  (params (OverlappedComponent :type Primitive%20Component%20Object%20Reference) (OtherActor :type Actor%20Object%20Reference) (OtherComp :type Primitive%20Component%20Object%20Reference) (OtherBodyIndex :type Integer) (bFromSweep :type Boolean) (SweepResult :type Hit%20Result%20Structure%20%28by%20ref%29))
  (bind _forwawrdlaunchforce (Variables|Public|GetForwawrdLaunchForce))
  (bind _returnvalue (* (Math|Vector|MakeVector 714.0 -189.0 0.0) _forwawrdlaunchforce))
  ;[0.1213 0.0219 0.125] When a character overlaps with the shroom's collider, launch them in the air, play a sound, play an animation, and spawn a niagara system.
  (bind _ascharacter (Utilities|Casting|CastToCharacter OtherActor))
  (Character|LaunchCharacter _ascharacter (Math|Vector|MakeVector (.x _returnvalue) (.y _returnvalue) (Variables|Public|GetLaunchForceZ)) false true)
  (Audio|Components|Audio|Play (Variables|Default|GetBounce) 0.05)
  (Components|Animation|PlayAnimation (Variables|Default|GetSkeletalMesh) "/Game/Assets/WorldAnimations/NEWBOUNCE/Bounce_Mushroom_02_Anim.Bounce_Mushroom_02_Anim" false)
  (Niagara|SpawnSystematLocation "/Game/Assets/VFX/RainbowSpore/NS_Spore.NS_Spore" (Transformation|GetActorLocation)))

(fn ConstructionScript)