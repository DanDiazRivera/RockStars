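; Cloud movement Blueprint that moves a transform pivot along a path between two marker transforms, pausing while its trigger is overlapped.
; After an initial delay on BeginPlay, a timeline lerps the pivot's world transform between the End and Start transforms without sweeping.
; Beginning a trigger overlap stops the timeline, and ending one resumes it after a short delay.
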(event OnComponentBeginOverlap(Trigger)
  (params (OverlappedComponent :type Primitive%20Component%20Object%20Reference) (OtherActor :type Actor%20Object%20Reference) (OtherComp :type Primitive%20Component%20Object%20Reference) (OtherBodyIndex :type Integer) (bFromSweep :type Boolean) (SweepResult :type Hit%20Result%20Structure%20%28by%20ref%29))
  (bind _cloudmovement (Timeline|CloudMoving Stop)
    (:Update
      (Transformation|SetWorldTransform (Variables|Default|GetTransformPivot) (Math|Transform|Lerp(Transform) (Transformation|GetWorldTransform (Variables|Default|GetEndTransform)) (Transformation|GetWorldTransform (Variables|Default|GetStartTransform)) _cloudmovement) false false))))

(event OnComponentEndOverlap(Trigger)
  (params (OverlappedComponent :type Primitive%20Component%20Object%20Reference) (OtherActor :type Actor%20Object%20Reference) (OtherComp :type Primitive%20Component%20Object%20Reference) (OtherBodyIndex :type Integer))
  (Utilities|FlowControl|Delay 0.5)
  (bind _cloudmovement (Timeline|CloudMoving Play)
    (:Update
      (Transformation|SetWorldTransform (Variables|Default|GetTransformPivot) (Math|Transform|Lerp(Transform) (Transformation|GetWorldTransform (Variables|Default|GetEndTransform)) (Transformation|GetWorldTransform (Variables|Default|GetStartTransform)) _cloudmovement) false false))))

(event EventBeginPlay
  (Utilities|FlowControl|Delay (Variables|Default|GetDuration))
  (bind _cloudmovement (Timeline|CloudMoving PlayFromStart)
    (:Update
      (Transformation|SetWorldTransform (Variables|Default|GetTransformPivot) (Math|Transform|Lerp(Transform) (Transformation|GetWorldTransform (Variables|Default|GetEndTransform)) (Transformation|GetWorldTransform (Variables|Default|GetStartTransform)) _cloudmovement) false false))))

(fn ConstructionScript)