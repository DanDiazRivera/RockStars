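; BP_SplineFollower is an actor that moves along the first BP_Spline found in the level, starting at BeginPlay.
; A timeline, with play rate set from TimeToCompleteS, lerps distance along the spline to drive the actor's world location and rotation.
; When a third-person character overlaps its box collider, it enables physics on the Erg component and destroys itself after a two-second delay.
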(event OnComponentBeginOverlap(BoxCollider)
  (params (OverlappedComponent :type Primitive%20Component%20Object%20Reference) (OtherActor :type Actor%20Object%20Reference) (OtherComp :type Primitive%20Component%20Object%20Reference) (OtherBodyIndex :type Integer) (bFromSweep :type Boolean) (SweepResult :type Hit%20Result%20Structure%20%28by%20ref%29))
  (Utilities|Casting|CastToBP_ThirdPersonCharacter OtherActor)
  (Development|PrintString "ColliderHit")
  (Physics|SetSimulatePhysics (Variables|Default|GetErg) true)
  (Utilities|FlowControl|Delay 2.0)
  (Actor|DestroyActor))

(event Custom|MoveObject
  (bind _spline_ref (Variables|Default|GetSpline%20Ref))
  (bind _spline (Variables|/Game/Users/John/BP_Spline.BP_Spline_C|GetSpline _spline_ref))
  (Components|Timeline|SetPlayRate (Variables|Default|GetTimeline) (/ 1.0 (Variables|Default|GetTime%20to%20Complete%20%28s%29)))
  (bind _newtrack_0 (Timeline|Timeline Play)
    (:Update
      (Transformation|SetActorTransform (Math|Transform|MakeTransform (Spline|GetLocationatDistanceAlongSpline _spline (Math|Float|Lerp 0.0 (Spline|GetSplineLength (Variables|/Game/Users/John/BP_Spline.BP_Spline_C|GetSpline (Variables|Default|GetSpline%20Ref))) _newtrack_0) "World") (Spline|GetRotationatDistanceAlongSpline _spline (Math|Float|Lerp 0.0 (Spline|GetSplineLength (Variables|/Game/Users/John/BP_Spline.BP_Spline_C|GetSpline (Variables|Default|GetSpline%20Ref))) _newtrack_0) "World") "1.000000,1.000000,1.000000")))))

(event EventBeginPlay
  (bind _returnvalue (Actor|GetActorOfClass "/Game/Users/John/BP_Spline.BP_Spline_C"))
  (Variables|Default|SetSpline%20Ref _returnvalue)
  (CallFunction|MoveObject))

(fn ConstructionScript)