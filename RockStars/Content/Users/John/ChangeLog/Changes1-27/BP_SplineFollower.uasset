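; BP_SplineFollower is an actor that moves along the spline of a BP_Spline found in the level.
; On BeginPlay it grabs that reference and runs MoveObject, a Timeline whose play rate is set from TimeToCompleteS.
; Each update maps the timeline alpha onto spline length to set the actor's world location and rotation.
; ErgFall, called from BP_Spline, enables physics on the Erg component and destroys the actor two seconds later.
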(event Custom|MoveObject
  (bind _spline_ref (Variables|Default|GetSpline%20Ref))
  (bind _spline (Variables|/Game/Users/John/ChangeLog/Changes1-27/BP_Spline.BP_Spline_C|GetSpline _spline_ref))
  (Components|Timeline|SetPlayRate (Variables|Default|GetTimeline) (/ 1.0 (Variables|Default|GetTime%20to%20Complete%20%28s%29)))
  (bind _newtrack_0 (Timeline|Timeline Play)
    (:Update
      (Transformation|SetActorTransform (Math|Transform|MakeTransform (Spline|GetLocationatDistanceAlongSpline _spline (Math|Float|Lerp 0.0 (Spline|GetSplineLength (Variables|/Game/Users/John/ChangeLog/Changes1-27/BP_Spline.BP_Spline_C|GetSpline (Variables|Default|GetSpline%20Ref))) _newtrack_0) "World") (Spline|GetRotationatDistanceAlongSpline _spline (Math|Float|Lerp 0.0 (Spline|GetSplineLength (Variables|/Game/Users/John/ChangeLog/Changes1-27/BP_Spline.BP_Spline_C|GetSpline (Variables|Default|GetSpline%20Ref))) _newtrack_0) "World") "1.000000,1.000000,1.000000")))))

(event Custom|ErgFall
  ;[1 1 1] Called in BP_Spline
  (Physics|SetSimulatePhysics (Variables|Default|GetErg) true)
  (Utilities|FlowControl|Delay 2.0)
  (Actor|DestroyActor))

(event EventBeginPlay
  ;[1 1 1] Gets Refernce from BP_Spline
  (bind _returnvalue (Actor|GetActorOfClass "/Game/Users/John/ChangeLog/Changes1-27/BP_Spline.BP_Spline_C"))
  (Variables|Default|SetSpline%20Ref _returnvalue)
  (CallFunction|MoveObject))

(fn ConstructionScript)