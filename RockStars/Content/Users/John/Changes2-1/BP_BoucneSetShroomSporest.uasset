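; Bounce mushroom that teleports the third-person character to a fixed spot on overlap and launches them along a configurable force.
; Each bounce plays a sound and mushroom animation, re-enables double jump and briefly disables the character's input.
; The first bounce also sets a fixed facing and plays the Sporest bounce level sequence, locking controller input until it ends.
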(event OnComponentBeginOverlap(BoxCollider)
  (params (OverlappedComponent :type Primitive%20Component%20Object%20Reference) (OtherActor :type Actor%20Object%20Reference) (OtherComp :type Primitive%20Component%20Object%20Reference) (OtherBodyIndex :type Integer) (bFromSweep :type Boolean) (SweepResult :type Hit%20Result%20Structure%20%28by%20ref%29))
  (bind _forwawrdlaunchforce (Variables|Public|GetForwawrdLaunchForce))
  (bind _y_force (Variables|Default|GetY%20Force))
  (bind _x_force (Variables|Default|GetX%20Force))
  (bind _returnvalue (* (Math|Vector|MakeVector _x_force _y_force 0.0) _forwawrdlaunchforce))
  ;[0.1213 0.0219 0.125] When a character overlaps with the shroom's collider, launch them in the air, play a sound, play an animation, and spawn a niagara system.
  (bind _asbp_third_person_character (Utilities|Casting|CastToBP_ThirdPersonCharacter OtherActor))
  (Utilities|FlowControl|Sequence
    (:then_0
      (Transformation|SetActorLocation _asbp_third_person_character "12932.000000,-37345.000000,10035.000000" false false)
      (Character|LaunchCharacter _asbp_third_person_character (Math|Vector|MakeVector (.x _returnvalue) (.y _returnvalue) (Variables|Public|GetLaunchForceZ)) false true)
      (Input|DisableInput _asbp_third_person_character 0)
      (Audio|Components|Audio|Play (Variables|Default|GetBounce) 0.05)
      (Components|Animation|PlayAnimation (Variables|Default|GetSkeletalMesh) "/Game/Assets/WorldAnimations/NEWBOUNCE/Bounce_Mushroom_02_Anim.Bounce_Mushroom_02_Anim" false)
      (Variables|/Game/LevelStuff/ThirdPerson/Blueprints/Movement/BP_ThirdPersonCharacter.BP_ThirdPersonCharacter_C|SetCanDoubleJump _asbp_third_person_character true)
      (Utilities|FlowControl|Delay 0.4)
      (Input|EnableInput _asbp_third_person_character 0))
    (:then_1
      (Utilities|FlowControl|DoOnce false
        (:Completed
          (Transformation|SetActorRotation _asbp_third_person_character "0.000000,157.109024,0.000000")
          (CallFunction|CameraSequence))))))

(event Custom|CameraSequence
  (bind _returnvalue (Game|GetPlayerController 0))
  (bind _returnvalue_2 (Sequencer|Player|CreateLevelSequencePlayer "/Game/Users/John/Sequence_SporestBounce.Sequence_SporestBounce"))
  (Input|DisableInput _returnvalue 0)
  (Sequencer|Player|Play _returnvalue_2 :!class /Script/MovieScene.MovieSceneSequencePlayer)
  (Utilities|FlowControl|Delay (Class|TimeManagementBlueprintLibrary|ToSeconds(QualifiedFrameTime) (Media|MediaPlayer|GetDuration _returnvalue_2)))
  (Input|EnableInput _returnvalue 0)
  (Development|PrintString "Hello"))

(fn ConstructionScript)