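; BPC_ValidRefs is a Blueprint component that provides cached, typed references to core gameplay objects: game instance, game mode, player character and player controller.
; Each getter returns its stored reference when valid.
; Otherwise it fetches the object, casts it to the project's Blueprint class, caches it and returns it.
; Player lookups use index 0, and a failed cast ends the getter without assigning the reference.
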(fn ValidGameInstance
  (bind _gameinstanceref (Variables|Default|GetGameInstanceRef)
    (:then
      (return _gameinstanceref))
    (:else
      (bind _asbp_game_instance (Utilities|Casting|CastToBP_GameInstance (Game|GetGameInstance)))
      (bind _output_get (Variables|Default|SetGameInstanceRef _asbp_game_instance))
      (return _output_get))))

(fn ValidGameMode
  (bind _gamemoderef (Variables|Default|GetGameModeRef)
    (:then
      (return _gamemoderef))
    (:else
      (bind _asbp_third_person_game_mode (Utilities|Casting|CastToBP_ThirdPersonGameMode (Game|GetGameMode)))
      (bind _output_get (Variables|Default|SetGameModeRef _asbp_third_person_game_mode))
      (return _output_get))))

(fn ValidPlayer
  (bind _playerref (Variables|Default|GetPlayerRef)
    (:then
      (return _playerref))
    (:else
      (bind _asbp_third_person_character (Utilities|Casting|CastToBP_ThirdPersonCharacter (Game|GetPlayerCharacter 0)))
      (bind _output_get (Variables|Default|SetPlayerRef _asbp_third_person_character))
      (return _output_get))))

(fn ValidPlayerController
  (bind _playercontrollerref (Variables|Default|GetPlayerControllerRef)
    (:then
      (return _playercontrollerref))
    (:else
      (bind _asbp_player_controller (Utilities|Casting|CastToBP_PlayerController (Game|GetPlayerController 0)))
      (bind _output_get (Variables|Default|SetPlayerControllerRef _asbp_player_controller))
      (return _output_get))))