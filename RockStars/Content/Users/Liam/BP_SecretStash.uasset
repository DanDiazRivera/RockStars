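; Hidden stash hitbox that rewards the player for repeatedly attacking or stunning it, as an easter egg.
; Strike and stun events share a DoOnce that resets after a short delay, debouncing the hit counter.
; At thirteen hits it unlocks a Steam achievement once and spawns four bandaid pickups at hard-coded world locations.
; Its shockwave interaction function simply returns false.
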(event EventStunnedbyPlayer
  (params (Player :type BP%20Third%20Person%20Character%20Object%20Reference) (ProjectileVelocity :type Vector :default "0, 0, 0") (ProjectileLocation :type Vector :default "0, 0, 0"))
  ;[0.162 0.03434 0.03311] If the secret stash hitbox is hit by an attack, or the lead electric stun wave, do the stuff.
  (Utilities|FlowControl|DoOnce false :!label _label
    (:Completed
      (Utilities|FlowControl|Sequence
        (:then_0
          (bind _result (Math|Integer|IncrementInt (Variables|Default|GetTimesHit))
            (:%20%20
              (if (>= _result 13)
                (Utilities|FlowControl|DoOnce false
                  (:Completed
                    (Default|UnlockSteamAchievement (Default|ValidGameInstance (Variables|Default|GetBPC_ValidRefs)) "ACH_EE_Secret_Stash_RS")
                    (Game|SpawnActorfromClass "/Game/Assets/PickUps/Bandaid/BP_Bandaid.BP_Bandaid_C" (Math|Transform|MakeTransform "8050.000000,-23560.000000,7040.000000" "0, 0, 0" "1.000000,1.000000,1.000000") "Undefined" "MultiplyWithRoot" 0 0)
                    (Game|SpawnActorfromClass "/Game/Assets/PickUps/Bandaid/BP_Bandaid.BP_Bandaid_C" (Math|Transform|MakeTransform "8150.000000,-23680.000000,6970.000000" "0, 0, 0" "1.000000,1.000000,1.000000") "Undefined" "MultiplyWithRoot" 0 0)
                    (Game|SpawnActorfromClass "/Game/Assets/PickUps/Bandaid/BP_Bandaid.BP_Bandaid_C" (Math|Transform|MakeTransform "8150.000000,-23900.000000,6980.000000" "0, 0, 0" "1.000000,1.000000,1.000000") "Undefined" "MultiplyWithRoot" 0 0)
                    (Game|SpawnActorfromClass "/Game/Assets/PickUps/Bandaid/BP_Bandaid.BP_Bandaid_C" (Math|Transform|MakeTransform "8150.000000,-24090.000000,7090.000000" "0, 0, 0" "1.000000,1.000000,1.000000") "Undefined" "MultiplyWithRoot" 0 0)))))))
        (:then_1
          (Utilities|FlowControl|Delay 0.2)
          (goto _label Reset))))))

(event EventStruckbyPlayer
  (params (Player :type BP%20Third%20Person%20Character%20Object%20Reference) (DamageOutput :type Float%20%28double-precision%29))
  ;[0.162 0.03434 0.03311] If the secret stash hitbox is hit by an attack, or the lead electric stun wave, do the stuff.
  (Utilities|FlowControl|DoOnce false :!label _label
    (:Completed
      (Utilities|FlowControl|Sequence
        (:then_0
          (bind _result (Math|Integer|IncrementInt (Variables|Default|GetTimesHit))
            (:%20%20
              (if (>= _result 13)
                (Utilities|FlowControl|DoOnce false
                  (:Completed
                    (Default|UnlockSteamAchievement (Default|ValidGameInstance (Variables|Default|GetBPC_ValidRefs)) "ACH_EE_Secret_Stash_RS")
                    (Game|SpawnActorfromClass "/Game/Assets/PickUps/Bandaid/BP_Bandaid.BP_Bandaid_C" (Math|Transform|MakeTransform "8050.000000,-23560.000000,7040.000000" "0, 0, 0" "1.000000,1.000000,1.000000") "Undefined" "MultiplyWithRoot" 0 0)
                    (Game|SpawnActorfromClass "/Game/Assets/PickUps/Bandaid/BP_Bandaid.BP_Bandaid_C" (Math|Transform|MakeTransform "8150.000000,-23680.000000,6970.000000" "0, 0, 0" "1.000000,1.000000,1.000000") "Undefined" "MultiplyWithRoot" 0 0)
                    (Game|SpawnActorfromClass "/Game/Assets/PickUps/Bandaid/BP_Bandaid.BP_Bandaid_C" (Math|Transform|MakeTransform "8150.000000,-23900.000000,6980.000000" "0, 0, 0" "1.000000,1.000000,1.000000") "Undefined" "MultiplyWithRoot" 0 0)
                    (Game|SpawnActorfromClass "/Game/Assets/PickUps/Bandaid/BP_Bandaid.BP_Bandaid_C" (Math|Transform|MakeTransform "8150.000000,-24090.000000,7090.000000" "0, 0, 0" "1.000000,1.000000,1.000000") "Undefined" "MultiplyWithRoot" 0 0)))))))
        (:then_1
          (Utilities|FlowControl|Delay 0.2)
          (goto _label Reset))))))

(fn ConstructionScript)

(fn ShockwaveInteract
  (return false))