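; BP_BackgroundMusicChange is a trigger box that switches the background music when the player character overlaps it.
; On overlap it plays its BGM, sets a Triggered flag and requests a synchronous save through the game instance.
; Its SaveData event writes that BGM to the save object only while flagged, then clears the flag, so only triggered volumes record their track.
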(event OnComponentBeginOverlap(Box)
  (params (OverlappedComponent :type Primitive%20Component%20Object%20Reference) (OtherActor :type Actor%20Object%20Reference) (OtherComp :type Primitive%20Component%20Object%20Reference) (OtherBodyIndex :type Integer) (bFromSweep :type Boolean) (SweepResult :type Hit%20Result%20Structure%20%28by%20ref%29))
  (Utilities|Casting|CastToBP_ThirdPersonCharacter OtherActor)
  (CallFunction|PlayBGM (Variables|Default|GetBGM))
  (Variables|Default|SetTriggered true)
  (Class|BPIPersistence|RequestSave(Message) (CallFunction|ValidGameInstance) false "NewEnumerator0"))

(event EventSaveData
  (params (SaveGameRef :type BP%20Game%20Save%20Data%20Object%20Reference))
  (if (Variables|Default|GetTriggered)
    (Variables|/Game/Users/Liam/Saving/BP_GameSaveData.BP_GameSaveData_C|SetBGMSaved SaveGameRef (Variables|Default|GetBGM))
    (Variables|Default|SetTriggered false)))

(fn ConstructionScript)