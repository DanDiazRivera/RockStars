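; Anim notify that plays surface-dependent attack impact audio for BP_ThirdPersonCharacter.
; On notify, it runs a zero-length Visibility sphere trace at the right-hand socket, with debug drawing left on.
; The hit's physical surface selects the sound played at the hit location, covering rock, dirt and two creature surfaces.
; A miss shares the fallback sound with unmatched surfaces, still using the trace result's location rather than the hand's.
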(fn ReceivedNotify
  (params (MeshComp :type Skeletal%20Mesh%20Component%20Object%20Reference) (Animation :type Anim%20Sequence%20Base%20Object%20Reference) (EventReference :type Anim%20Notify%20Event%20Reference%20Structure%20%28by%20ref%29))
  (bind _asbp_third_person_character (Utilities|Casting|CastToBP_ThirdPersonCharacter (Components|GetOwner MeshComp)))
  (bind (_outhit _returnvalue) (Collision|SphereTraceByChannel (Transformation|GetSocketLocation (Variables|/Script/Engine.Character|GetMesh _asbp_third_person_character) "hand_r") (Transformation|GetSocketLocation (Variables|/Script/Engine.Character|GetMesh _asbp_third_person_character) "hand_r") 85.0 "TraceTypeQuery1" false 0 "ForDuration"))
  (if _returnvalue
    (LocalVariables|SetLocation (.Location (Collision|BreakHitResult _outhit)))
    (switch Utilities|FlowControl|Switch|SwitchonEPhysicalSurface (Collision|GetSurfaceType _outhit)
      (:SurfaceType_Default
        (Audio|PlaySoundatLocation "/Engine/VREditor/Sounds/UI/Floating_UI_Close.Floating_UI_Close" (LocalVariables|GetLocation) "0, 0, 0" 0.6 1.0 0.0 0 0 0 0 :!label _label))
      (:SurfaceType2
        (Audio|PlaySoundatLocation "/Game/Users/Liam/DynamicAttackAudio/Audio/LeadElectric/Lead_AxeSwing.Lead_AxeSwing" (LocalVariables|GetLocation) "0, 0, 0" 1.0 1.0 0.0 0 0 0 0))
      (:SurfaceType3
        (Audio|PlaySoundatLocation "/Game/Users/Liam/DynamicAttackAudio/Audio/LeadElectric/Lead_AxeSwing.Lead_AxeSwing" (LocalVariables|GetLocation) "0, 0, 0" 1.3 1.0 0.0 0 0 0 0))
      (:SurfaceType4
        (Audio|PlaySoundatLocation "/Game/Users/Liam/DynamicAttackAudio/Audio/Mic/XLR_Impact_Erg.XLR_Impact_Erg" (LocalVariables|GetLocation) "0, 0, 0" 1.0 1.0 0.0 0 0 0 0))
      (:SurfaceType5
        (Audio|PlaySoundatLocation "/Game/LevelStuff/StarterContent/Audio/Explosion01.Explosion01" (LocalVariables|GetLocation) "0, 0, 0" 0.6 1.0 0.0 0 0 0 0)))
    (else
      (goto _label)))
  (return false))