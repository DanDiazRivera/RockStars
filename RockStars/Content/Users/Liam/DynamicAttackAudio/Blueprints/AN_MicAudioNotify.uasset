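; Anim notify that plays an impact or miss sound during third-person character animations, likely attacks.
; A sphere trace at the right-hand socket finds what was hit, and the hit's surface type selects the sound.
; SetAudios maps the character's current weapon index to rock, Erg Crawler and miss sounds.
; Dirt and Sporus Maw surfaces use fixed sounds; other surfaces or no hit play the miss sound.
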(fn ReceivedNotify
  (params (MeshComp :type Skeletal%20Mesh%20Component%20Object%20Reference) (Animation :type Anim%20Sequence%20Base%20Object%20Reference) (EventReference :type Anim%20Notify%20Event%20Reference%20Structure%20%28by%20ref%29))
  (bind _asbp_third_person_character (Utilities|Casting|CastToBP_ThirdPersonCharacter (Components|GetOwner MeshComp)))
  (bind (_outhit _returnvalue) (Collision|SphereTraceByChannel (Transformation|GetSocketLocation (Variables|/Script/Engine.Character|GetMesh _asbp_third_person_character) "hand_r") (Transformation|GetSocketLocation (Variables|/Script/Engine.Character|GetMesh _asbp_third_person_character) "hand_r") 85.0 "TraceTypeQuery1" false 0 "None"))
  (if _returnvalue
    (LocalVariables|SetLocation (.Location (Collision|BreakHitResult _outhit)))
    (switch Utilities|FlowControl|Switch|SwitchonEPhysicalSurface (Collision|GetSurfaceType _outhit)
      (:SurfaceType_Default
        (Audio|PlaySoundatLocation (.MissSound (CallFunction|SetAudios (Variables|/Game/LevelStuff/ThirdPerson/Blueprints/Movement/BP_ThirdPersonCharacter.BP_ThirdPersonCharacter_C|GetCurrentWeaponIndex _asbp_third_person_character))) (LocalVariables|GetLocation) "0, 0, 0" 0.6 1.0 0.0 0 0 0 0 :!label _label))
      (:SurfaceType2
        (Audio|PlaySoundatLocation (.RockSound (CallFunction|SetAudios (Variables|/Game/LevelStuff/ThirdPerson/Blueprints/Movement/BP_ThirdPersonCharacter.BP_ThirdPersonCharacter_C|GetCurrentWeaponIndex _asbp_third_person_character))) (LocalVariables|GetLocation) "0, 0, 0" 1.0 1.0 0.0 0 0 0 0))
      (:SurfaceType3
        (Audio|PlaySoundatLocation "/Game/Users/Liam/DynamicFootstepAudio/Audio/Player_Walk_Dirt.Player_Walk_Dirt" (LocalVariables|GetLocation) "0, 0, 0" 1.3 1.0 0.0 0 0 0 0))
      (:SurfaceType4
        (Audio|PlaySoundatLocation (.ErgCrawlerSound (CallFunction|SetAudios (Variables|/Game/LevelStuff/ThirdPerson/Blueprints/Movement/BP_ThirdPersonCharacter.BP_ThirdPersonCharacter_C|GetCurrentWeaponIndex _asbp_third_person_character))) (LocalVariables|GetLocation) "0, 0, 0" 1.0 1.0 0.0 0 0 0 0))
      (:SurfaceType5
        (Audio|PlaySoundatLocation "/Game/LevelStuff/StarterContent/Audio/Explosion01.Explosion01" (LocalVariables|GetLocation) "0, 0, 0" 0.6 1.0 0.0 0 0 0 0)))
    (else
      (goto _label)))
  (return false))

(fn SetAudios
  (params (WeaponIndex :type Integer))
  (switch int WeaponIndex
    (:0
      (return "/Game/Users/Liam/DynamicAttackAudio/Audio/Mic/XLR_Impact_Wall.XLR_Impact_Wall" "/Game/Users/Liam/DynamicAttackAudio/Audio/Mic/XLR_Impact_Erg.XLR_Impact_Erg" "/Engine/VREditor/Sounds/UI/Dockable_Window_Open.Dockable_Window_Open"))
    (:1
      (return "/Engine/VREditor/Sounds/UI/Camera_Shutter.Camera_Shutter" "/Game/StarterContent/Audio/Explosion01.Explosion01" "/Engine/EngineSounds/1kSineTonePing.1kSineTonePing"))
    (:2
      (return "/Game/Users/Liam/DynamicAttackAudio/Audio/LeadElectric/InterestingStuffYa.InterestingStuffYa" "/Engine/EngineSounds/1kSineTonePing.1kSineTonePing" "/Engine/VREditor/Sounds/UI/Floating_UI_Close.Floating_UI_Close"))))