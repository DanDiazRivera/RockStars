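; Anim notify that plays weapon attack impact or miss sounds for BP_ThirdPersonCharacter.
; A stationary sphere trace at the hand_r socket reads the hit's physical surface to pick wall, rock, enemy or miss audio at the hit location.
; SetAudios maps the current weapon index to a sound set, whose metal sound is unused.
; Erg Crawler and Sporus Maw surfaces layer a creature sound over the weapon's enemy-hit sound.
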(fn ReceivedNotify
  (params (MeshComp :type Skeletal%20Mesh%20Component%20Object%20Reference) (Animation :type Anim%20Sequence%20Base%20Object%20Reference) (EventReference :type Anim%20Notify%20Event%20Reference%20Structure%20%28by%20ref%29))
  (bind _asbp_third_person_character (Utilities|Casting|CastToBP_ThirdPersonCharacter (Components|GetOwner MeshComp)))
  (bind (_outhit _returnvalue) (Collision|SphereTraceByChannel (Transformation|GetSocketLocation (Variables|/Script/Engine.Character|GetMesh _asbp_third_person_character) "hand_r") (Transformation|GetSocketLocation (Variables|/Script/Engine.Character|GetMesh _asbp_third_person_character) "hand_r") 75.0 "TraceTypeQuery1" false 0 "None"))
  (if _returnvalue
    (LocalVariables|SetLocation (.Location (Collision|BreakHitResult _outhit)))
    (switch Utilities|FlowControl|Switch|SwitchonEPhysicalSurface (Collision|GetSurfaceType _outhit)
      (:SurfaceType_Default
        (Audio|PlaySoundatLocation (.MissSound (CallFunction|SetAudios (Variables|/Game/LevelStuff/ThirdPerson/Blueprints/Movement/BP_ThirdPersonCharacter.BP_ThirdPersonCharacter_C|GetCurrentWeaponIndex _asbp_third_person_character))) (LocalVariables|GetLocation) "0, 0, 0" 0.6 1.0 0.0 0 0 0 0 :!label _label))
      (:SurfaceType1
        (Audio|PlaySoundatLocation (.WallSound (CallFunction|SetAudios (Variables|/Game/LevelStuff/ThirdPerson/Blueprints/Movement/BP_ThirdPersonCharacter.BP_ThirdPersonCharacter_C|GetCurrentWeaponIndex _asbp_third_person_character))) (LocalVariables|GetLocation) "0, 0, 0" 1.0 1.0 0.0 0 0 0 0))
      (:SurfaceType2
        (Audio|PlaySoundatLocation (.RockSound (CallFunction|SetAudios (Variables|/Game/LevelStuff/ThirdPerson/Blueprints/Movement/BP_ThirdPersonCharacter.BP_ThirdPersonCharacter_C|GetCurrentWeaponIndex _asbp_third_person_character))) (LocalVariables|GetLocation) "0, 0, 0" 1.0 1.0 0.0 0 0 0 0))
      (:SurfaceType4
        (Audio|PlaySoundatLocation (.HitEnemy (CallFunction|SetAudios (Variables|/Game/LevelStuff/ThirdPerson/Blueprints/Movement/BP_ThirdPersonCharacter.BP_ThirdPersonCharacter_C|GetCurrentWeaponIndex _asbp_third_person_character))) (LocalVariables|GetLocation) "0, 0, 0" 1.0 1.0 0.0 0 0 0 0)
        (Audio|PlaySoundatLocation "/Game/Assets/Enemies/ErgCrawler/Erg_Screech.Erg_Screech" (LocalVariables|GetLocation) "0, 0, 0" 0.5 2.0 0.0 0 0 0 0))
      (:SurfaceType5
        (Audio|PlaySoundatLocation (.HitEnemy (CallFunction|SetAudios (Variables|/Game/LevelStuff/ThirdPerson/Blueprints/Movement/BP_ThirdPersonCharacter.BP_ThirdPersonCharacter_C|GetCurrentWeaponIndex _asbp_third_person_character))) (LocalVariables|GetLocation) "0, 0, 0" 0.6 1.0 0.0 0 0 0 0)
        (Audio|PlaySoundatLocation "/Game/Users/Liam/DynamicAttackAudio/Audio/Maw/Maw_Hit.Maw_Hit" (LocalVariables|GetLocation) "0, 0, 0" 0.5 2.5 0.0 0 0 0 0)))
    (else
      (goto _label)))
  (return false))

(fn SetAudios
  (params (WeaponIndex :type Integer))
  (switch int WeaponIndex
    (:0
      (return "/Game/Users/Liam/DynamicAttackAudio/Audio/Mic/Mic_MissSwing.Mic_MissSwing" "/Game/Users/Liam/DynamicAttackAudio/Audio/Mic/XLR_Impact_Wall.XLR_Impact_Wall" "/Game/Users/Liam/DynamicFootstepAudio/Audio/Rock/Rock_Player_Walk1.Rock_Player_Walk1" "/Game/Users/Liam/DynamicAttackAudio/Audio/Mic/Mic_MetalHit.Mic_MetalHit" "/Game/Users/Liam/BounceMushroom/Audio/BounceShroom_Bounce.BounceShroom_Bounce"))
    (:1
      (return "/Engine/EngineSounds/1kSineTonePing.1kSineTonePing" "/Game/Users/Liam/RhythmicAttackAudio/1Chord.1Chord" "/Engine/VREditor/Sounds/UI/Camera_Shutter.Camera_Shutter" "/Game/Users/Liam/GrappleHook/Audio/Grapple_Metal2.Grapple_Metal2" "/Game/StarterContent/Audio/Explosion01.Explosion01"))
    (:2
      (return "/Engine/VREditor/Sounds/UI/Floating_UI_Close.Floating_UI_Close" "/Game/Users/Liam/RhythmicAttackAudio/5Chord.5Chord" "/Game/Users/Liam/Stalagmites/ColumnDestroyed.ColumnDestroyed" "/Game/Users/Liam/DynamicAttackAudio/Audio/LeadElectric/InterestingStuffYa.InterestingStuffYa" "/Game/Users/Liam/DynamicAttackAudio/Audio/LeadElectric/Lead_AxeSwing.Lead_AxeSwing"))))