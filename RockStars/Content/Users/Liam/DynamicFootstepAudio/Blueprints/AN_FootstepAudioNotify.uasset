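; Animation notify that plays footstep sounds matched to the surface beneath the animated mesh's owner.
; When fired, it line-traces down from the owner's location along its up axis on the Visibility channel and reads the hit's physical surface type.
; Rock and Dirt surfaces each play a random sound from their own array at the impact location, with volume and pitch randomized within configurable ranges.
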(fn ReceivedNotify
  (params (MeshComp :type Skeletal%20Mesh%20Component%20Object%20Reference) (Animation :type Anim%20Sequence%20Base%20Object%20Reference) (EventReference :type Anim%20Notify%20Event%20Reference%20Structure%20%28by%20ref%29))
  (bind _returnvalue (Components|GetOwner MeshComp))
  (bind _returnvalue_2 (Transformation|GetActorLocation _returnvalue))
  (bind (_outhit _returnvalue_3) (Collision|LineTraceByChannel _returnvalue_2 (+ _returnvalue_2 (* (Transformation|GetActorUpVector _returnvalue) -2e+02)) "TraceTypeQuery1" false 0 "None"))
  (if _returnvalue_3
    (LocalVariables|SetLocation (.Location (Collision|BreakHitResult _outhit)))
    (switch Utilities|FlowControl|Switch|SwitchonEPhysicalSurface (Collision|GetSurfaceType _outhit)
      (:SurfaceType2
        (Audio|PlaySoundatLocation (Private|Constant|GetRandomRockAudio) (LocalVariables|GetLocation) "0, 0, 0" (Math|Random|RandomFloatinRange (Variables|Volume|GetMinVolume) (Variables|Volume|GetMaxVolume)) (Math|Random|RandomFloatinRange (Variables|Pitch|GetMinPitch) (Variables|Pitch|GetMaxPitch)) 0.0 0 0 0 0))
      (:SurfaceType3
        (Audio|PlaySoundatLocation (Private|Constant|GetRandomDirtAudio) (LocalVariables|GetLocation) "0, 0, 0" (Math|Random|RandomFloatinRange (Variables|Volume|GetMinVolume) (Variables|Volume|GetMaxVolume)) (Math|Random|RandomFloatinRange (Variables|Pitch|GetMinPitch) (Variables|Pitch|GetMaxPitch)) 0.0 0 0 0 0))))
  (return false))

(fn GetRandomRockAudio
  (return (.OutItem (Utilities|Array|Random (Variables|Default|GetRockAudio)))))

(fn GetRandomDirtAudio
  (return (.OutItem (Utilities|Array|Random (Variables|Default|GetDirtAudio)))))