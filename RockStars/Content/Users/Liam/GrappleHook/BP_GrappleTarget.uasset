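; Grapple point actor that shows the player a widget marker for where they can grapple.
; Each tick it checks distance and a line trace to the player, hiding the marker or showing out-of-range or wrong-weapon styling.
; It refreshes its player reference through a game mode event.
; It exposes in-range image, target location and impact VFX functions not called here; distance-based scaling is never run.
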(event Custom|GetPlayerRef
  (bind _asbp_third_person_character (Utilities|Casting|CastToBP_ThirdPersonCharacter (Game|GetPlayerCharacter 0)))
  (Variables|Default|SetPlayerRef _asbp_third_person_character))

(event EventTick
  (params (DeltaSeconds :type Float%20%28single-precision%29))
  (if (and (< (Pure|Const|DistancetoPlayer) (Variables|Private|Constant|GetVisibilityDistance)) (Pure|CheckSightlinetoPlayer))
    (if (== (Variables|/Game/LevelStuff/ThirdPerson/Blueprints/Movement/BP_ThirdPersonCharacter.BP_ThirdPersonCharacter_C|GetCurrentWeaponIndex (Variables|Default|GetPlayerRef)) 0)
      (CallFunction|DetermineGrappleTargetVisibility)
      (else
        ;[0 0 0] If the mic isn't equipped, turn the target on and use the wrong weapon image to notify the player that they are using the wrong weapon.
        (ChangeTarget|Visibility|ActiveandWrongWeaponImage true)))
    (else
      (ChangeTarget|Visibility|SetActive false))))

(event EventBeginPlay
  ;[0 0 0] Reference to player to calculate distance between player and this target.
  (CallFunction|GetPlayerRef)
  (bind _asbp_third_person_game_mode (Utilities|Casting|CastToBP_ThirdPersonGameMode (Game|GetGameMode)))
  (EventDispatchers|BindEventtoUpdatePlayerReference _asbp_third_person_game_mode (delegate Custom|GetPlayerRef)))

(fn ConstructionScript)

(fn SetActive
  (params (Active :type Boolean))
  (Rendering|SetVisibility (Variables|Default|GetWidget) Active false))

(fn GetCharacterTargetLocation
  (return (Math|Transform|TransformLocation (Transformation|GetActorTransform) (Variables|Default|GetCharacterOffset1))))

(fn SetActiveandOutOfRange
  (params (Active :type Boolean))
  ;[1 1 1] Set the target to active and change its color. This function is used when the grapple target is out of range.
  (ChangeTarget|Visibility|SetActive Active)
  (ChangeTarget|Image|GrappleOutOfRangeImage))

(fn GrappleOutOfRangeImage
  ;[0.05729 0.05729 0.05729] Set the grapple image to the out of range one.
  (bind _aswbp_grapple_target (Utilities|Casting|CastToWBP_GrappleTarget (UserInterface|GetWidget (Variables|Default|GetWidget))))
  (Default|ChangeColor _aswbp_grapple_target "(R=1.000000,G=1.000000,B=1.000000,A=1.000000)")
  (Default|ChangeImageOutOfRange _aswbp_grapple_target))

(fn GrappleinRangeImage
  ;[0.05208 0.05208 0.05208] Change the image to the in range one.
  (bind _aswbp_grapple_target (Utilities|Casting|CastToWBP_GrappleTarget (UserInterface|GetWidget (Variables|Default|GetWidget))))
  (Default|ChangeColor _aswbp_grapple_target "(R=1.000000,G=1.000000,B=1.000000,A=1.000000)")
  (Default|ChangeImageinRange _aswbp_grapple_target))

(fn DistancetoPlayer
  (bind _playerref (Variables|Default|GetPlayerRef)
    (:then
      (return (Math|Vector|Distance(Vector) (Transformation|GetActorLocation) (Transformation|GetActorLocation _playerref))))
    (:else)))

(fn PlayGrappleImpactVFX
  (ChangeTarget|Visibility|SetActive false)
  (bind _returnvalue (Game|SpawnActorfromClass "/Game/Assets/VFX/GrappleImpact/BP_GrappleImpactVFX.BP_GrappleImpactVFX_C" (Transformation|GetActorTransform) "AlwaysSpawn" "MultiplyWithRoot" 0 0))
  (Variables|Default|SetFlipbookVFX (Variables|/Game/Assets/VFX/GrappleImpact/BP_GrappleImpactVFX.BP_GrappleImpactVFX_C|GetPaperFlipbook _returnvalue))
  (Variables|Default|SetIsVFXPlaying true))

(fn CheckSightlinetoPlayer
  (bind _outhit (Collision|LineTraceByChannel (Transformation|GetActorLocation) (Transformation|GetActorLocation (Variables|Default|GetPlayerRef)) "TraceTypeQuery3" false 0 "None"))
  (if (not (.bBlockingHit (Collision|BreakHitResult _outhit)))
    (return true)
    (else
      (ChangeTarget|Visibility|SetActive false)
      (return false))))

(fn DetermineGrappleTargetVisibility
  ;[0 0 0] Player is too far to grapple to the target, but they are close enough to see where the target is.
  (if (> (Pure|Const|DistancetoPlayer) (Variables|Private|Constant|GetPlayerGrappleDistance))
    (ChangeTarget|Visibility|SetActiveandOutOfRange true)
    (else
      ;[0 0 0] If the widget is not currently active (it isn't the current target) and the player is currently in the retracted grapple state (they aren't grappling), turn the widget on and set it to the out of range image so the player knows it's there.
      (if (and (not (Components|Activation|IsActive (Variables|Default|GetWidget))) (Utilities|Enum|Equal(Enum) (Variables|/Game/Users/Liam/GrappleHook/V2GrappleComponent.V2GrappleComponent_C|GetGrappleState (Variables|/Game/LevelStuff/ThirdPerson/Blueprints/Movement/BP_ThirdPersonCharacter.BP_ThirdPersonCharacter_C|GetV2GrappleComponent (Variables|Default|GetPlayerRef))) "NewEnumerator0"))
        (ChangeTarget|Visibility|SetActiveandOutOfRange true)))))

(fn ActiveandWrongWeaponImage
  (params (Active :type Boolean))
  ;[1 1 1] Set the target to active and change its color. This function is used when the grapple target is in visible range, but the right weapon is not equipped.
  (ChangeTarget|Visibility|SetActive Active)
  (ChangeTarget|Image|GrappleWrongWeaponImage))

(fn GrappleWrongWeaponImage
  ;[0.05729 0.05729 0.05729] Set the grapple image to the wrong weapon one as the player has the wrong weapon equipped.
  (bind _aswbp_grapple_target (Utilities|Casting|CastToWBP_GrappleTarget (UserInterface|GetWidget (Variables|Default|GetWidget))))
  (Default|ChangeColor _aswbp_grapple_target "(R=1.000000,G=0.000000,B=0.026519,A=1.000000)")
  (Default|ChangeImageOutOfRange _aswbp_grapple_target))

(fn AdjustScaleBasedonDistance
  (bind _distance (Pure|Const|DistancetoPlayer))
  (bind _visibilitydistance (Variables|Private|Constant|GetVisibilityDistance))
  (bind _playergrappledistance (Variables|Private|Constant|GetPlayerGrappleDistance))
  (bind _playergrappledistance_2 (Variables|Private|Constant|GetPlayerGrappleDistance))
  (bind _minscale (Variables|Default|GetMinScale))
  (bind _normalscale (Variables|Default|GetNormalScale))
  (bind _returnvalue (- _distance _playergrappledistance_2))
  (bind _returnvalue_2 (- _visibilitydistance _playergrappledistance))
  (bind _returnvalue_3 (/ _returnvalue _returnvalue_2))
  (bind _returnvalue_4 (Math|Float|Clamp(Float) _returnvalue_3))
  (bind _returnvalue_5 (Math|Vector|Lerp(Vector) _normalscale _minscale _returnvalue_4))
  (Development|PrintString (Utilities|String|Append (Utilities|String|ToString(Vector) _returnvalue_5) "scale"))
  (Transformation|SetWorldScale3D (Variables|Default|GetBillboard) _returnvalue_5))