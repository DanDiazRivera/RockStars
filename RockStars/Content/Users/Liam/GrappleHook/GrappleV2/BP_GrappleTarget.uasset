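; BP_GrappleTarget is an actor that marks a grapple target, with a widget indicator that can be shown, hidden and recolored.
; SetActive toggles the widget's visibility, and SetActiveAndChangeColor also tints its WBP_GrappleTarget image, as used for out-of-range targets.
; GetCharacterTargetLocation converts CharacterOffset from the actor's local space to world space to give the character's target position.
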(fn ConstructionScript)

(fn SetActive
  (params (Active :type Boolean))
  (Rendering|SetVisibility (Variables|Default|GetWidget) Active false))

(fn GetCharacterTargetLocation
  (return (Math|Transform|TransformLocation (Transformation|GetActorTransform) (Variables|Default|GetCharacterOffset))))

(fn SetActiveandChangeColor
  (params (Active :type Boolean) (New%20Color :type Linear%20Color%20Structure))
  ;[1 1 1] Set the target to active and change its color. This function is used when the grapple target is out of range.
  (CallFunction|SetActive Active)
  (CallFunction|ChangeWidgetImageColor New%20Color))

(fn ChangeWidgetImageColor
  (params (New%20Color :type Linear%20Color%20Structure))
  ;[1 1 1] Change the color of the image used by the widget.
  (bind _aswbp_grapple_target (Utilities|Casting|CastToWBP_GrappleTarget (UserInterface|GetWidget (Variables|Default|GetWidget))))
  (Default|ChangeColor _aswbp_grapple_target New%20Color))