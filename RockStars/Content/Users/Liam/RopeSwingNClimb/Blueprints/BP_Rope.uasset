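; BP_Rope is a skeletal-mesh rope actor that hangs or moves under physics, apparently for a rope swing and climb feature.
; On BeginPlay it caches the third-person player character, then enables physics simulation on Bone_118 and all bones below it.
; A DisplaySockets debug helper can draw every socket name at its location, but its call is disconnected and Tick does nothing.
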(event EventBeginPlay
  (Utilities|FlowControl|Sequence
    (:then_0
      ;[0.09896 0.09896 0.09896] Get the character.
      (bind _asbp_third_person_character (Utilities|Casting|CastToBP_ThirdPersonCharacter (Game|GetPlayerCharacter 0)))
      (Variables|Default|SetCharacterRef _asbp_third_person_character))
    (:then_1
      ;[0.1042 0.1042 0.1042] Simulate physics on the rope.
      (Class|SkeletalMeshComponent|SetAllBodiesBelowSimulatePhysics (Variables|Default|GetSkeletalMesh) (Utilities|Name|MakeLiteralName "Bone_118") true true))))

(event EventTick
  (params (DeltaSeconds :type Float%20%28single-precision%29))
  ;[0.125 0.125 0.125] Display the locations of the bones.
)

(fn ConstructionScript)

(fn DisplaySockets
  (params (DisplaySockets :type Boolean))
  (if DisplaySockets
    (for _array_element (Transformation|GetAllSocketNames (Variables|Default|GetSkeletalMesh))
      (Rendering|Debug|DrawDebugString (Transformation|GetSocketLocation (Variables|Default|GetSkeletalMesh) _array_element) (Utilities|String|ToString(Name) _array_element) 0 "(R=1.000000,G=1.000000,B=1.000000,A=1.000000)"))))