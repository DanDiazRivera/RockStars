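; BP_DoubleEighthNote is a short-lived eighth-note visual effect that rises after spawning and then destroys itself.
; A timeline started on BeginPlay drives the EighthNote component's relative location, and its completion destroys the actor.
; Each tick, FacePlayer billboards the note on yaw only toward the player camera, with a fixed rotation offset.
; The construction script turns off looping on the Sprite so its animation plays once.
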(event EventTick
  (params (DeltaSeconds :type Float%20%28single-precision%29))
  (CallFunction|FacePlayer))

(event EventBeginPlay
  ;[0 0 0] When this is spawned, move it upwards. Once the movement is done, destroy it.
  (bind _z_axismovement (Timeline|VerticalMovementTimeline PlayFromStart)
    (:Update
      (Transformation|SetRelativeLocation (Variables|Default|GetEighthNote) _z_axismovement false false))
    (:Finished
      (Actor|DestroyActor))))

(fn ConstructionScript
  ;[0 0 0] When created, turn off looping.
  (Components|Timeline|SetLooping (Variables|Default|GetSprite) false))

(fn FacePlayer
  (Transformation|SetWorldRotation (Variables|Default|GetEighthNote) (Math|Rotator|CombineRotators (Math|Rotator|MakeRotator 0.0 0.0 (.yaw (Math|Rotator|FindLookatRotation (Transformation|GetWorldLocation (Variables|Default|GetEighthNote)) (Transformation|GetWorldLocation (Variables|/Script/Engine.PlayerCameraManager|GetTransformComponent (Game|GetPlayerCameraManager 0)))))) "0.000000,270.000000,0.000000") false false))