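; Crystal destructible actor that swaps an intact static mesh for a Chaos destructible when it breaks.
; On BeginPlay the CrystalDestructible component is put to sleep and hidden, leaving CrystalMesh as the stand-in.
; The first Chaos break event reveals the destructible and destroys the static mesh, guarded by a DoOnce.
; StunnedByPlayer is an empty stub, and the asset name marks it as an old version.
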(event OnChaosBreakEvent(CrystalDestructible)
  (params (BreakEvent :type Chaos%20Break%20Event%20Structure%20%28by%20ref%29))
  (Utilities|FlowControl|DoOnce false
    (:Completed
      ;[1 1 1] Destructible: Not Hidden
      (Development|SetHiddeninGame (Variables|Default|GetCrystalDestructible) false false)
      ;[1 1 1] Static Mesh: Destroyed
      (Components|DestroyComponent (Variables|Default|GetCrystalMesh)))))

(event EventBeginPlay
  ;[1 1 1] Destructible: Asleep/Hidden
  (Class|PrimitiveComponent|PutRigidBodytoSleep (Variables|Default|GetCrystalDestructible) "None")
  (Development|SetHiddeninGame (Variables|Default|GetCrystalDestructible) true false))

(fn ConstructionScript)

(fn StunnedbyPlayer
  (params (Player :type BP%20Third%20Person%20Character%20Object%20Reference) (ProjectileVelocity :type Vector :default "0, 0, 0") (ProjectileLocation :type Vector :default "0, 0, 0"))
  (return))