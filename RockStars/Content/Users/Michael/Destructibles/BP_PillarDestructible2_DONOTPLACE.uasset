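; Chaos destructible pillar that shatters when the player's stun projectile hits it.
; StunnedbyPlayer applies the projectile velocity as an impulse, then spawns and triggers an FS_MasterField at the hit location to fracture the mesh.
; The first break event plays audio, a level sequence and a camera shake centered on the player.
; It also starts a timeline that abruptly destroys the whole actor, debris included, when finished.
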(event OnChaosBreakEvent(DestructibleMesh)
  (params (BreakEvent :type Chaos%20Break%20Event%20Structure%20%28by%20ref%29))
  (Utilities|FlowControl|DoOnce false
    (:Completed
      (Utilities|FlowControl|Sequence
        (:then_0
          (Audio|Components|Audio|Play (Variables|Default|GetAudio) 0.1)
          (bind _outactor (Sequencer|Player|CreateLevelSequencePlayer (Variables|Default|GetLevel%20Sequence)))
          (Sequencer|Player|Play (Variables|/Script/LevelSequence.LevelSequenceActor|GetSequencePlayer _outactor) :!class /Script/MovieScene.MovieSceneSequencePlayer)
          (bind _asbp_third_person_character (Utilities|Casting|CastToBP_ThirdPersonCharacter (Game|GetPlayerCharacter 0)))
          (Camera|PlayWorldCameraShake "/Game/Users/Liam/CameraShake/BP_DestructibleCameraShake.BP_DestructibleCameraShake_C" (Transformation|GetActorLocation _asbp_third_person_character) 0.0 1e+03))
        (:then_1
          ;[1 1 1] Option to remove all remaining bits after set time. This is a sudden and obvious deletion, I haven't been able to get it gradual because Unreal is dookie with destructible stuff, so can't
          (Timeline|Timeline PlayFromStart
            (:Finished
              (Actor|DestroyActor))))))))

(event EventStunnedbyPlayer
  (params (Player :type BP%20Third%20Person%20Character%20Object%20Reference) (ProjectileVelocity :type Vector :default "0, 0, 0") (ProjectileLocation :type Vector :default "0, 0, 0"))
  ;[1 1 1] Applies an impulse force
  (Physics|AddImpulseatLocation (Variables|Default|GetDestructibleMesh) ProjectileVelocity ProjectileLocation "None")
  (Utilities|FlowControl|Delay 0.01)
  ;[1 1 1] Spawns a master field, which triggers the fracture all over the destructible
  (bind _returnvalue (Game|SpawnActorfromClass "/Engine/EditorResources/FieldNodes/FS_MasterField.FS_MasterField_C" (Math|Transform|MakeTransform ProjectileLocation "0, 0, 0" "2.000000,2.000000,2.000000") "Undefined" "MultiplyWithRoot" 0 0))
  (Variables|/Engine/EditorResources/FieldNodes/FS_MasterField.FS_MasterField_C|SetActivationType _returnvalue "NewEnumerator4")
  (Default|CETrigger _returnvalue))

(fn ConstructionScript)