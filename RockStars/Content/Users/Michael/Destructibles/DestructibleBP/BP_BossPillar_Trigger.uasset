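; BP_BossPillar_Trigger is a placed boss pillar that breaks when stunned by a player projectile and drops its linked stalactites.
; On stun it hides itself, spawns BP_BossPillar_DONOTPLACE, forwards projectile velocity multiplied by root scale cubed, and enables gravity on editor-assigned stalactites.
; It registers the spawned pillar as respawnable and itself as resettable with the game mode; ResetActor restores visibility, collision and initial transform.
; A breaking camera sequence is present but unconnected.
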(event Custom|CameraSequence)

(event Custom|AddToRespawnable
  ;[0 0.09759 0.5841] Adds to Respawnable Struct Array so that Destructible respawns on player death
  (Utilities|Array|AddUnique (Variables|/Game/LevelStuff/ThirdPerson/Blueprints/Movement/BP_ThirdPersonGameMode.BP_ThirdPersonGameMode_C|GetRespawnableActors (Variables|Default|GetGameModeRef)) (Utilities|Struct|MakeStruct_RespawnableActors 0 (stale EventStunnedbyPlayer _returnvalue) "0.000000,0.000000,0.000000|0.000000,0.000000,0.000000|1.000000,1.000000,1.000000")))

(event Custom|AddToResettable
  ;[0.298 0 0] Adds to Resettable Array so that Trigger resets on player death
  (Utilities|Array|AddUnique (Variables|/Game/LevelStuff/ThirdPerson/Blueprints/Movement/BP_ThirdPersonGameMode.BP_ThirdPersonGameMode_C|GetResettableActors (Variables|Default|GetGameModeRef)) self))

(event EventBeginPlay
  ;[0.9823 0.1683 0] Saves Initial Transform
  (Variables|Default|SetInitialTransform (Transformation|GetActorTransform)))

(event EventResetActor
  ;[0.298 0 0] Resettable Actor: This is called on player death to reset the actor. This adds visibility, collision, and resets transform to initial
  (Rendering|SetActorHiddenInGame false)
  (Collision|SetCollisionEnabled (Variables|Default|GetStaticMesh) "QueryAndPhysics")
  (Transformation|SetActorTransform (Variables|Default|GetInitialTransform)))

(event EventStunnedbyPlayer
  (params (Player :type BP%20Third%20Person%20Character%20Object%20Reference) (ProjectileVelocity :type Vector :default "0, 0, 0") (ProjectileLocation :type Vector :default "0, 0, 0"))
  (Variables|Default|SetRootScale (Transformation|GetWorldScale (Variables|Default|GetDefaultSceneRoot)))
  (bind _asbp_third_person_game_mode (Utilities|Casting|CastToBP_ThirdPersonGameMode (Game|GetGameMode)))
  (Variables|Default|SetGameModeRef _asbp_third_person_game_mode)
  ;[1 1 1] Hides StaticMesh, spawns new Destructible, then applies force
  (Rendering|SetActorHiddenInGame true)
  (Collision|SetCollisionEnabled (Variables|Default|GetStaticMesh) "NoCollision")
  (bind _returnvalue (Game|SpawnActorfromClass "/Game/Users/Michael/Destructibles/DestructibleBP/BP_BossPillar_DONOTPLACE.BP_BossPillar_DONOTPLACE_C" (Transformation|GetActorTransform) "Undefined" "MultiplyWithRoot" 0 0))
  (Class|BPICombatInterface|StunnedbyPlayer(Message) _returnvalue 0 (* ProjectileVelocity (Variables|Default|GetRootScale) (Variables|Default|GetRootScale) (Variables|Default|GetRootScale)) ProjectileLocation)
  (CallFunction|AddtoRespawnable)
  (CallFunction|AddtoResettable)
  ;[1 1 1] Loops through the Stalactite array (add stalactites in Editor), and enables their gravity
  (for _array_element (Variables|Default|GetStalactites)
    (bind _asbp_stalactite_trigger (Utilities|Casting|CastToBP_Stalactite_Trigger _array_element))
    (Default|EnableGravity _asbp_stalactite_trigger)))

(fn ConstructionScript)