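; Destructible boss platform that shatters when its BossTantrum event fires.
; The event applies a radial impulse from the ImpulseDirection component, then after a tiny delay spawns and triggers a large FS_MasterField to fracture the whole platform.
; The first Chaos break event plays platform and crystal audio and starts a timeline that destroys the actor when finished, removing all debris abruptly.
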(event OnChaosBreakEvent(BossPlatform)
  (params (BreakEvent :type Chaos%20Break%20Event%20Structure%20%28by%20ref%29))
  (Utilities|FlowControl|DoOnce false
    (:Completed
      (Utilities|FlowControl|Sequence
        (:then_0
          (Audio|Components|Audio|Play (Variables|Default|GetPlatformAudio) 0.1)
          (Audio|Components|Audio|Play (Variables|Default|GetCrystalAudio) 0.1))
        (:then_1
          ;[1 1 1] Option to remove all remaining bits after set time. This is a sudden and obvious deletion, I haven't been able to get it gradual because Unreal is dookie with destructible stuff, so can't
          (Timeline|Timeline PlayFromStart
            (:Finished
              (Actor|DestroyActor))))))))

(event EventBossTantrum
  (bind _impulsedirection (Variables|Default|GetImpulseDirection))
  (bind _returnvalue (Transformation|GetWorldLocation _impulsedirection))
  ;[1 1 1] Applies an impulse force
  (Physics|AddRadialImpulse (Variables|Default|GetBossPlatform) _returnvalue 1e+04 1e+04 "RIF_Constant" true)
  (Utilities|FlowControl|Delay 0.01)
  ;[1 1 1] Spawns a master field, which triggers the fracture all over the destructible
  (bind _returnvalue_2 (Game|SpawnActorfromClass "/Engine/EditorResources/FieldNodes/FS_MasterField.FS_MasterField_C" (Math|Transform|MakeTransform _returnvalue "0, 0, 0" "20.000000,20.000000,20.000000") "Undefined" "MultiplyWithRoot" 0 0))
  (Variables|/Engine/EditorResources/FieldNodes/FS_MasterField.FS_MasterField_C|SetActivationType _returnvalue_2 "NewEnumerator4")
  (Default|CETrigger _returnvalue_2))

(fn ConstructionScript)