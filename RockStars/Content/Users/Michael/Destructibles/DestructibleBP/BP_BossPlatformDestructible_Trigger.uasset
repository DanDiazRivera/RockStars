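; Boss platform with six crystals that swaps itself for a destructible version when the boss throws a tantrum.
; BossTantrum hides the actor, disables its collision, spawns BP_BossPlatformDestructible_DONOTPLACE at its transform and triggers that actor's tantrum.
; It registers the spawned destructible as respawnable and itself as resettable with the game mode for player death.
; ResetActor restores visibility and collision, but never applies the transform saved on BeginPlay.
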(event Custom|AddToRespawnable
  ;[0 0.09759 0.5841] Adds to Respawnable Struct Array so that Destructible respawns on player death
  (Utilities|Array|AddUnique (Variables|/Game/LevelStuff/ThirdPerson/Blueprints/Movement/BP_ThirdPersonGameMode.BP_ThirdPersonGameMode_C|GetRespawnableActors (Variables|Default|GetGame%20Mode%20Ref)) (Utilities|Struct|MakeStruct_RespawnableActors 0 (stale EventBossTantrum _returnvalue) "0.000000,0.000000,0.000000|0.000000,0.000000,0.000000|1.000000,1.000000,1.000000")))

(event Custom|AddToResettable
  ;[0.298 0 0] Adds to Resettable Array so that Trigger resets on player death
  (Utilities|Array|AddUnique (Variables|/Game/LevelStuff/ThirdPerson/Blueprints/Movement/BP_ThirdPersonGameMode.BP_ThirdPersonGameMode_C|GetResettableActors (Variables|Default|GetGame%20Mode%20Ref)) self))

(event EventBeginPlay
  ;[0.9823 0.1683 0] Saves Initial Transform
  (Variables|Default|SetInitialTransform (Transformation|GetActorTransform)))

(event EventResetActor
  ;[0.298 0 0] Resettable Actor: This is called on player death to reset the actor. This adds visibility, collision, and resets transform to initial
  (Rendering|SetActorHiddenInGame false)
  (Collision|SetCollisionEnabled (Variables|Default|GetBossPlatform) "QueryAndPhysics")
  (Collision|SetCollisionEnabled (Variables|Default|GetCrystal1) "QueryAndPhysics")
  (Collision|SetCollisionEnabled (Variables|Default|GetCrystal2) "QueryAndPhysics")
  (Collision|SetCollisionEnabled (Variables|Default|GetCrystal3) "QueryAndPhysics")
  (Collision|SetCollisionEnabled (Variables|Default|GetCrystal4) "QueryAndPhysics")
  (Collision|SetCollisionEnabled (Variables|Default|GetCrystal5) "QueryAndPhysics")
  (Collision|SetCollisionEnabled (Variables|Default|GetCrystal6) "QueryAndPhysics"))

(event EventBossTantrum
  (Variables|Default|SetGame%20Mode%20Ref (CallFunction|ValidGameMode))
  ;[1 1 1] Disables Visibility and Collision for Boss Platform (and all the crystals)
  (Rendering|SetActorHiddenInGame true)
  (Collision|SetCollisionEnabled (Variables|Default|GetBossPlatform) "NoCollision")
  (Collision|SetCollisionEnabled (Variables|Default|GetCrystal1) "NoCollision")
  (Collision|SetCollisionEnabled (Variables|Default|GetCrystal2) "NoCollision")
  (Collision|SetCollisionEnabled (Variables|Default|GetCrystal3) "NoCollision")
  (Collision|SetCollisionEnabled (Variables|Default|GetCrystal4) "NoCollision")
  (Collision|SetCollisionEnabled (Variables|Default|GetCrystal5) "NoCollision")
  (Collision|SetCollisionEnabled (Variables|Default|GetCrystal6) "NoCollision")
  ;[1 1 1] Destroys StaticMesh, spawns new Destructible, then applies force
  (bind _returnvalue (Game|SpawnActorfromClass "/Game/Users/Michael/Destructibles/DestructibleBP/BP_BossPlatformDestructible_DONOTPLACE.BP_BossPlatformDestructible_DONOTPLACE_C" (Transformation|GetActorTransform) "Undefined" "MultiplyWithRoot" 0 0))
  (Default|BossTantrum _returnvalue)
  (CallFunction|AddtoRespawnable)
  (CallFunction|AddtoResettable))

(fn ConstructionScript)

(fn ShockwaveInteract
  (return false))