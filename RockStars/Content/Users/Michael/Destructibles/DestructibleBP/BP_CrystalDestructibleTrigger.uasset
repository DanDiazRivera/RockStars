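; BP_CrystalDestructibleTrigger is a placed crystal that swaps itself for a destructible version when stunned by the player's projectile.
; On StunnedbyPlayer it records its root world scale, destroys itself and spawns BP_CrystalDestructibleDONOTPLACE at the same transform.
; It forwards the hit location and projectile velocity to the new actor, multiplying velocity by the cubed scale per axis to adjust force for scaled crystals.
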(event EventStunnedbyPlayer
  (params (Player :type BP%20Third%20Person%20Character%20Object%20Reference) (ProjectileVelocity :type Vector :default "0, 0, 0") (ProjectileLocation :type Vector :default "0, 0, 0"))
  ;[1 1 1] Set initial RootScale
  (Variables|Default|SetRootScale (Transformation|GetWorldScale (Variables|Default|GetDefaultSceneRoot)))
  ;[1 1 1] Destroys StaticMesh, spawns new Destructible, then applies force
  (Actor|DestroyActor)
  (bind _returnvalue (Game|SpawnActorfromClass "/Game/Users/Michael/Destructibles/DestructibleBP/BP_CrystalDestructibleDONOTPLACE.BP_CrystalDestructibleDONOTPLACE_C" (Transformation|GetActorTransform) "Undefined" "MultiplyWithRoot" 0 0))
  (Class|BPICombatInterface|StunnedbyPlayer(Message) _returnvalue 0 (* ProjectileVelocity (Math|Vector|MakeVector (Math|Float|Power (.x (Variables|Default|GetRootScale)) 3.0) (Math|Float|Power (.y (Variables|Default|GetRootScale)) 3.0) (Math|Float|Power (.z (Variables|Default|GetRootScale)) 3.0))) ProjectileLocation))

(fn ConstructionScript)