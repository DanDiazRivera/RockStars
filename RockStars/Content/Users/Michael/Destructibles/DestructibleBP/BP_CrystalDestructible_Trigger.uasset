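; Placeable crystal trigger that swaps itself for a destructible crystal when stunned by a player projectile.
; On stun it saves its scale and transform, destroys itself and spawns BP_CrystalDestructible_DONOTPLACE in its place.
; It forwards the hit location and velocity, multiplying velocity by root scale cubed per axis to adjust force for scaled crystals.
; It then registers in BP_ThirdPersonGameMode's RespawnableActors for respawn on player death.
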(event Custom|AddToRespawnable
  ;[0 0.09759 0.5841] Adds to Respawnable Struct Array so that Destructible respawns on player death
  (bind _asbp_third_person_game_mode (Utilities|Casting|CastToBP_ThirdPersonGameMode (Game|GetGameMode)))
  (Utilities|Array|Add (Variables|/Game/LevelStuff/ThirdPerson/Blueprints/Movement/BP_ThirdPersonGameMode.BP_ThirdPersonGameMode_C|GetRespawnableActors _asbp_third_person_game_mode) (Utilities|Struct|MakeStruct_RespawnableActors "BP_CrystalDestructible_Trigger_C" (stale EventStunnedbyPlayer _returnvalue) (Variables|Default|GetInitialTransform))))

(event EventStunnedbyPlayer
  (params (Player :type BP%20Third%20Person%20Character%20Object%20Reference) (ProjectileVelocity :type Vector :default "0, 0, 0") (ProjectileLocation :type Vector :default "0, 0, 0"))
  ;[0.9823 0.1683 0] Set initial RootScale and Initial Transform
  (Variables|Default|SetRootScale (Transformation|GetWorldScale (Variables|Default|GetDefaultSceneRoot)))
  (Variables|Default|SetInitialTransform (Transformation|GetActorTransform))
  ;[0.09759 0 0.491] Destroys StaticMesh, spawns new Destructible, then applies force
  (Actor|DestroyActor)
  (bind _returnvalue (Game|SpawnActorfromClass "/Game/Users/Michael/Destructibles/DestructibleBP/BP_CrystalDestructible_DONOTPLACE.BP_CrystalDestructible_DONOTPLACE_C" (Variables|Default|GetInitialTransform) "Undefined" "MultiplyWithRoot" 0 0))
  (Class|BPICombatInterface|StunnedbyPlayer(Message) _returnvalue 0 (* ProjectileVelocity (Math|Vector|MakeVector (Math|Float|Power (.x (Variables|Default|GetRootScale)) 3.0) (Math|Float|Power (.y (Variables|Default|GetRootScale)) 3.0) (Math|Float|Power (.z (Variables|Default|GetRootScale)) 3.0))) ProjectileLocation)
  ;[0 0.09804 0.5843] Calls Add to Respawnable
  (CallFunction|AddtoRespawnable))

(fn ConstructionScript)