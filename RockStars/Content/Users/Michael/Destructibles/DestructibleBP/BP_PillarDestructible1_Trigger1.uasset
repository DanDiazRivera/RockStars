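; Placeholder pillar destructible that, when stunned by a player projectile, destroys itself and spawns BP_PillarDestructible1_DONOTPLACE at its transform.
; It forwards the hit location and velocity to the spawned actor, multiplying velocity by the cube of root world scale to adjust force for scaled pieces.
; A CameraSequence event plays the Column1 breaking sequence with player input disabled for its duration, but its only call here is disconnected.
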(event Custom|CameraSequence
  (bind _returnvalue (Game|GetPlayerController 0))
  (bind _returnvalue_2 (Sequencer|Player|CreateLevelSequencePlayer "/Game/Users/John/Sequence_Column1Breaking.Sequence_Column1Breaking"))
  (Input|DisableInput _returnvalue _returnvalue)
  (Sequencer|Player|Play _returnvalue_2 :!class /Script/MovieScene.MovieSceneSequencePlayer)
  (Utilities|FlowControl|Delay (Class|TimeManagementBlueprintLibrary|ToSeconds(QualifiedFrameTime) (Media|MediaPlayer|GetDuration _returnvalue_2)))
  (Input|EnableInput _returnvalue _returnvalue))

(event EventStunnedbyPlayer
  (params (Player :type BP%20Third%20Person%20Character%20Object%20Reference) (ProjectileVelocity :type Vector :default "0, 0, 0") (ProjectileLocation :type Vector :default "0, 0, 0"))
  (Variables|Default|SetRootScale (Transformation|GetWorldScale (Variables|Default|GetDefaultSceneRoot)))
  ;[1 1 1] Destroys StaticMesh, spawns new Destructible, then applies force
  (Actor|DestroyActor)
  (bind _returnvalue (Game|SpawnActorfromClass "/Game/Users/Michael/Destructibles/DestructibleBP/BP_PillarDestructible1_DONOTPLACE.BP_PillarDestructible1_DONOTPLACE_C" (Transformation|GetActorTransform) "Undefined" "MultiplyWithRoot" 0 0))
  (Class|BPICombatInterface|StunnedbyPlayer(Message) _returnvalue 0 (* ProjectileVelocity (Variables|Default|GetRootScale) (Variables|Default|GetRootScale) (Variables|Default|GetRootScale)) ProjectileLocation))

(fn ConstructionScript)