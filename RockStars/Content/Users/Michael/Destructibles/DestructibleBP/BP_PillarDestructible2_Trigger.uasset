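; Trigger actor for the second destructible pillar, which breaks when stunned by a player projectile and saves that state.
; On stun it saves, swaps itself for BP_PillarDestructible2_DONOTPLACE, forwarding projectile velocity scaled by root scale cubed.
; It then starts the Sequence_Column2 camera sequence with player input disabled, after already calling DestroyActor.
; On load, a saved trigger plays ColumnLevelSequence from its end and removes the actor.
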(event Custom|CameraSequence
  (bind _returnvalue (Game|GetPlayerController 0))
  (bind _returnvalue_2 (Sequencer|Player|CreateLevelSequencePlayer "/Game/Users/John/Sequence_Column2.Sequence_Column2"))
  (Input|DisableInput _returnvalue _returnvalue)
  (Sequencer|Player|Play _returnvalue_2 :!class /Script/MovieScene.MovieSceneSequencePlayer)
  (Utilities|FlowControl|Delay (Class|TimeManagementBlueprintLibrary|ToSeconds(QualifiedFrameTime) (Media|MediaPlayer|GetDuration _returnvalue_2)))
  (Input|EnableInput _returnvalue _returnvalue)
  (Development|PrintString "Hello"))

(event EventStunnedbyPlayer
  (params (Player :type BP%20Third%20Person%20Character%20Object%20Reference) (ProjectileVelocity :type Vector :default "0, 0, 0") (ProjectileLocation :type Vector :default "0, 0, 0"))
  (Variables|Default|SetRootScale (Transformation|GetWorldScale (Variables|Default|GetDefaultSceneRoot)))
  (Variables|Default|SetColumn%20Triggered true)
  (Class|BPIPersistence|RequestSave(Message) (Default|ValidGameInstance (Variables|Default|GetBPC_ValidRefs)) false "NewEnumerator0")
  ;[1 1 1] Destroys StaticMesh, spawns new Destructible, then applies force
  (Actor|DestroyActor)
  (bind _returnvalue (Game|SpawnActorfromClass "/Game/Users/Michael/Destructibles/DestructibleBP/BP_PillarDestructible2_DONOTPLACE.BP_PillarDestructible2_DONOTPLACE_C" (Transformation|GetActorTransform) "Undefined" "MultiplyWithRoot" 0 0))
  (Class|BPICombatInterface|StunnedbyPlayer(Message) _returnvalue 0 (* ProjectileVelocity (Variables|Default|GetRootScale) (Variables|Default|GetRootScale) (Variables|Default|GetRootScale)) ProjectileLocation)
  (CallFunction|CameraSequence))

(event EventBeginPlay
  (Class|BPIPersistence|RequestLoad(Message) (Default|ValidGameInstance (Variables|Default|GetBPC_ValidRefs)) self "NewEnumerator0"))

(event EventSaveData
  (params (SaveGameRef :type BP%20Game%20Save%20Data%20Object%20Reference))
  (Variables|/Game/Users/Liam/Saving/BP_GameSaveData.BP_GameSaveData_C|SetColumn2Saved SaveGameRef (Variables|Default|GetColumn%20Triggered)))

(event EventLoadData
  (params (SaveGameRef :type BP%20Game%20Save%20Data%20Object%20Reference))
  (bind _columnlevelsequence (Variables|Default|GetColumnLevelSequence))
  (if (Variables|/Game/Users/Liam/Saving/BP_GameSaveData.BP_GameSaveData_C|GetColumn2Saved SaveGameRef)
    (bind _returnvalue (Class|MovieSceneSequenceExtensions|GetPlaybackEndSeconds _columnlevelsequence))
    (bind _outactor (Sequencer|Player|CreateLevelSequencePlayer _columnlevelsequence (Utilities|Struct|MakeMovieSceneSequencePlaybackSettings false "(Value=0)" 1.0 _returnvalue false false false false false false "None" false)))
    (Sequencer|Player|Play (Variables|/Script/LevelSequence.LevelSequenceActor|GetSequencePlayer _outactor) :!class /Script/MovieScene.MovieSceneSequencePlayer)
    (Actor|DestroyActor)))

(fn ConstructionScript)

(fn ShockwaveInteract
  (return false))