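; Falling stalactite trigger that damages the Mother Erg boss and shatters into a destructible version on contact.
; EnableGravity registers it as resettable with the game mode, then after a random delay turns on physics and pushes the capsule down.
; A boss hit or overlap hides the trigger, spawns the destructible with the fall velocity and registers it for removal on player death.
; ResetActor restores the hidden trigger to its starting transform.
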(event OnComponentHit(Capsule)
  (params (HitComponent :type Primitive%20Component%20Object%20Reference) (OtherActor :type Actor%20Object%20Reference) (OtherComp :type Primitive%20Component%20Object%20Reference) (NormalImpulse :type Vector :default "0, 0, 0") (Hit :type Hit%20Result%20Structure%20%28by%20ref%29))
  (bind _returnvalue (Transformation|GetActorTransform))
  ;[1 1 1] Still messing with collisions, so idk which it will use in final product, so i have both for now
  (if (Class|GameplayStatics|ObjectIsA OtherActor "/Game/Users/Dylan/EnemyBlueprints/MotherErg_AI/BP_MotherErgBoss.BP_MotherErgBoss_C")
    (Class|BPICombatInterface|StruckbyPlayer(Message) OtherActor 0 5e+01)
    ;[1 1 1] Saves Transform/Velocity of Falling Capsule
    (Variables|Default|SetActorTransform (Math|Transform|MakeTransform (.location (Transformation|GetWorldTransform (Variables|Default|GetStaticMesh))) (.rotation _returnvalue) (.scale _returnvalue)))
    (Variables|Default|SetActorVelocity (Transformation|GetComponentVelocity (Variables|Default|GetCapsule)))
    ;[1 1 1] Disables Visibility, Collision, Gravity, and Physics of Trigger
    (Rendering|SetActorHiddenInGame true)
    (Collision|SetCollisionEnabled (Variables|Default|GetStaticMesh) "NoCollision")
    (Physics|SetEnableGravity (Variables|Default|GetCapsule) false)
    (Physics|SetSimulatePhysics (Variables|Default|GetCapsule) false)
    ;[1 1 1] Spawns Destructible Stalactite and applies the existing Velocity of the Trigger
    (bind _returnvalue_2 (Game|SpawnActorfromClass "/Game/Users/Michael/Destructibles/DestructibleBP/BP_StalactiteDestructible_DONOTPLACE.BP_StalactiteDestructible_DONOTPLACE_C" (Variables|Default|GetActorTransform) "Undefined" "MultiplyWithRoot" 0 0))
    (Class|GeometryCollectionComponent|ApplyLinearVelocity (Variables|/Game/Users/Michael/Destructibles/DestructibleBP/BP_StalactiteDestructible_DONOTPLACE.BP_StalactiteDestructible_DONOTPLACE_C|GetDestructibleMesh _returnvalue_2) 0 (Variables|Default|GetActorVelocity))
    ;[0 0.07619 0.4452] Adds the reference to specific Destructible BP, but no class or transform. This will remove any destructible pieces and not respawn anything.
    (CallFunction|AddtoRespawnable _returnvalue_2)))

(event OnComponentBeginOverlap(Capsule)
  (params (OverlappedComponent :type Primitive%20Component%20Object%20Reference) (OtherActor :type Actor%20Object%20Reference) (OtherComp :type Primitive%20Component%20Object%20Reference) (OtherBodyIndex :type Integer) (bFromSweep :type Boolean) (SweepResult :type Hit%20Result%20Structure%20%28by%20ref%29))
  (bind _returnvalue (Transformation|GetActorTransform))
  ;[1 1 1] Still messing with collisions, so idk which it will use in final product, so i have both for now
  (if (Class|GameplayStatics|ObjectIsA OtherActor "/Game/Users/Dylan/EnemyBlueprints/MotherErg_AI/BP_MotherErgBoss.BP_MotherErgBoss_C")
    (Class|BPICombatInterface|StruckbyPlayer(Message) OtherActor 0 5e+01)
    ;[1 1 1] Saves Transform/Velocity of Falling Capsule
    (Variables|Default|SetActorTransform (Math|Transform|MakeTransform (.location (Transformation|GetWorldTransform (Variables|Default|GetStaticMesh))) (.rotation _returnvalue) (.scale _returnvalue)))
    (Variables|Default|SetActorVelocity (Transformation|GetComponentVelocity (Variables|Default|GetCapsule)))
    ;[1 1 1] Disables Visibility, Collision, Gravity, and Physics of Trigger
    (Rendering|SetActorHiddenInGame true)
    (Collision|SetCollisionEnabled (Variables|Default|GetStaticMesh) "NoCollision")
    (Physics|SetEnableGravity (Variables|Default|GetCapsule) false)
    (Physics|SetSimulatePhysics (Variables|Default|GetCapsule) false)
    ;[1 1 1] Spawns Destructible Stalactite and applies the existing Velocity of the Trigger
    (bind _returnvalue_2 (Game|SpawnActorfromClass "/Game/Users/Michael/Destructibles/DestructibleBP/BP_StalactiteDestructible_DONOTPLACE.BP_StalactiteDestructible_DONOTPLACE_C" (Variables|Default|GetActorTransform) "Undefined" "MultiplyWithRoot" 0 0))
    (Class|GeometryCollectionComponent|ApplyLinearVelocity (Variables|/Game/Users/Michael/Destructibles/DestructibleBP/BP_StalactiteDestructible_DONOTPLACE.BP_StalactiteDestructible_DONOTPLACE_C|GetDestructibleMesh _returnvalue_2) 0 (Variables|Default|GetActorVelocity))
    ;[0 0.07619 0.4452] Adds the reference to specific Destructible BP, but no class or transform. This will remove any destructible pieces and not respawn anything.
    (CallFunction|AddtoRespawnable _returnvalue_2)))

(event Custom|EnableGravity
  ;[0.6105 0.2232 1] Enables Gravity of Stalactites at a random rate / Adds to Resettable Array
  (bind _asbp_third_person_game_mode (Utilities|Casting|CastToBP_ThirdPersonGameMode (Game|GetGameMode)))
  (Variables|Default|SetGameModeRef _asbp_third_person_game_mode)
  (CallFunction|AddtoResettable)
  (Utilities|FlowControl|Delay (Math|Random|RandomFloatinRange 0.0 1.6))
  (Physics|SetSimulatePhysics (Variables|Default|GetCapsule) true)
  (Physics|SetEnableGravity (Variables|Default|GetCapsule) true)
  (Physics|AddImpulse (Variables|Default|GetCapsule) "0.000000,0.000000,-4000.000000" "None" true))

(event Custom|AddToRespawnable
  (params (ActorReference :type Actor%20Object%20Reference))
  ;[0 0.09759 0.5841] Adds to Respawnable Struct Array so that Destructible Stalactite respawns on player death
  ; - Unique Implementation for Stalactites Explanation: Normal triggers destroy themselves immediately upon being hit and replace the trigger BP with the destructible BP, but for stalactites there is a period where they are falling as the trigger BP before the destructible is spawned. This means that the trigger should be added to the array when gravity is enabled, and then another entry is added to the respawnable array with no class or transform, but just the reference to the destructible instance. This will destroy it if still active when player respawns.
  (Utilities|Array|AddUnique (Variables|/Game/LevelStuff/ThirdPerson/Blueprints/Movement/BP_ThirdPersonGameMode.BP_ThirdPersonGameMode_C|GetRespawnableActors (Variables|Default|GetGameModeRef)) (Utilities|Struct|MakeStruct_RespawnableActors 0 ActorReference "0.000000,0.000000,0.000000|0.000000,0.000000,0.000000|1.000000,1.000000,1.000000")))

(event Custom|AddToResettable
  ;[0.298 0 0] Adds to Resettable Array so that Trigger resets on player death
  (Utilities|Array|AddUnique (Variables|/Game/LevelStuff/ThirdPerson/Blueprints/Movement/BP_ThirdPersonGameMode.BP_ThirdPersonGameMode_C|GetResettableActors (Variables|Default|GetGameModeRef)) self))

(event EventBeginPlay
  ;[0.9216 0.162 0.000304] Saves Initial Transform for Capsule Component
  (Variables|Default|SetInitialCapsuleTransform (Transformation|GetWorldTransform (Variables|Default|GetCapsule))))

(event EventResetActor
  ;[0.298 0 0] Resettable Actor: This is called on player death to reset the actor. This turns off Gravity and Physics, adds Visibility, Collision, and resets Transform to initial
  (Physics|SetEnableGravity (Variables|Default|GetCapsule) false)
  (Physics|SetSimulatePhysics (Variables|Default|GetCapsule) false)
  (Rendering|SetActorHiddenInGame false)
  (Collision|SetCollisionEnabled (Variables|Default|GetStaticMesh) "QueryAndPhysics")
  (Transformation|SetWorldTransform (Variables|Default|GetCapsule) (Variables|Default|GetInitialCapsuleTransform) false true))

(fn ConstructionScript)