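; Placeable falling stalactite that swaps itself for a destructible version on contact.
; The EnableGravity event turns on capsule gravity after a short random delay, so stalactites drop at staggered times.
; Any capsule hit or overlap, with no filtering, destroys the actor and spawns BP_Stalactite_DONOTPLACE at the mesh location.
; The capsule's velocity passes to the new destructible mesh to carry the motion through the swap.
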(event OnComponentHit(Capsule)
  (params (HitComponent :type Primitive%20Component%20Object%20Reference) (OtherActor :type Actor%20Object%20Reference) (OtherComp :type Primitive%20Component%20Object%20Reference) (NormalImpulse :type Vector :default "0, 0, 0") (Hit :type Hit%20Result%20Structure%20%28by%20ref%29))
  (bind _returnvalue (Transformation|GetActorTransform))
  (Development|PrintString "HIT!!!! YOOOOO")
  (Variables|Default|SetActorTransform (Math|Transform|MakeTransform (.location (Transformation|GetWorldTransform (Variables|Default|GetStaticMesh))) (.rotation _returnvalue) (.scale _returnvalue)))
  (Variables|Default|SetActorVelocity (Transformation|GetComponentVelocity (Variables|Default|GetCapsule)))
  (Actor|DestroyActor)
  (bind _returnvalue_2 (Game|SpawnActorfromClass "/Game/Users/Michael/Destructibles/DestructibleBP/BP_Stalactite_DONOTPLACE.BP_Stalactite_DONOTPLACE_C" (Variables|Default|GetActorTransform) "Undefined" "MultiplyWithRoot" 0 0))
  (Class|GeometryCollectionComponent|ApplyLinearVelocity (Variables|/Game/Users/Michael/Destructibles/DestructibleBP/BP_Stalactite_DONOTPLACE.BP_Stalactite_DONOTPLACE_C|GetDestructibleMesh _returnvalue_2) 0 (Variables|Default|GetActorVelocity)))

(event OnComponentBeginOverlap(Capsule)
  (params (OverlappedComponent :type Primitive%20Component%20Object%20Reference) (OtherActor :type Actor%20Object%20Reference) (OtherComp :type Primitive%20Component%20Object%20Reference) (OtherBodyIndex :type Integer) (bFromSweep :type Boolean) (SweepResult :type Hit%20Result%20Structure%20%28by%20ref%29))
  (bind _returnvalue (Transformation|GetActorTransform))
  (Development|PrintString "HIT!!!! YOOOOO")
  (Variables|Default|SetActorTransform (Math|Transform|MakeTransform (.location (Transformation|GetWorldTransform (Variables|Default|GetStaticMesh))) (.rotation _returnvalue) (.scale _returnvalue)))
  (Variables|Default|SetActorVelocity (Transformation|GetComponentVelocity (Variables|Default|GetCapsule)))
  (Actor|DestroyActor)
  (bind _returnvalue_2 (Game|SpawnActorfromClass "/Game/Users/Michael/Destructibles/DestructibleBP/BP_Stalactite_DONOTPLACE.BP_Stalactite_DONOTPLACE_C" (Variables|Default|GetActorTransform) "Undefined" "MultiplyWithRoot" 0 0))
  (Class|GeometryCollectionComponent|ApplyLinearVelocity (Variables|/Game/Users/Michael/Destructibles/DestructibleBP/BP_Stalactite_DONOTPLACE.BP_Stalactite_DONOTPLACE_C|GetDestructibleMesh _returnvalue_2) 0 (Variables|Default|GetActorVelocity)))

(event Custom|EnableGravity
  ;[1 1 1] Enables Gravity of Stalactites at a random rate
  (Utilities|FlowControl|Delay (Math|Random|RandomFloatinRange 0.0 1.6))
  (Physics|SetEnableGravity (Variables|Default|GetCapsule) true))

(fn ConstructionScript)