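; BP_OLDPillarDestructible is a destructible pillar that swaps an intact static mesh for a Chaos destructible when it breaks.
; At BeginPlay the destructible sleeps, hidden behind the mesh.
; The first break event plays the Destroyed effect and a level sequence, then shakes the camera around the player's location, reveals the destructible and destroys the static mesh.
; The shake and swap require a successful cast to BP_ThirdPersonCharacter.
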(event OnChaosBreakEvent(PillarDestructible)
  (params (BreakEvent :type Chaos%20Break%20Event%20Structure%20%28by%20ref%29))
  (Utilities|FlowControl|DoOnce false
    (:Completed
      (Audio|Components|Audio|Play (Variables|Default|GetDestroyed) 0.1)
      (bind _outactor (Sequencer|Player|CreateLevelSequencePlayer (Variables|Default|GetLevel%20Sequence)))
      (Sequencer|Player|Play (Variables|/Script/LevelSequence.LevelSequenceActor|GetSequencePlayer _outactor) :!class /Script/MovieScene.MovieSceneSequencePlayer)
      (bind _asbp_third_person_character (Utilities|Casting|CastToBP_ThirdPersonCharacter (Game|GetPlayerCharacter 0)))
      (Camera|PlayWorldCameraShake "/Game/Users/Liam/CameraShake/BP_DestructibleCameraShake.BP_DestructibleCameraShake_C" (Transformation|GetActorLocation _asbp_third_person_character) 0.0 1e+03)
      ;[1 1 1] Destructible: Not Hidden
      (Development|SetHiddeninGame (Variables|Default|GetPillarDestructible) false false)
      ;[1 1 1] Static Mesh: Destroyed
      (Components|DestroyComponent (Variables|Default|GetPillarMesh)))))

(event EventBeginPlay
  ;[1 1 1] Destructible: Asleep/Hidden
  (Class|PrimitiveComponent|PutRigidBodytoSleep (Variables|Default|GetPillarDestructible) "None")
  (Development|SetHiddeninGame (Variables|Default|GetPillarDestructible) true false))

(fn ConstructionScript)