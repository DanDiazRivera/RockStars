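; Trigger volume that changes the player's camera boom length and can cue the Mother Erg boss to turn.
; Overlap plays or reverses a timeline that lerps between the initial arm length and a multiplied one.
; If turning is enabled, it calls the boss's SearchConditions when phase index and readiness match, otherwise retrying on a timer that exit clears.
; It registers with the game mode as resettable, re-finding the boss on reset.
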(event OnComponentBeginOverlap(Box)
  (params (OverlappedComponent :type Primitive%20Component%20Object%20Reference) (OtherActor :type Actor%20Object%20Reference) (OtherComp :type Primitive%20Component%20Object%20Reference) (OtherBodyIndex :type Integer) (bFromSweep :type Boolean) (SweepResult :type Hit%20Result%20Structure%20%28by%20ref%29))
  ;[0.03955 0.6584 0] When Entering/Exiting the Box Collider, lerp between the old and new Camera Boom Arm Lengths
  (if (Actor|ActorHasTag OtherActor "Player")
    (bind _asbp_third_person_character (Utilities|Casting|CastToBP_ThirdPersonCharacter OtherActor))
    (if (Utilities|IsValid _asbp_third_person_character)
      (bind _output_get (Variables|Default|SetCamera%20Boom (Variables|/Game/LevelStuff/ThirdPerson/Blueprints/Movement/BP_ThirdPersonCharacter.BP_ThirdPersonCharacter_C|GetCameraBoom _asbp_third_person_character)))
      (CallFunction|BossTurn)
      (if (== (Variables|Default|GetPlayerArmLength) (Variables|/Script/Engine.SpringArmComponent|GetTargetArmLength _output_get))
        (bind _camerazoom (Timeline|Timeline_1 PlayFromStart)
          (:Update
            (if (Utilities|IsValid (Variables|Default|GetCamera%20Boom))
              (Variables|/Script/Engine.SpringArmComponent|SetTargetArmLength (Variables|Default|GetCamera%20Boom) (Math|Float|Lerp (Variables|Default|GetPlayerArmLength) (Variables|Default|GetCustomArmLength) _camerazoom)))))
        (else
          (Timeline|Timeline_1 Play))))))

(event OnComponentEndOverlap(Box)
  (params (OverlappedComponent :type Primitive%20Component%20Object%20Reference) (OtherActor :type Actor%20Object%20Reference) (OtherComp :type Primitive%20Component%20Object%20Reference) (OtherBodyIndex :type Integer))
  ;[0.03955 0.6584 0] When Entering/Exiting the Box Collider, lerp between the old and new Camera Boom Arm Lengths
  (if (Actor|ActorHasTag OtherActor "Player")
    (bind _asbp_third_person_character (Utilities|Casting|CastToBP_ThirdPersonCharacter OtherActor))
    (if (Utilities|IsValid _asbp_third_person_character)
      (bind _output_get (Variables|Default|SetCamera%20Boom (Variables|/Game/LevelStuff/ThirdPerson/Blueprints/Movement/BP_ThirdPersonCharacter.BP_ThirdPersonCharacter_C|GetCameraBoom _asbp_third_person_character)))
      (CallFunction|NoMoreGettingTurnt)
      (if (== (Variables|Default|GetCustomArmLength) (Variables|/Script/Engine.SpringArmComponent|GetTargetArmLength _output_get))
        (bind _camerazoom (Timeline|Timeline_1 ReverseFromEnd)
          (:Update
            (if (Utilities|IsValid (Variables|Default|GetCamera%20Boom))
              (Variables|/Script/Engine.SpringArmComponent|SetTargetArmLength (Variables|Default|GetCamera%20Boom) (Math|Float|Lerp (Variables|Default|GetPlayerArmLength) (Variables|Default|GetCustomArmLength) _camerazoom)))))
        (else
          (Timeline|Timeline_1 Reverse))))))

(event Custom|BossTurn
  (bind _bossref (Variables|Default|GetBossRef))
  ;[1 0.6667 0.6745] ADDED BY DYLAN: Tell boss to turn around!
  (Utilities|IsValid _bossref
    (:Is%20Valid
      (if (Variables|Default|GetShouldTurnTo)
        (if (and (== (Variables|Default|GetCamBoxIndex) (Variables|/Game/Users/Dylan/EnemyBlueprints/MotherErg_AI/BP_MotherErgBoss.BP_MotherErgBoss_C|GetPhaseIndex _bossref)) (Variables|/Game/Users/Dylan/EnemyBlueprints/MotherErg_AI/BP_MotherErgBoss.BP_MotherErgBoss_C|GetReadyToTurn _bossref))
          (Development|PrintString "Turn Valid! Mother Erg gets turnt!" true true "(R=0.213835,G=1.000000,B=0.240111,A=1.000000)")
          (Default|SearchConditions _bossref)
          (if (Utilities|Time|IsValidTimerHandle (Variables|Default|GetTurntTimer))
            (Utilities|Time|ClearandInvalidateTimerbyHandle (Variables|Default|GetTurntTimer)))
          (else
            (bind _returnvalue (Utilities|Time|SetTimerbyEvent (delegate Custom|BossTurn) 1.0 true))
            (Variables|Default|SetTurntTimer _returnvalue)
            (Development|PrintString "Turn Invalid! Check again in 1 second!" true true "(R=1.000000,G=0.255229,B=0.195485,A=1.000000)")))))))

(event Custom|NoMoreGettingTurnt
  (bind _turnttimer (Variables|Default|GetTurntTimer))
  ;[1 0.6667 0.6745] ADDED BY DYLAN: Tell boss to turn around!
  (if (Utilities|Time|IsValidTimerHandle _turnttimer)
    (Utilities|Time|ClearandInvalidateTimerbyHandle _turnttimer)))

(event Custom|AddToResettable
  ;[0.298 0 0] Adds to Resettable Array so that Trigger resets on player death.
  ; Delayed so that it doesn't call as the array is being cleared in gamemode
  (Utilities|FlowControl|Delay 1.0)
  (Utilities|Array|AddUnique (Variables|/Game/LevelStuff/ThirdPerson/Blueprints/Movement/BP_ThirdPersonGameMode.BP_ThirdPersonGameMode_C|GetResettableActors (CallFunction|ValidGameMode)) self))

(event EventBeginPlay
  ;[0 0.3916 0.8796] Gets the initial length of the Camera Boom Arm Length and saves variables for the arm length and the multiplier
  (bind _asbp_third_person_character (Utilities|Casting|CastToBP_ThirdPersonCharacter (Game|GetPlayerCharacter 0)))
  (bind _output_get (Variables|Default|SetPlayerArmLength (Variables|/Game/LevelStuff/ThirdPerson/Blueprints/Movement/BP_ThirdPersonCharacter.BP_ThirdPersonCharacter_C|GetInitialCamBoomLength _asbp_third_person_character)))
  (Variables|Default|SetCustomArmLength (* _output_get (Variables|Default|GetCustomArmMultiplier)))
  (Utilities|FlowControl|Delay 0.1)
  (Collision|SetCollisionEnabled (Variables|Default|GetBox) "QueryOnly")
  (bind _returnvalue (Actor|GetActorOfClass "/Game/Users/Dylan/EnemyBlueprints/MotherErg_AI/BP_MotherErgBoss.BP_MotherErgBoss_C"))
  (Variables|Default|SetBossRef _returnvalue)
  (CallFunction|AddtoResettable))

(event EventResetActor
  ;[0.298 0 0] Adds to Resettable Array so that Trigger resets on player death.
  ; Delayed so that it doesn't call as the array is being cleared in gamemode
  (bind _returnvalue (Actor|GetActorOfClass "/Game/Users/Dylan/EnemyBlueprints/MotherErg_AI/BP_MotherErgBoss.BP_MotherErgBoss_C"))
  (Variables|Default|SetBossRef _returnvalue))

(fn ConstructionScript)

(fn GetDectetion
  (return (Variables|Default|GetBox)))