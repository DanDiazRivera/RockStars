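; BP_SporeMine is a proximity hazard that glows as the player nears and releases an area effect at close range.
; An outer sphere runs a looping timer mapping player distance to a dynamic material's emissive intensity.
; An inner sphere spawns BP_SporeMineAOE after a short delay, then disables glow and collision for a Timeline-driven cooldown.
; The first glow overlap registers the mine with BP_ThirdPersonGameMode for respawn on player death.
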(event OnComponentBeginOverlap(GlowDetection)
  (params (OverlappedComponent :type Primitive%20Component%20Object%20Reference) (OtherActor :type Actor%20Object%20Reference) (OtherComp :type Primitive%20Component%20Object%20Reference) (OtherBodyIndex :type Integer) (bFromSweep :type Boolean) (SweepResult :type Hit%20Result%20Structure%20%28by%20ref%29))
  ;[1 0.06274 0.02353] Glow Detection: When entering the Glow Detection range, start looping timer to calculate distance to Player
  (if (Actor|ActorHasTag OtherActor "Player")
    (Variables|Default|SetPlayer OtherActor)
    (bind _returnvalue (Utilities|Time|SetTimerbyFunctionName 0 "GlowDistanceCalculator" 0.1 true))
    (Variables|Default|SetGlowDetectionTimer _returnvalue)
    (Utilities|FlowControl|DoOnce false
      (:Completed
        (CallFunction|AddtoRespawnable)))))

(event OnComponentEndOverlap(GlowDetection)
  (params (OverlappedComponent :type Primitive%20Component%20Object%20Reference) (OtherActor :type Actor%20Object%20Reference) (OtherComp :type Primitive%20Component%20Object%20Reference) (OtherBodyIndex :type Integer))
  ;[1 0.06274 0.02353] Exit Glow Detection: When exiting Glow Detection range, turn off Glow Detection Timer
  (if (Actor|ActorHasTag OtherActor "Player")
    (Utilities|Time|ClearandInvalidateTimerbyHandle (Variables|Default|GetGlowDetectionTimer))))

(event OnComponentBeginOverlap(DamageDetection)
  (params (OverlappedComponent :type Primitive%20Component%20Object%20Reference) (OtherActor :type Actor%20Object%20Reference) (OtherComp :type Primitive%20Component%20Object%20Reference) (OtherBodyIndex :type Integer) (bFromSweep :type Boolean) (SweepResult :type Hit%20Result%20Structure%20%28by%20ref%29))
  (bind _initialtransform (Variables|Default|GetInitialTransform))
  ;[0.0549 0.02353 0.02745] Damage Detection: When entering Damage Detection range, spawn AOE effect, and conduct Spore Mine Cooldown procedures. Emissive is set to 0 and Collisions are turned off until Cooldown is over
  (if (Actor|ActorHasTag OtherActor "Player")
    (Utilities|FlowControl|Delay 0.5)
    (Game|SpawnActorfromClass "/Game/Users/Michael/SporeMines/BP_SporeMineAOE.BP_SporeMineAOE_C" (Math|Transform|MakeTransform (.location _initialtransform) (.rotation _initialtransform) (* (.scale _initialtransform) 2.5)) "Undefined" "MultiplyWithRoot" 0 0)
    (Rendering|Material|SetScalarParameterValue (Variables|Default|GetSporeMineMaterial) "EmissiveIntensity" 0.0 :!class /Script/Engine.MaterialInstanceDynamic)
    (Collision|SetCollisionEnabled (Variables|Default|GetDamageDetection) "NoCollision")
    (Collision|SetCollisionEnabled (Variables|Default|GetGlowDetection) "NoCollision")
    ;;[0.5573 0.3622 0.04681] Set Cooldown value in Timeline
    (Timeline|Timeline PlayFromStart
      (:Finished
        (Rendering|Material|SetScalarParameterValue (Variables|Default|GetSporeMineMaterial) "EmissiveIntensity" (Variables|Default|GetGlowEmissiveLow) :!class /Script/Engine.MaterialInstanceDynamic)
        (Collision|SetCollisionEnabled (Variables|Default|GetDamageDetection) "QueryOnly")
        (Collision|SetCollisionEnabled (Variables|Default|GetGlowDetection) "QueryOnly")))))

(event Custom|GlowDistanceCalculator
  (bind _player (Variables|Default|GetPlayer))
  ;[0.03955 0.6584 0] Glow Distance Calculator: Calculates distance between Spore Mine and Player, and sets Emissive Value accordingly
  (if (Utilities|IsValid _player)
    (bind _output_get (Variables|Default|SetPlayerDistance (Math|Vector|Distance(Vector) (.location (Variables|Default|GetInitialTransform)) (Transformation|GetActorLocation _player))))
    (Rendering|Material|SetScalarParameterValue (Variables|Default|GetSporeMineMaterial) "EmissiveIntensity" (Math|Float|MapRangeClamped _output_get (Variables|Default|GetDamageRadius) (Variables|Default|GetGlowRadius) (Variables|Default|GetGlowEmissiveHigh) (Variables|Default|GetGlowEmissiveLow)) :!class /Script/Engine.MaterialInstanceDynamic)))

(event Custom|AddToRespawnable
  ;[0 0.09804 0.5843] Adds to Respawnable Struct Array so that Spore Mine respawns on player death
  (bind _asbp_third_person_game_mode (Utilities|Casting|CastToBP_ThirdPersonGameMode (Game|GetGameMode)))
  (Utilities|Array|Add (Variables|/Game/LevelStuff/ThirdPerson/Blueprints/Movement/BP_ThirdPersonGameMode.BP_ThirdPersonGameMode_C|GetRespawnableActors _asbp_third_person_game_mode) (Utilities|Struct|MakeStruct_RespawnableActors "BP_SporeMine_C" self (Variables|Default|GetInitialTransform))))

(event EventBeginPlay
  ;[0.2789 0.1095 0.4452] Begin Play: Creates Dynamic Material Instance and sets initial variables
  (bind _returnvalue (Rendering|Material|CreateDynamicMaterialInstance (Variables|Default|GetMushroom) 0 "/Game/Assets/EnvironmentFBX/Mushrooms/Textures/MIShrooms/MI_DeathMines.MI_DeathMines" "None" :!class /Script/Engine.PrimitiveComponent))
  (bind _output_get (Variables|Default|SetSporeMineMaterial _returnvalue))
  (Rendering|Material|SetScalarParameterValue _output_get "EmissiveIntensity" (Variables|Default|GetGlowEmissiveLow) :!class /Script/Engine.MaterialInstanceDynamic)
  (Variables|Default|SetGlowRadius (Components|Sphere|GetScaledSphereRadius (Variables|Default|GetGlowDetection)))
  (Variables|Default|SetDamageRadius (Components|Sphere|GetScaledSphereRadius (Variables|Default|GetDamageDetection)))
  (Variables|Default|SetInitialTransform (Transformation|GetWorldTransform (Variables|Default|GetDefaultSceneRoot)))
  ;;[0 0.09804 0.5843] Reenables collision to avoid Respawning errors
  (Utilities|FlowControl|Delay 0.1)
  (Collision|SetCollisionEnabled (Variables|Default|GetDamageDetection) "QueryOnly")
  (Collision|SetCollisionEnabled (Variables|Default|GetGlowDetection) "QueryOnly"))

(fn ConstructionScript)