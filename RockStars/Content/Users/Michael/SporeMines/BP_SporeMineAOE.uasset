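; Spore mine area-of-effect cloud that raises the hallucination meter of overlapping actors implementing BPI_CombatInterface, then destroys itself when its Niagara effect finishes.
; The increase rate starts high and drops to low shortly after spawn.
; Entering the field sends an immediate hallucination message and starts a looping one-second timer to repeat it.
; A single timer handle serves the field, and any end overlap clears it.
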(event OnComponentBeginOverlap(OverlapField)
  (params (OverlappedComponent :type Primitive%20Component%20Object%20Reference) (OtherActor :type Actor%20Object%20Reference) (OtherComp :type Primitive%20Component%20Object%20Reference) (OtherBodyIndex :type Integer) (bFromSweep :type Boolean) (SweepResult :type Hit%20Result%20Structure%20%28by%20ref%29))
  ;[0.3255 1 0.5725] The player's Hallucination Meter goes up by 10% per second spent in the overlap field!
  (if (Utilities|DoesObjectImplementInterface OtherActor "/Game/LevelStuff/ThirdPerson/Blueprints/Weapons/BPI_CombatInterface.BPI_CombatInterface_C")
    (Class|BPICombatInterface|InvokeHallucination(Message) OtherActor 0.0 (Variables|Default|GetHallucinationIncrease))
    (bind _returnvalue (Utilities|Time|SetTimerbyEvent (delegate Custom|HallucinateOverSeconds) 1.0 true))
    (Variables|Default|SetHallucinateHandle _returnvalue)))

(event OnComponentEndOverlap(OverlapField)
  (params (OverlappedComponent :type Primitive%20Component%20Object%20Reference) (OtherActor :type Actor%20Object%20Reference) (OtherComp :type Primitive%20Component%20Object%20Reference) (OtherBodyIndex :type Integer))
  ;[0.2941 0 1] If the player leaves the field, clear the hallucination timer!
  (Utilities|Time|ClearandInvalidateTimerbyHandle (Variables|Default|GetHallucinateHandle)))

(event OnSystemFinished(Niagara)
  (params (PSystem :type Niagara%20Component%20Object%20Reference))
  ;[0.1302 0.08816 0.08816] When the smoke clear, the object is destroyed!
  (Actor|DestroyActor))

(event Custom|HallucinateOverSeconds
  ;[0.3255 1 0.5725] The player's Hallucination Meter goes up by 10% per second spent in the overlap field!
  (Class|BPICombatInterface|InvokeHallucination(Message) (stale OnComponentBeginOverlap(OverlapField) OtherActor) 0.0 (Variables|Default|GetHallucinationIncrease))
  (Development|PrintString "AFTER"))

(event EventBeginPlay
  (Variables|Default|SetHallucinationIncrease (Variables|Default|GetHallucinationHigh))
  (Utilities|FlowControl|Delay 0.2)
  (Variables|Default|SetHallucinationIncrease (Variables|Default|GetHallucinationLow)))

(fn ConstructionScript)