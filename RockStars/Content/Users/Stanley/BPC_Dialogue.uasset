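; Dialogue component that runs NPC and overlap-triggered gameplay conversations from a DataTable, matched by owner class and encounter index.
; For NPCs, it locks player movement and turns the player toward the speaker before talking.
; A looping timer types lines into a UW_Dialogue widget character by character; talking again reveals the full line or advances.
; Finished lines can hand over the NPC's weapon, and exhausting them restores walking and removes the widget.
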(event Custom|Enter%20Dialogue
  (params (OverlappedComponent :type Primitive%20Component%20Object%20Reference) (OtherActor :type Actor%20Object%20Reference) (OtherComp :type Primitive%20Component%20Object%20Reference) (OtherBodyIndex :type Integer) (bFromSweep :type Boolean) (SweepResult :type Hit%20Result%20Structure%20%28by%20ref%29))
  (bind _asbp_third_person_character (Utilities|Casting|CastToBP_ThirdPersonCharacter OtherActor))
  (Variables|Default|SetPlayer _asbp_third_person_character)
  (if (Variables|Default|GetinConversation)
    (CallFunction|Talk)
    (else
      ;[0.2917 0.2917 0.2917] if not already in conversation, start talking
      (Utilities|Casting|CastToBP_NPC (Components|GetOwner)
        (:then
          (Default|FunctManageIMC (Variables|Default|GetPlayer))
          (Pawn|Components|CharacterMovement|DisableMovement (Variables|/Script/Engine.Character|GetCharacterMovement (Variables|Default|GetPlayer)))
          (bind _returnvalue (Utilities|Time|SetTimerbyEvent (delegate Custom|Turn%20to%20Person) (Utilities|Time|GetWorldDeltaSeconds) true))
          (Variables|Default|SetTimer_TurntoPerson _returnvalue))
        (:CastFailed
          (CallFunction|StartTalking))))))

(event Custom|Start%20Talking
  ;[0.2396 0.2396 0.2396] Start Talking
  (Variables|Default|SetinConversation true)
  (Utilities|FlowControl|Sequence
    (:then_0
      (bind _returnvalue (UserInterface|CreateWidget "/Game/Users/Stanley/UW_Dialogue.UW_Dialogue_C" (Game|GetPlayerController 0)))
      (bind _output_get (Variables|Default|SetUW_Dialogue _returnvalue))
      (UserInterface|Viewport|AddtoViewport _output_get 0))
    (:then_1
      (switch Utilities|FlowControl|Switch|SwitchonEnum_DialogueMethod (Variables|Default|GetDialogue%20Method)
        (:NewEnumerator0
          (CallFunction|SetupDialogueNPC))
        (:NewEnumerator1
          (CallFunction|SetupGameplayDialogue))))))

(event Custom|Add%20Next%20Char
  (params (Line%20to%20Add%20to :type String))
  (Variables|Dialogue|Characters|SetPrevious%20Character%20Index (Variables|Dialogue|Characters|GetCharacter%20Index))
  (bind _result (Math|Integer|IncrementInt (Variables|Dialogue|Characters|GetCharacter%20Index))
    (:%20%20
      (if (.Valid? (Dialogue|Characters|FunctGetChar@Index Line%20to%20Add%20to _result))
        (bind _output_get (Variables|Dialogue|SetCurrent%20Dialogue (CallFunction|FunctAddChartoLine (Variables|Dialogue|GetCurrent%20Dialogue) Line%20to%20Add%20to (Variables|Dialogue|Characters|GetCharacter%20Index))))
        (Dialogue|FunctUpdateDialogueHUD _output_get)
        (else
          ;[0.3802 0.3802 0.3802 1 12] If character @ index is not valid, assume line is fully printed, therefore no longer revealing
          (CallFunction|LineFinished))))))

(event Custom|Setup%20Gameplay%20Dialogue
  (bind _dt_maindialogue (Variables|Dialogue|Main|GetDT_MainDialogue))
  (bind _outrownames (DataTable|GetDataTableRowNames _dt_maindialogue))
  (bind (_array_element _array_index) (Utilities|Array|ForEachLoopwithBreak _outrownames)
    (:LoopBody
      (bind _returnvalue (Utilities|GetDataTableRow _dt_maindialogue _array_element)
        (:then
          (bind _output_get (Variables|Default|SetStruct_MainDialogue _returnvalue))
          (if (Utilities|IsValidClass (.DialogueTrigger (Utilities|Struct|BreakStruct_Dialogue _output_get)))
            (if (and (== (.DialogueTrigger (Utilities|Struct|BreakStruct_Dialogue _output_get)) (Utilities|GetClass (Components|GetOwner))) (== (.EncounterIndex (Utilities|Struct|BreakStruct_Dialogue _output_get)) (Variables|Default|GetEncounter%20Index)))
              (Variables|Default|SetConversation%20Index _array_index)
              (CallFunction|FindGameplayLine))))))))

(event Custom|Find%20Gameplay%20Line
  (Utilities|FlowControl|Sequence
    (:then_0
      (Utilities|Array|ForEachLoopwithBreak (stale Custom|Setup%20Gameplay%20Dialogue _outrownames)) ; enters at Break
    )
    (:then_1
      (CallFunction|Talk))))

(event Custom|Talk
  (bind (_dialogue_line _person_talking _valid_line_) (CallFunction|FunctGetDialogueItems@Index))
  (if (Variables|Default|GetisRevealingLine)
    ;[0.2396 0.2396 0.2396] if input during a line being printed, it should stop printing each character & just reveal the whole line
    (CallFunction|LineFinished)
    (CallFunction|RevealFullDialogueLine)
    (else
      (Math|Integer|IncrementInt (Variables|Dialogue|Main|GetMain%20Dialogue%20Index)
        (:%20%20
          (Variables|Dialogue|Characters|SetCharacter%20Index -1)
          (Variables|Dialogue|SetCurrent%20Dialogue "")
          (Variables|Default|SetisRevealingLine true)
          (Variables|Default|SetlineFinished false)))))
  (bind _outrownames (DataTable|GetDataTableRowNames (Variables|Dialogue|Main|GetDT_MainDialogue)))
  (bind _returnvalue (Utilities|GetDataTableRow (Variables|Dialogue|Main|GetDT_MainDialogue) (Utilities|Array|Get(acopy) _outrownames (Variables|Default|GetConversation%20Index)))
    (:then
      (Variables|Default|SetStruct_MainDialogue _returnvalue)
      ;[0.2552 0.2552 0.2552 1 9] Check if new line is valid
      (if _valid_line_
        (CallFunction|FunctUpdatePersonTalkingHUD _person_talking)
        (CallFunction|StartAddingCharacters)
        (else
          ;[0.375 0.375 0.375] Ran out of main dialogue?
          (Variables|Dialogue|Main|SetfinishedMainDialogue? true)
          (CallFunction|ExitDialogue))))))

(event Custom|Turn%20to%20Person
  (bind (_new_rot _target_rot) (CallFunction|FunctPlayerLook@NPC))
  ;[0.2917 0.2917 0.2917] if not already in conversation, start talking
  (Transformation|SetActorRotation (Variables|Default|GetPlayer) _new_rot)
  (if (Utilities|Operators|EqualEqual _new_rot _target_rot 15.0)
    (Utilities|Time|ClearandInvalidateTimerbyHandle (Variables|Default|GetTimer_TurntoPerson))
    (CallFunction|StartTalking)))

(event Custom|Decide%20if%20to%20Add%20Char
  (if (Variables|Dialogue|Main|GetfinishedMainDialogue?)
    ;[0.2969 0.2969 0.2969] Main Dialogue
    (if (Variables|Default|GetisRevealingLine)
      (CallFunction|AddNextChar (.OutItem (Utilities|Array|Random (.SecondaryDialogue (Utilities|Struct|BreakStruct_Dialogue (Variables|Default|GetStruct_MainDialogue))))))
      (else
        (CallFunction|RevealFullDialogueLine)))
    (else
      ;[0.2969 0.2969 0.2969] Main Dialogue
      (if (Variables|Default|GetisRevealingLine)
        (CallFunction|AddNextChar (.Dialogue%20Line (CallFunction|FunctGetDialogueItems@Index)))
        (else
          (CallFunction|RevealFullDialogueLine))))))

(event Custom|Reveal%20Full%20Dialogue%20Line
  ;[0.2292 0.2292 0.2292] Reveal the whole line
  (bind _outrownames (DataTable|GetDataTableRowNames (Variables|Dialogue|Main|GetDT_MainDialogue)))
  (bind _returnvalue (Utilities|GetDataTableRow (Variables|Dialogue|Main|GetDT_MainDialogue) (Utilities|Array|Get(acopy) _outrownames (Variables|Default|GetConversation%20Index)))
    (:then
      (Variables|Default|SetStruct_MainDialogue _returnvalue)
      (bind _output_get (Variables|Dialogue|SetCurrent%20Dialogue (.Dialogue%20Line (CallFunction|FunctGetDialogueItems@Index))))
      (Dialogue|FunctUpdateDialogueHUD _output_get)
      (Variables|Default|SetlineFinished true))))

(event Custom|Exit%20Dialogue
  (Default|FunctManageIMC (Variables|Default|GetPlayer))
  (Pawn|Components|CharacterMovement|SetMovementMode (Variables|/Script/Engine.Character|GetCharacterMovement (Variables|Default|GetPlayer)) "MOVE_Walking" 0)
  (Widget|RemovefromParent (Variables|Default|GetUW_Dialogue))
  (Variables|Default|SetinConversation false)
  (bind _output_get (Variables|Dialogue|Main|SetMain%20Dialogue%20Index -1))
  (Variables|Dialogue|Characters|SetCharacter%20Index _output_get))

(event Custom|Line%20Finished
  (Variables|Default|SetisRevealingLine false)
  (Utilities|Time|ClearandInvalidateTimerbyHandle (Variables|Dialogue|Characters|GetTimer_AddCharacter))
  (Variables|Default|SetlineFinished true)
  ;[0.2292 0.2292 0.2292] Rn, if a conversation is supposed to give the player weapon, it does so at end of convo/exit dialogue
  (if (Utilities|Struct|BreakStruct_Dialogue (Variables|Default|GetStruct_MainDialogue))
    (bind _asbp_npc (Utilities|Casting|CastToBP_NPC (Components|GetOwner)))
    (if (Utilities|IsValidClass (Variables|/Game/LevelStuff/ThirdPerson/Blueprints/Movement/BP_ThirdPersonCharacter.BP_ThirdPersonCharacter_C|GetStartingWeap _asbp_npc))
      (Utilities|IsValid (Variables|/Script/Engine.ChildActorComponent|GetChildActor (Actor|GetComponentbyClass _asbp_npc "/Script/Engine.ChildActorComponent"))
        (:Is%20Valid
          (Class|BPIInteract|BPIGiveWeap(Message) (Variables|Default|GetPlayer) (Variables|/Game/LevelStuff/ThirdPerson/Blueprints/Movement/BP_ThirdPersonCharacter.BP_ThirdPersonCharacter_C|GetStartingWeap _asbp_npc))
          (ChildActorComponent|SetChildActorClass (Actor|GetComponentbyClass _asbp_npc "/Script/Engine.ChildActorComponent") 0))))))

(event Custom|Find%20NPC%20Line
  ;[0.2135 0.2135 0.2135] Setup NPC before Talking
  (Utilities|FlowControl|Sequence
    (:then_0
      (Utilities|Array|ForEachLoopwithBreak (stale Custom|Setup%20Dialogue_NPC _outrownames)) ; enters at Break
    )
    (:then_1
      (CallFunction|Talk))))

(event Custom|Setup%20Dialogue_NPC
  (bind _dt_maindialogue (Variables|Dialogue|Main|GetDT_MainDialogue))
  ;[0.2135 0.2135 0.2135] Setup NPC before Talking
  (bind _outrownames (DataTable|GetDataTableRowNames _dt_maindialogue))
  (bind (_array_element _array_index) (Utilities|Array|ForEachLoopwithBreak _outrownames)
    (:LoopBody
      (bind _returnvalue (Utilities|GetDataTableRow _dt_maindialogue _array_element)
        (:then
          ;;[0.2865 0.2865 0.2865] Get the row/struct of this  NPC and Encounter
          (bind _output_get (Variables|Default|SetStruct_MainDialogue _returnvalue))
          (if (Utilities|IsValidClass (.NPC (Utilities|Struct|BreakStruct_Dialogue _output_get)))
            (if (and (== (.NPC (Utilities|Struct|BreakStruct_Dialogue _output_get)) (Utilities|GetClass (Components|GetOwner))) (== (.EncounterIndex (Utilities|Struct|BreakStruct_Dialogue _output_get)) (Variables|Default|GetEncounter%20Index)))
              (Variables|Default|SetConversation%20Index _array_index)
              (CallFunction|FindNPCLine))))))))

(event Custom|Start%20Adding%20Characters
  (bind _returnvalue (Utilities|Time|SetTimerbyEvent (delegate Custom|Decide%20if%20to%20Add%20Char) 0.05 true))
  (Variables|Dialogue|Characters|SetTimer_AddCharacter _returnvalue))

(event EventBeginPlay
  (bind _returnvalue (Components|GetOwner))
  (bind _returnvalue_2 (Actor|GetComponentbyClass _returnvalue "/Script/Engine.BoxComponent"))
  (if (or (Utilities|IsValid _returnvalue_2) (Utilities|IsValid (Actor|GetComponentbyClass _returnvalue "/Script/Engine.SphereComponent")))
    (switch Utilities|FlowControl|Switch|SwitchonEnum_DialogueMethod (Variables|Default|GetDialogue%20Method)
      (:NewEnumerator1
        (Collision|BindEventtoOnComponentBeginOverlap _returnvalue_2 (delegate Custom|Enter%20Dialogue))))))

(fn FunctUpdateDialogueHUD
  (params (Current%20Dialogue :type String))
  (bind _uw_dialogue (Variables|Default|GetUW_Dialogue)
    (:then
      (Variables|/Script/UMG.TextBlock|SetText (Variables|/Game/Users/Stanley/UW_Dialogue.UW_Dialogue_C|GetTxt_Dialogue _uw_dialogue) (Utilities|Text|ToText(String) Current%20Dialogue)))
    (:else)))

(fn FunctAddChartoLine
  (params (Dialogue%20to%20Add%20to :type String) (SourceString :type String) (Character%20Index :type Integer))
  (return (Utilities|String|Append Dialogue%20to%20Add%20to (.Char (Dialogue|Characters|FunctGetChar@Index SourceString Character%20Index)))))

(fn FunctAddCharacter
  (bind _returnvalue (Utilities|String|GetCharacterArrayfromString ""))
  (bind _character_index (Variables|Dialogue|Characters|GetCharacter%20Index))
  (if (Variables|Default|GetisRevealingLine)
    (Utilities|FlowControl|Sequence
      (:then_0
        ;[1 1 1] Should ensure the same character @ index is not printed again
        (Variables|Dialogue|Characters|SetPrevious%20Character%20Index (Variables|Dialogue|Characters|GetCharacter%20Index))
        (Math|Integer|IncrementInt (Variables|Dialogue|Characters|GetCharacter%20Index)))
      (:then_1
        (if (not (== (Variables|Dialogue|Characters|GetCharacter%20Index) (Variables|Dialogue|Characters|GetPrevious%20Character%20Index)))
          ;[1 1 1] If character @ index is not valid, assume line is fully printed, therefore no longer revealing
          (if (Utilities|Array|IsValidIndex _returnvalue _character_index)
            (bind _output_get (Variables|Dialogue|SetCurrent%20Dialogue (Utilities|String|Append (Variables|Dialogue|GetCurrent%20Dialogue) (Utilities|Array|Get(acopy) _returnvalue _character_index))))
            (Dialogue|FunctUpdateDialogueHUD _output_get)
            (else
              (Variables|Default|SetisRevealingLine false)
              (Utilities|Time|ClearandInvalidateTimerbyHandle (Variables|Dialogue|Characters|GetTimer_AddCharacter)))))))
    (else
      ;[1 1 1] Show the whole line of text instantly
      (bind _output_get_2 (Variables|Dialogue|SetCurrent%20Dialogue ""))
      (Dialogue|FunctUpdateDialogueHUD _output_get_2))))

(fn FunctGetChar@Index
  (params (SourceString :type String) (Index :type Integer))
  (bind _returnvalue (Utilities|String|GetCharacterArrayfromString SourceString))
  (return (Utilities|Array|Get(acopy) _returnvalue Index) (Utilities|Array|IsValidIndex _returnvalue Index)))

(fn FunctPlayerLook@NPC
  (bind _returnvalue (Components|GetOwner))
  (bind _player (Variables|Default|GetPlayer))
  (bind _returnvalue_2 (Transformation|GetActorLocation _player))
  (bind _returnvalue_3 (Transformation|GetActorLocation _returnvalue))
  (bind _returnvalue_4 (Math|Rotator|FindLookatRotation _returnvalue_2 _returnvalue_3))
  (return (Math|Interpolation|RInterpTo (Transformation|GetActorRotation _player) _returnvalue_4 (Utilities|Time|GetWorldDeltaSeconds) 2.0) _returnvalue_4))

(fn FunctGetDialogueItems@Index
  (bind _struct_maindialogue (Variables|Default|GetStruct_MainDialogue))
  (bind _main_dialogue_index (Variables|Dialogue|Main|GetMain%20Dialogue%20Index))
  (bind _maindialoguelines (Utilities|Struct|BreakStruct_Dialogue _struct_maindialogue))
  (return (Utilities|Array|Get(acopy) _maindialoguelines _main_dialogue_index) (Utilities|Array|Get(acopy) (.PersonTalking (Utilities|Struct|BreakStruct_Dialogue (Variables|Default|GetStruct_MainDialogue))) (Variables|Dialogue|Main|GetMain%20Dialogue%20Index)) (Utilities|Array|IsValidIndex _maindialoguelines _main_dialogue_index)))

(fn FunctUpdatePersonTalkingHUD
  (params (Current%20Person%20Talking :type String))
  (bind _uw_dialogue (Variables|Default|GetUW_Dialogue)
    (:then
      (Variables|/Script/UMG.TextBlock|SetText (Variables|/Game/Users/Stanley/UW_Dialogue.UW_Dialogue_C|GetTxt_PersonTalking _uw_dialogue) (Utilities|Text|ToText(String) Current%20Person%20Talking)))
    (:else)))

(fn BPITalk
  (params (wasTalking :type Boolean))
  (return false))