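; BP_DialogueTrigger is a box trigger that records a gameplay dialogue encounter as used, so it does not return after a load.
; Player overlap sets a Triggered flag and requests a synchronous save through the GameInstance, and SaveData then stores the BPCDialogue encounter index.
; On BeginPlay it requests a load, and LoadData destroys the actor if that index is already saved.
; The graph itself never starts the dialogue.
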(event OnComponentBeginOverlap(Box)
  (params (OverlappedComponent :type Primitive%20Component%20Object%20Reference) (OtherActor :type Actor%20Object%20Reference) (OtherComp :type Primitive%20Component%20Object%20Reference) (OtherBodyIndex :type Integer) (bFromSweep :type Boolean) (SweepResult :type Hit%20Result%20Structure%20%28by%20ref%29))
  (if (Actor|ActorHasTag OtherActor "Player")
    (Variables|Default|SetTriggered true)
    (Class|BPIPersistence|RequestSave(Message) (Variables|Default|GetGameInstanceRef) false "NewEnumerator0")))

(event EventBeginPlay
  (bind _output_get (Variables|Default|SetGameInstanceRef (CallFunction|ValidGameInstance)))
  (Class|BPIPersistence|RequestLoad(Message) _output_get self "NewEnumerator0"))

(event EventSaveData
  (params (SaveGameRef :type BP%20Game%20Save%20Data%20Object%20Reference))
  (if (Variables|Default|GetTriggered)
    (Utilities|Array|AddUnique (Variables|/Game/Users/Liam/Saving/BP_GameSaveData.BP_GameSaveData_C|GetGameplayDialogueSaved SaveGameRef) (Variables|/Game/Users/Stanley/BPC_Dialogue.BPC_Dialogue_C|GetEncounter%20Index (Variables|Default|GetBPC_Dialogue)))
    (Variables|Default|SetTriggered false)))

(event EventLoadData
  (params (SaveGameRef :type BP%20Game%20Save%20Data%20Object%20Reference))
  (for _array_element (Variables|/Game/Users/Liam/Saving/BP_GameSaveData.BP_GameSaveData_C|GetGameplayDialogueSaved SaveGameRef)
    (if (== _array_element (Variables|/Game/Users/Stanley/BPC_Dialogue.BPC_Dialogue_C|GetEncounter%20Index (Variables|Default|GetBPC_Dialogue)))
      (Actor|DestroyActor))))

(fn ConstructionScript)