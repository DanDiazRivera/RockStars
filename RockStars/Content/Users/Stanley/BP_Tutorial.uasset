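; BP_Tutorial is a tutorial trigger actor meant to show a pausing popup with title, description and image.
; Trigger overlap and the interactive interface event both call InteractWithTutorial, but it and the enter/exit events are empty.
; Unconnected logic holds the intended toggle: create UW_Tutorial, swap input mapping contexts, show the cursor and pause, or undo this and destroy the actor.
; As wired, none of that logic runs.
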(event Custom|Interact%20with%20Tutorial
  (params (OverlappedComponent :type Primitive%20Component%20Object%20Reference) (OtherActor :type Actor%20Object%20Reference) (OtherComp :type Primitive%20Component%20Object%20Reference) (OtherBodyIndex :type Integer) (bFromSweep :type Boolean) (SweepResult :type Hit%20Result%20Structure%20%28by%20ref%29)))

(event Custom|Enter%20Tutorial
  ;[1 1 1] Enter Tutorial
)

(event Custom|Exit%20Tutorial)

(event EventBeginPlay
  (Collision|BindEventtoOnComponentBeginOverlap (Variables|Default|GetTrigger%20Box) (delegate Custom|Interact%20with%20Tutorial)))

(event EventBPITriggerInteractive
  (params (Actor :type Actor%20Object%20Reference))
  (CallFunction|InteractwithTutorial 0 Actor 0 0 false))

(fn ConstructionScript)